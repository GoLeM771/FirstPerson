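; Parent class for monster generator body parts, which can shoot at the player and spawn FlootBug enemies.
; BeginPlay randomizes Mass, and getters expose it with attachment coordinates, mesh and state, some as empty stubs.
; Enabling shooting turns on Tick, which aims the Arrow at the player within HoverDistance, and starts a looping projectile timer with a randomized interval.
; A second timer spawns bugs at the Arrow, either unlimited or until EnemySpawnCount runs out.
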(event Custom|AimAtTarget
  (Transformation|SetWorldRotation (Variables|Default|GetArrow) (Math|Rotator|FindLookatRotation (Transformation|GetActorLocation) (Transformation|GetActorLocation (Variables|Default|GetTargetPlayer))) false false))

(event Custom|ResetAim)

(event EventBeginPlay
  (Variables|Default|SetMass (* (Variables|Default|GetMass) (Math|Random|RandomFloatinRange 1.0 (Variables|Default|GetMaximumPossibleMass)))))

(event Collision|EventActorBeginOverlap
  (params (OtherActor :type Actor%20Object%20Reference)))

(event EventTick
  (params (DeltaSeconds :type Float%20%28single-precision%29))
  (Variables|Default|SetTargetLocation (Transformation|GetActorLocation (Variables|Default|GetTargetPlayer)))
  (if (<= (Math|Vector|VectorLength (- (Transformation|GetActorLocation) (Variables|Default|GetTargetLocation))) (Variables|Default|GetHoverDistance))
    (CallFunction|AimatTarget)
    (else
      (CallFunction|ResetAim))))

(event EventCanSpawnEnemySetter
  (params (CanSpawn? :type Boolean))
  (Variables|Default|SetCanSpawn? CanSpawn?))

(event EventBodyPartSpawnEnemy
  (params (SpawnWithoutCount? :type Boolean))
  (Variables|Default|SetSpawnWithoutCount? SpawnWithoutCount?)
  (Utilities|Time|SetTimerbyFunctionName self "SpawnEnemy" (Variables|Default|GetFireRate) true 0.2))

(event EventBodyPartsCanShoot?
  (Development|SetHiddeninGame (Variables|Default|GetArrow) false false)
  (Actor|Tick|SetActorTickEnabled true)
  (Variables|Default|SetTargetPlayer (Game|GetPlayerCharacter 0))
  (Utilities|Time|SetTimerbyFunctionName self "BodyPartShoot" (Math|Random|RandomFloatinRange 2.0 4.0) true))

(fn ConstructionScript)

(fn BodyPartShoot
  (bind _bulletspeed (Variables|Default|GetBulletSpeed))
  (bind _returnvalue (Game|SpawnActorfromClass "/Game/Blueprints/FirstPersonProjectile.FirstPersonProjectile_C" (Transformation|GetWorldTransform (Variables|Default|GetArrow)) "Undefined" 0 true (Variables|Default|GetBulletDamage) 0))
  (Variables|/Script/Engine.ProjectileMovementComponent|SetInitialSpeed (Variables|/Game/Blueprints/FirstPersonProjectile.FirstPersonProjectile_C|GetProjectile _returnvalue) _bulletspeed)
  (Variables|/Script/Engine.ProjectileMovementComponent|SetMaxSpeed (Variables|/Game/Blueprints/FirstPersonProjectile.FirstPersonProjectile_C|GetProjectile _returnvalue) _bulletspeed))

(fn SpawnEnemy
  (LocalVariables|SetSpawnLocation (Math|Transform|MakeTransform (Transformation|GetWorldLocation (Variables|Default|GetArrow))))
  (if (Variables|Default|GetSpawnWithoutCount?)
    (Game|SpawnActorfromClass "/Game/Bot/FlootBug/FlootBug.FlootBug_C" (LocalVariables|GetSpawnLocation) "Undefined" 0 0 false 2 0.0 0 0)
    (return)
    (elif (> (Variables|Default|GetEnemySpawnCount) 0)
      (Game|SpawnActorfromClass "/Game/Bot/FlootBug/FlootBug.FlootBug_C" (LocalVariables|GetSpawnLocation) "Undefined" 0 0 false 2 0.0 0 0)
      (Variables|Default|SetEnemySpawnCount (- (Variables|Default|GetEnemySpawnCount) 1))
      (return))))

(fn ArmsCoordinateGetter
  (return (Variables|Default|GetArmsCoordinates)))

(fn BodyPartMassGetter
  (return (Variables|Default|GetMass)))

(fn BodyPartsArreyGetter
  (return 0))

(fn CanSpawnEnemyGetter
  (return (Variables|Default|GetCanSpawn?)))

(fn EnemySkeletalMeshGetter
  (return (Variables|Default|GetSkeletalMesh)))

(fn HeadCoordinateGetter
  (return (Variables|Default|GetHeadCoordinates_0)))

(fn IsDeadGetter
  (return false))

(fn TorsoCoordinateGetter
  (return (Variables|Default|GetTorsoCoordinates)))