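; Mutant enemy that chases and melees the player, with health and walk speed scaled by its generated model's mass.
; PawnSensing or a zerg-spawn flag drives AIMoveTo, while an overlap volume loops delayed line-trace attacks.
; Hits feed projected wounds, spaced torso blood-soak spots and WoundSystemExtras health.
; First sighting reveals its minimap icon, music state follows sightings and nearby-group deaths, and three "Beton" counts halt movement.
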(event OnSeePawn(PawnSensing)
  (params (Pawn :type Pawn%20Object%20Reference))
  ;[1 1 1] MoveToPlayerIfSee
  (CallFunction|ShowMinimapIcon)
  (if (not (Variables|Default|GetIsDead?))
    (if (Utilities|DoesObjectImplementInterface Pawn "/Game/Blueprints/Interfaces/PlayerInterface.PlayerInterface_C")
      (Variables|Default|SetPlayerinAgro true)
      (AI|AIMoveTo self "0, 0, 0" Pawn 1.2e+02 false
        (:then
          (Utilities|FlowControl|Sequence
            (:then_0
              (Utilities|FlowControl|DoOnce false
                (:Completed
                  (Audio|PlaySoundatLocation (Variables|Default|GetChargeSound) (Transformation|GetActorLocation self) "0, 0, 0" 1.0 1.0 0.0 0 0 0))))
            (:then_1
              (Class|BPLMusic|ChangeMusicState(Message) (Game|GetGameState) 1.0))))))))

(event OnComponentBeginOverlap(Sphere)
  (params (OverlappedComponent :type Primitive%20Component%20Object%20Reference) (OtherActor :type Actor%20Object%20Reference) (OtherComp :type Primitive%20Component%20Object%20Reference) (OtherBodyIndex :type Integer) (bFromSweep :type Boolean) (SweepResult :type Hit%20Result%20Structure%20%28by%20ref%29))
  (bind _asbase_zombie_character (Utilities|Casting|CastToBaseZombieCharacter OtherActor))
  (Utilities|Array|Add (Variables|Default|GetGroupArray) _asbase_zombie_character))

(event OnComponentEndOverlap(Sphere)
  (params (OverlappedComponent :type Primitive%20Component%20Object%20Reference) (OtherActor :type Actor%20Object%20Reference) (OtherComp :type Primitive%20Component%20Object%20Reference) (OtherBodyIndex :type Integer))
  (bind _asbase_zombie_character (Utilities|Casting|CastToBaseZombieCharacter OtherActor))
  (Utilities|Array|RemoveItem (Variables|Default|GetGroupArray) _asbase_zombie_character))

(event OnComponentBeginOverlap(PlayerSencing)
  (params (OverlappedComponent :type Primitive%20Component%20Object%20Reference) (OtherActor :type Actor%20Object%20Reference) (OtherComp :type Primitive%20Component%20Object%20Reference) (OtherBodyIndex :type Integer) (bFromSweep :type Boolean) (SweepResult :type Hit%20Result%20Structure%20%28by%20ref%29))
  ;[1 1 1] Attack
  (if (not (Variables|Default|GetIsDead?))
    (if (Utilities|DoesObjectImplementInterface OtherActor "/Game/Blueprints/Interfaces/PlayerInterface.PlayerInterface_C")
      (Variables|Default|SetPlayerinBox true)
      (Utilities|FlowControl|Delay 0.5 :!label _label)
      (Variables|Default|SetBotAttack true)
      (CallFunction|AttackPlayer 150 (* (/ (Variables|Default|GetDamage) 1e+02) -1.0))
      (if (Variables|Default|GetPlayerinBox)
        (goto _label)
        (else
          (Variables|Default|SetBotAttack false)
          (if (Variables|Default|GetPlayerinAgro)
            (AI|AIMoveTo self "0, 0, 0" (Game|GetPlayerCharacter 0) 5.0 false)))))))

(event OnComponentEndOverlap(PlayerSencing)
  (params (OverlappedComponent :type Primitive%20Component%20Object%20Reference) (OtherActor :type Actor%20Object%20Reference) (OtherComp :type Primitive%20Component%20Object%20Reference) (OtherBodyIndex :type Integer))
  ;[1 1 1] Attack
  (if (not (Variables|Default|GetIsDead?))
    (if (Utilities|DoesObjectImplementInterface OtherActor "/Game/Blueprints/Interfaces/PlayerInterface.PlayerInterface_C")
      (Variables|Default|SetPlayerinBox false)
      (Variables|Default|SetBotAttack false))))

(event Custom|SimpleDamage
  (params (Damage :type Float%20%28single-precision%29))
  ;[1 1 1] Дамаг в обход системы виз дамага
  (Default|HealthDecrease (Variables|Default|GetWoundSystemExtras) Damage "None"))

(event Custom|ZergPlayer
  (AI|AIMoveTo self "0, 0, 0" (Game|GetPlayerCharacter 0) 5.0 false))

(event Custom|BossCharge
  ;[1 1 1] MoveToPlayerIfSee
)

(event Custom|ShowMinimapIcon
  (Utilities|FlowControl|DoOnce false
    (:Completed
      (Rendering|SetVisibility (Variables|Default|GetMiniMapIcon) true false)
      (CallFunction|AddInfotoMinimap))))

(event Collision|EventActorBeginOverlap
  (params (OtherActor :type Actor%20Object%20Reference)))

(event EventTick
  (params (DeltaSeconds :type Float%20%28single-precision%29))
  (if (Variables|Default|GetIsDead?)
    (Components|Movement|StopMovementImmediately (Variables|Character|GetCharacterMovement) :!label _label)
    (else
      (if (Variables|/Script/AIModule.PawnSensingComponent|GetbSeePawns (Variables|Default|GetPawnSensing))
        _
        (else
          (Variables|Default|SetPlayerinAgro false)))
      (if (>= (Variables|Default|GetSpawnedBetonInt) 3)
        (goto _label)))))

(event EventBetonCounterPlus
  ;[1 1 1] Вызовы интерфейса
  (Variables|Default|SetSpawnedBetonInt (+ (Variables|Default|GetSpawnedBetonInt) 1)))

(event EventSimpleDamageEnemy
  (params (Damage :type Float%20%28single-precision%29))
  ;[1 1 1] Вызовы интерфейса
  (Default|HealthDecrease (Variables|Default|GetWoundSystemExtras) Damage "None"))

(event EventTurnOffPaperSpriteInterface
  (bind _minimapicon (Variables|Default|GetMiniMapIcon))
  (Utilities|IsValid _minimapicon
    (:Is%20Valid
      (Rendering|SetVisibility _minimapicon false false))))

(event Game|Damage|EventPointDamage
  (params (Damage :type Float%20%28single-precision%29) (DamageType :type Damage%20Type%20Object%20Reference) (HitLocation :type Vector :default "0, 0, 0") (HitNormal :type Vector :default "0, 0, 0") (HitComponent :type Primitive%20Component%20Object%20Reference) (BoneName :type Name :default "None") (ShotFromDirection :type Vector :default "0, 0, 0") (InstigatedBy :type Controller%20Object%20Reference) (DamageCauser :type Actor%20Object%20Reference) (HitInfo :type Hit%20Result%20Structure%20%28by%20ref%29))
  ;[1 1 1] You should call this event from your weapon
  (if (== (Variables|Character|GetMesh) HitComponent)
    (Default|TakeHit (Variables|Default|GetWoundComponent) BoneName HitLocation (* HitNormal -1.0) (select (Variables|/Game/Materials/CharacterWoundSystem/Components/WoundComponent.WoundComponent_C|GetUseProjectedWound (Variables|Default|GetWoundComponent)) (Math|Random|RandomFloatinRange 3.0 5.0) (Math|Random|RandomFloatinRange 1e+01 15.0)))
    (Default|Hit (Variables|Default|GetWoundSystemExtras) Damage HitLocation HitNormal HitComponent BoneName ShotFromDirection HitInfo)
    (bind _yes (CallFunction|CanAddSoakungWound BoneName HitLocation 2e+01))
    (if _yes
      (Default|TakeHit (Variables|Default|GetBloodSoakingSpotComponent) HitLocation BoneName 15.0 0.1 3.0))))

(event EventTurnonPaperSpriteInterface
  (bind _minimapicon (Variables|Default|GetMiniMapIcon))
  (Utilities|IsValid _minimapicon
    (:Is%20Valid
      (Rendering|SetVisibility _minimapicon true false))))

(event EventBeginPlay
  (bind _woundsystemextras (Variables|Default|GetWoundSystemExtras))
  (bind _charactermovement (Variables|Character|GetCharacterMovement))
  (Utilities|FlowControl|Sequence
    (:then_0
      ;[1 1 1] Initialize the WoundComponent
      (bind _returnvalue (AddComponent|AddSceneCaptureComponent2D false (Math|Transform|MakeTransform "0, 0,250.000000" "-90.000000,90.000000,180.000000"))) ; There's some properties set in this node details panel
      (Transformation|AttachComponentToComponent _returnvalue (Variables|Character|GetMesh) "None" "SnapToTarget" "SnapToTarget" "SnapToTarget" true) ; This way even if you transform your mesh the scene capture still works
      (Default|Initialize (Variables|Default|GetWoundComponent) (Variables|Character|GetMesh) _returnvalue)
      (Default|Initialize (Variables|Default|GetBloodSoakingSpotComponent) (Variables|Character|GetMesh))
      (Variables|/Game/Materials/CharacterWoundSystem/Demo/Blueprint/Components/WoundSystemExtras.WoundSystemExtras_C|SetHealth (Variables|Default|GetWoundSystemExtras) (Variables|Default|GetEnemyHealth))
      (Variables|/Game/Materials/CharacterWoundSystem/Demo/Blueprint/Components/WoundSystemExtras.WoundSystemExtras_C|SetbNavigation _woundsystemextras false)
      (Variables|/Game/Materials/CharacterWoundSystem/Demo/Blueprint/Components/WoundSystemExtras.WoundSystemExtras_C|SetUseRagdoll _woundsystemextras false)
      (if (Variables|Default|GetZergRushSpwn?)
        (CallFunction|ZergPlayer)))
    (:then_1
      ;[1 1 1] HealthChangeMass
      (Utilities|FlowControl|Sequence
        (:then_0
          (bind _asmodel_generator (Utilities|Casting|CastToModelGenerator (Variables|/Script/Engine.ChildActorComponent|GetChildActor (Variables|Default|GetModelGenerator))))
          (Variables|Default|SetMassCoeff (/ (Variables|/Game/MonsterGenerator/ModelGenerator.ModelGenerator_C|GetMass _asmodel_generator) 6.0)))
        (:then_1
          (Variables|Default|SetEnemyHealth (Math|Float|Truncate (* (Variables|Default|GetMassCoeff) 2e+02))))
        (:then_2
          ;[1 1 1] SpeedChangeofMass
          (if (< (- 2.0 (Variables|Default|GetMassCoeff)) 1.0)
            (Variables|/Script/Engine.CharacterMovementComponent|SetMaxWalkSpeed _charactermovement (* (- 2.0 (Variables|Default|GetMassCoeff)) 1.5e+02))
            (else
              (Variables|/Script/Engine.CharacterMovementComponent|SetMaxWalkSpeed _charactermovement (* (- 2.0 (Variables|Default|GetMassCoeff)) 2.5e+02)))))))))

(fn ConstructionScript)

(fn CanAddSoakungWound
  (params (BoneName :type Name) (WorldLocation :type Vector) (MinDistance :type Float%20%28single-precision%29))
  (bind _bloodsoakingspotcomponent (Variables|Default|GetBloodSoakingSpotComponent))
  (if (Math|Boolean|ORBoolean (Utilities|Name|Equal(Name) BoneName "pelvis") (Utilities|Name|Equal(Name) BoneName "spine_01") (Utilities|Name|Equal(Name) BoneName "spine_02") (Utilities|Name|Equal(Name) BoneName "spine_03"))
    (LocalVariables|SetLocalMeshSpaceLocation (Default|TransformLocationbyRefBoneTransform _bloodsoakingspotcomponent BoneName WorldLocation))
    (bind _array_element (Utilities|Array|ForEachLoopwithBreak (Variables|/Game/Materials/CharacterWoundSystem/Components/BloodSoakingSpotComponent.BloodSoakingSpotComponent_C|GetLocations _bloodsoakingspotcomponent) :!label _label)
      (:LoopBody
        (if (< (Math|Vector|VectorLength (- _array_element (LocalVariables|GetLocalMeshSpaceLocation))) MinDistance)
          (LocalVariables|SetResult false)
          (goto _label Break)))
      (:Completed
        (return (LocalVariables|GetResult))))
    (else
      (return false))))

(fn AttackPlayer
  (params (AttRange :type Integer) (Damage :type Float%20%28single-precision%29))
  (bind _capsulecomponent (Variables|Collision|GetCapsuleComponent))
  (bind _returnvalue (Transformation|GetWorldLocation _capsulecomponent))
  (if (not (Variables|Default|GetIsDead?))
    (Components|Movement|StopMovementImmediately (Variables|Character|GetCharacterMovement))
    (bind (_outhit _returnvalue_2) (Collision|LineTraceByChannel _returnvalue (+ _returnvalue (* (Math|Vector|GetForwardVector (Transformation|GetWorldRotation _capsulecomponent)) AttRange)) "TraceTypeQuery2" false (Utilities|Array|MakeArray self) "ForDuration"))
    (if _returnvalue_2
      (if (Utilities|DoesObjectImplementInterface (.HitActor (Collision|BreakHitResult _outhit)) "/Game/Blueprints/Interfaces/PlayerInterface.PlayerInterface_C")
        (Class|PlayerInterface|CreateHudHitWidgetInterface(Message) (.HitActor (Collision|BreakHitResult _outhit)) (.Location (Collision|BreakHitResult _outhit)))
        (Class|PlayerInterface|ModifyStatInterface(Message) (Game|GetPlayerCharacter 0) Damage "NewEnumerator1")
        (Variables|Default|SetAttackVar (Math|Random|RandomIntegerinRange 0 2))
        (else
          (Development|PrintString (Utilities|String|Append (Utilities|GetDisplayName self) " trace cross " (Utilities|GetDisplayName (.HitActor (Collision|BreakHitResult _outhit))))))))))

(fn DeadFuction
  (bind _grouparray (Variables|Default|GetGroupArray))
  (bind _minimapicon (Variables|Default|GetMiniMapIcon))
  (Utilities|IsValid _minimapicon
    (:Is%20Valid
      (Components|DestroyComponent _minimapicon))
    (:Is%20Not%20Valid
      _))
  (Collision|SetCollisionEnabled (Variables|Character|GetMesh) "NoCollision")
  (Collision|SetCollisionEnabled (Variables|Collision|GetCapsuleComponent) "NoCollision")
  (for _array_element _grouparray
    (if (Variables|/Game/Bot/BaseEnemyCharacter/BaseZombieCharacter.BaseZombieCharacter_C|GetIsDead? _array_element)
      (Utilities|Array|RemoveItem _grouparray _array_element)))
  (if (not (> (Utilities|Array|Length _grouparray) 0))
    (Class|BPLMusic|ChangeMusicState(Message) (Game|GetGameState) 0.2)))

(fn AddInfotoMinimap
  (bind _map (Class|PlayerInterface|FullMapReferenceGetter(Message) (Game|GetPlayerCharacter 0)))
  (switch int (Variables|Default|GetFloorNum)
    (:1
      (Utilities|Array|Add (Variables|/Game/Blueprints/UI/MiniMap_v2/FullMap.FullMap_C|GetKnownElementOnFloorOne _map) self))
    (:2
      (Utilities|Array|Add (Variables|/Game/Blueprints/UI/MiniMap_v2/FullMap.FullMap_C|GetKnownElementOnFloorTwo _map) self))
    (:3
      (Utilities|Array|Add (Variables|/Game/Blueprints/UI/MiniMap_v2/FullMap.FullMap_C|GetKnownElementOnFloorThree _map) self)))
  (return))

(fn DistancetoPlayerGetter
  (return "NewEnumerator0"))

(fn FloorNumGetter
  (return 0))

(fn WorldLocationGetterInterface
  (return "0, 0, 0"))