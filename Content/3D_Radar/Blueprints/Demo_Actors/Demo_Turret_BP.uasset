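; Demo turret actor for the 3D Radar content that animates continuously and carries faction tags for a radar return.
; On BeginPlay, two timelines drive the relative yaw of the turret and the relative pitch of the barrel, each restarting when it finishes to loop indefinitely.
; The construction script copies the actor's faction tags into its RadarReturnBPBase.
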(event EventBeginPlay
  ;[1 1 1] Rotate barrel and turret regularly
  (Utilities|FlowControl|Sequence
    (:then_0
      (bind _rotation (Timeline|Turret%20Rot PlayFromStart)
        (:Update
          (Transformation|SetRelativeRotation (Variables|Default|GetTurret) (Math|Rotator|MakeRotator 0.0 0.0 _rotation) false false))
        (:Finished
          (Utilities|FlowControl|Sequence
            (:then_1
              (Timeline|Turret%20Rot PlayFromStart))))))
    (:then_1
      (bind _rotation_2 (Timeline|Barrel%20Rot PlayFromStart)
        (:Update
          (Transformation|SetRelativeRotation (Variables|Default|GetBarrel) (Math|Rotator|MakeRotator 0.0 _rotation_2 0.0) false false))
        (:Finished
          (Utilities|FlowControl|Sequence
            (:then_1
              (Timeline|Barrel%20Rot PlayFromStart))))))))

(fn ConstructionScript
  (Variables|/Game/3D_Radar/Blueprints/Radar_Return_BP.Radar_Return_BP_C|SetFaction%20Tags (Variables|Default|GetRadar_Return_BP_Base) (Variables|Default|GetFactions%20Tags)))