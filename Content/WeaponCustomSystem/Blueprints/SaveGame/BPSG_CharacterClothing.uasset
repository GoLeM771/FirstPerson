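; SaveGame Blueprint for the weapon customization system that stores character clothing data as an array of entries identified by socket name.
; FindDataBySocketName linearly searches the array and returns a found flag with the matching entry.
; AddCharacterClothingData acts as an upsert, overwriting the entry with the same socket name or appending a new one when none matches.
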(fn FindDatabySocketName
  (params (SocketName :type Name))
  (for _array_element (Variables|Info|GetCharacterClothingDataArray)
    (if (Utilities|Name|Equal(Name) (.SocketName (Utilities|Struct|BreakS_CharacterClothingData _array_element)) SocketName)
      (return true _array_element)))
  (return false ""))

(fn AddCharacterClothingData
  (params (Data :type S%20Character%20Clothing%20Data%20Structure%20%28by%20ref%29))
  (Utilities|FlowControl|Sequence
    (:then_0
      (for (_array_element _array_index) (Variables|Info|GetCharacterClothingDataArray)
        (if (Utilities|Name|Equal(Name) (.SocketName (Utilities|Struct|BreakS_CharacterClothingData _array_element)) (.SocketName (Utilities|Struct|BreakS_CharacterClothingData Data)))
          (Utilities|Array|SetArrayElem (Variables|Info|GetCharacterClothingDataArray) _array_index Data)
          (return))))
    (:then_1
      (Utilities|Array|Add (Variables|Info|GetCharacterClothingDataArray) Data)
      (return))))