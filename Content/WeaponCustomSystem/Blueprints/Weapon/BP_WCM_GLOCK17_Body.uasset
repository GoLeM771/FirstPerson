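; BP_WCM_GLOCK17_Body is the Glock 17 body Blueprint in the weapon customization system, providing the pistol's firing animation.
; Its StartFireAnimation event plays the weapon fire sequence on the skeletal mesh as a dynamic montage in the default slot, with no blending in or out.
; The construction script only calls the parent, and BeginPlay, overlap and Tick are disabled stubs.
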(event EventBeginPlay
  (|CallParentFunction) ; 此节点被禁用，将不会被调用。\n从引脚连出引线来编译功能。
)

(event Collision|EventActorBeginOverlap
  (params (OtherActor :type Actor%20Object%20Reference))
  (|CallParentFunction OtherActor) ; 此节点被禁用，将不会被调用。\n从引脚连出引线来编译功能。
)

(event EventTick
  (params (DeltaSeconds :type Float%20%28single-precision%29))
  (|CallParentFunction DeltaSeconds) ; 此节点被禁用，将不会被调用。\n从引脚连出引线来编译功能。
)

(event EventStartFireAnimation
  (Class|AnimInstance|PlaySlotAnimationasDynamicMontage (Components|SkeletalMesh|GetAnimInstance (Variables|Default|GetSkeletalMesh)) "/Game/WeaponCustomSystem/Animations/AnimSequence/Weapon/GLOCK17/AS_GLOCK17_Fire_Weapon.AS_GLOCK17_Fire_Weapon" "DefaultSlot" 0.0 0.0 1.0 1 -1.0 0.0))

(fn ConstructionScript
  (|CallParentFunction))