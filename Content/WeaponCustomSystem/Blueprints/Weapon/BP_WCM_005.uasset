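; BP_WCM_005 is a weapon customization Blueprint serving as an example of how to use CustomWeaponActionComponent, here to switch a light on and off.
; On BeginPlay it creates a dynamic material instance for the second material slot of its static mesh.
; The component's ToggleAction event sets the Light's visibility and drives that material's "Param" scalar between high and zero to match the on/off state.
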(event ToggleAction(BP_CustomWeaponActionComponent)
  (params (Status :type Boolean))
  ;[1 1 1] Example-1 How To Use CustomWeaponActionComponent
  (Rendering|SetVisibility (Variables|Default|GetLight) Status false)
  (if Status
    (Rendering|Material|SetScalarParameterValue (Variables|Default|GetMAT) "Param" 1e+03 :!class /Script/Engine.MaterialInstanceDynamic)
    (else
      (Rendering|Material|SetScalarParameterValue (Variables|Default|GetMAT) "Param" 0.0 :!class /Script/Engine.MaterialInstanceDynamic))))

(event EventBeginPlay
  ;[1 1 1] Example-1 How To Use CustomWeaponActionComponent
  (|CallParentFunction)
  (bind _returnvalue (Rendering|Material|CreateDynamicMaterialInstance (Rendering|Material|GetMaterial (Variables|Default|GetStaticMesh) 1) "None" :!class /Script/Engine.KismetMaterialLibrary))
  (bind _output_get (Variables|Default|SetMAT _returnvalue))
  (Rendering|Material|SetMaterial (Variables|Default|GetStaticMesh) 1 _output_get))

(fn ConstructionScript
  (|CallParentFunction))