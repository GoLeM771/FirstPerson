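; Weapon Blueprint in the weapon customization system that handles its own muzzle flash effect.
; Fire start and stop events activate and deactivate the Muzzle component, randomizing its world scale per axis on each activation for variation.
; A silencer-attached event sets a flag that makes both events skip the flash; nothing in this file clears it.
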(event EventBeginPlay
  (|CallParentFunction))

(event Collision|EventActorBeginOverlap
  (params (OtherActor :type Actor%20Object%20Reference))
  (|CallParentFunction OtherActor) ; 此节点被禁用，将不会被调用。\n从引脚连出引线来编译功能。
)

(event EventTick
  (params (DeltaSeconds :type Float%20%28single-precision%29))
  (|CallParentFunction DeltaSeconds) ; 此节点被禁用，将不会被调用。\n从引脚连出引线来编译功能。
)

(event EventStartMuzzleFlashParticleFire
  (bind _returnvalue (Math|Random|RandomFloatinRange 1.0 0.7))
  (bind _muzzle (Variables|Default|GetMuzzle))
  (if (not (Variables|Default|GetSilencerAttached?))
    (Components|Activation|Activate _muzzle true)
    (Transformation|SetWorldScale3D _muzzle (Math|Vector|MakeVector _returnvalue _returnvalue _returnvalue))))

(event EventStopMuzzleFlashParticleFire
  (if (not (Variables|Default|GetSilencerAttached?))
    (Components|Activation|Deactivate (Variables|Default|GetMuzzle))))

(event EventSilencerAttachedInterface
  (Variables|Default|SetSilencerAttached? true))

(fn ConstructionScript
  (|CallParentFunction))