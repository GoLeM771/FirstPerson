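; Manager that builds a modular weapon from a SaveGame preset and tracks its sight and action components.
; SpawnWeapon spawns the base under a root transform actor, then attaches parts through an ID-to-actor map, restoring their saved data.
; An optional backward sphere trace drops sights with something behind them.
; Other functions cycle active sights and actions through their widgets, expose weapon data, and recursively destroy the assembly.
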(event EventBeginPlay)

(event EventTick
  (params (DeltaSeconds :type Float%20%28single-precision%29)))

(fn SpawnWeapon
  (params (SaveGameSlotName :type String) (PresetIndex :type Integer) (CheckBlock :type Boolean))
  (Utilities|Array|Clear (Variables|Default|GetWeaponComponents))
  (Utilities|Array|Clear (Variables|SightPoint|GetSightPointWeaponComponents))
  (Utilities|FlowControl|Sequence
    (:then_0
      ;[1 1 1] (获取SaveGame，然后生成一个基础的武器组件)
      ; Get SaveGame and generate a basic weapon component
      (bind _returnvalue (SaveGame|LoadGamefromSlot SaveGameSlotName))
      (bind _asbpsg_weapon_component_spawn (Utilities|Casting|CastToBPSG_WeaponComponentSpawn _returnvalue))
      (LocalVariables|SetL_SaveGame _asbpsg_weapon_component_spawn)
      (bind _presetdata (Default|GetPresetData (LocalVariables|GetL_SaveGame)))
      (bind _output_get (LocalVariables|SetL_PresetData (Utilities|Array|Get(acopy) _presetdata PresetIndex)))
      (Variables|Default|SetCurrentWeaponData _output_get))
    (:then_1
      (bind _returnvalue_2 (Game|SpawnActorfromClass "/Game/WeaponCustomSystem/Blueprints/Weapon/BP_TransformActor.BP_TransformActor_C" (Math|Transform|MakeTransform "0, 0, 0" "0, 0, 0" "1,1,1") "Undefined" 0 0))
      (Variables|Default|SetRootTransformActor _returnvalue_2)
      (bind _returnvalue_3 (Game|SpawnActorfromClass (.BaseWeaponComponentClass (Utilities|Struct|BreakS_PresetData (LocalVariables|GetL_PresetData))) (Math|Transform|MakeTransform "0, 0, 0" "0, 0, 0" "1,1,1") "Undefined" 0 0))
      (bind _output_get_2 (LocalVariables|SetL_CurrentWeaponMainComponent _returnvalue_3))
      (Utilities|Array|Add (Variables|Default|GetWeaponComponents) _output_get_2)
      (Utilities|Map|Add (LocalVariables|GetL_Index_Actor) 0 (LocalVariables|GetL_CurrentWeaponMainComponent))
      (Transformation|AttachActorToActor (LocalVariables|GetL_CurrentWeaponMainComponent) (Variables|Default|GetRootTransformActor) "None" "SnapToTarget" "SnapToTarget" "SnapToTarget" true))
    (:then_2
      (for _array_element (.WeaponComponentSpawnDatas (Utilities|Struct|BreakS_PresetData (LocalVariables|GetL_PresetData)))
        (LocalVariables|SetL_WeaponComponentSpawnData _array_element)
        (Utilities|FlowControl|Sequence
          (:then_0
            ;[1 1 1] (通过CurrentID找到WeaponComponent，该WeaponComponent就是接下来要被附着的WeaponComponent)
            ; WeaponComponent is found by CurrentID, which is the WeaponComponent to be attached next
            (LocalVariables|SetL_WeaponComponent (.Value (Utilities|Map|Find (LocalVariables|GetL_Index_Actor) (Utilities|Struct|BreakS_WeaponComponentSocketData (Utilities|Struct|BreakS_WeaponComponentSpawnData (LocalVariables|GetL_WeaponComponentSpawnData)))))))
          (:then_1
            ;[1 1 1] （获取附着点的Actor,然后修改相对位置）
            ; Get the actor of the attachment point and modify the relative position
            (bind _customcomponent (Class|BPIPublicWeaponInterface|GetCustomComponent(Message) (LocalVariables|GetL_WeaponComponent)))
            (bind _transformactor (Default|FindTransfromActorbySocketData _customcomponent (Utilities|Struct|BreakS_WeaponComponentSpawnData (LocalVariables|GetL_WeaponComponentSpawnData))))
            (bind _output_get_3 (LocalVariables|SetL_TransformActor _transformactor))
            (Transformation|AddActorWorldOffset _output_get_3 (* (Utilities|Struct|BreakS_WeaponComponentSocketData (Utilities|Struct|BreakS_WeaponComponentSpawnData (LocalVariables|GetL_WeaponComponentSpawnData))) -1.0)))
          (:then_2
            ;[1 1 1] （生成组件并附着到上面获取的Actor中）
            ; Generate a component and attach it to the Actor obtained above
            (bind _returnvalue_4 (Game|SpawnActorfromClass (Utilities|Struct|BreakS_WeaponComponentData (Utilities|Struct|BreakS_WeaponComponentSpawnData (LocalVariables|GetL_WeaponComponentSpawnData))) (Math|Transform|MakeTransform "0, 0, 0" "0, 0, 0" "1,1,1") "Undefined" 0 0))
            (LocalVariables|SetL_CurrentPinWeaponComponent _returnvalue_4)
            (Utilities|FlowControl|Sequence
              (:then_0
                (bind _customcomponent_2 (Class|BPIPublicWeaponInterface|GetCustomComponent(Message) (LocalVariables|GetL_CurrentPinWeaponComponent)))
                (Default|AttachtoTransfromActor _customcomponent_2 (Variables|/Script/Engine.Actor|GetRootComponent (LocalVariables|GetL_TransformActor))))
              (:then_1
                ;[1 1 1] Reback Save Data
                (CallFunction|UpdateWeaponComponentData (LocalVariables|GetL_WeaponComponentSpawnData) (LocalVariables|GetL_CurrentPinWeaponComponent)))
              (:then_2
                (Utilities|Array|Add (Variables|Default|GetWeaponComponents) (LocalVariables|GetL_CurrentPinWeaponComponent)))))
          (:then_3
            ;[1 1 1] 添加数据
            ; adding data
            (Utilities|Map|Add (LocalVariables|GetL_Index_Actor) (Utilities|Struct|BreakS_WeaponComponentSocketData (Utilities|Struct|BreakS_WeaponComponentSpawnData (LocalVariables|GetL_WeaponComponentSpawnData))) (LocalVariables|GetL_CurrentPinWeaponComponent)))
          (:then_4
            ;[1 1 1] 获取拥有瞄准点的组件
            ; Get component with SightPoint
            (bind _customcomponent_3 (Class|BPIPublicWeaponInterface|GetCustomComponent(Message) (LocalVariables|GetL_CurrentPinWeaponComponent)))
            (bind _return (Default|HasSocket _customcomponent_3 "SightPoint"))
            (if _return
              (Utilities|Array|Add (Variables|SightPoint|GetSightPointWeaponComponents) (LocalVariables|GetL_CurrentPinWeaponComponent))))
          (:then_5
            ;[1 1 1] 获取拥有动作的组件
            ; Get ActionComponent
            (bind _component (Class|BPIPublicWeaponInterface|GetActionComponent(Message) (LocalVariables|GetL_CurrentPinWeaponComponent)))
            (Utilities|IsValid _component
              (:Is%20Valid
                (Utilities|Array|Add (Variables|ActionComponent|GetActionWeaponComponents) (LocalVariables|GetL_CurrentPinWeaponComponent))))))))
    (:then_3
      (if CheckBlock
        ;[1 1 1] 武器向前的方向
        ; Weapon forward direction
        (LocalVariables|SetL_ForwardVector (Math|Vector|GetForwardVector (Transformation|GetActorRotation (LocalVariables|GetL_CurrentWeaponMainComponent))))
        (for _array_element_2 (Variables|SightPoint|GetSightPointWeaponComponents)
          (bind _output_get_4 (LocalVariables|SetL_WeaponComponent _array_element_2))
          (bind _customcomponent_4 (Class|BPIPublicWeaponInterface|GetCustomComponent(Message) _output_get_4))
          ;[1 1 1] 先往后发出射线，如果检测不到碰撞说明它不是最靠前的瞄准点
          ; Fires LineTrace backwards, if no collision is detected, it is not the most forward aiming point
          (LocalVariables|SetL_CurrentLocation_ (Default|GetSocketLocation _customcomponent_4 "SightPoint"))
          (bind _returnvalue_5 (Collision|SphereTraceForObjects (LocalVariables|GetL_CurrentLocation_) (+ (LocalVariables|GetL_CurrentLocation_) (* (LocalVariables|GetL_ForwardVector) -1e+03)) 0.5 (Utilities|Array|MakeArray "ObjectTypeQuery7") true (Utilities|Array|MakeArray (LocalVariables|GetL_WeaponComponent)) "None"))
          (if (not _returnvalue_5)
            (Utilities|Array|Add (LocalVariables|GetL_SightWeaponComponent_Result) (LocalVariables|GetL_WeaponComponent))))
        (Variables|SightPoint|SetSightPointWeaponComponents (LocalVariables|GetL_SightWeaponComponent_Result))))
    (:then_4
      ;[1 1 1] 基本上用来获取相对位置
      ; Basically used to get the relative position
      (for _array_element_3 (Variables|Default|GetWeaponComponents)
        (bind _customcomponent_5 (Class|BPIPublicWeaponInterface|GetCustomComponent(Message) _array_element_3))
        (Variables|/Game/WeaponCustomSystem/Blueprints/Weapon/CustomComponent/BP_CustomComponent.BP_CustomComponent_C|SetRootParentActor _customcomponent_5 (Variables|Default|GetRootTransformActor))))))

(fn GetSightPointComponent
  (params (Status :type Boolean))
  (for _array_element (Variables|SightPoint|GetSightPointWeaponComponents)
    (bind _component (Class|BPIPublicWeaponInterface|GetActionComponent(Message) _array_element))
    (Utilities|IsValid _component
      (:Is%20Valid
        (if (Math|Boolean|Equal(Boolean) (Variables|/Game/WeaponCustomSystem/Blueprints/Weapon/CustomComponent/BP_ActionComponent.BP_ActionComponent_C|GetStatus _component) Status)
          (Utilities|Array|Add (LocalVariables|GetL_Array) _array_element :!label _label)))
      (:Is%20Not%20Valid
        (goto _label))))
  (return (LocalVariables|GetL_Array)))

(fn SwitchSightPointComponent
  (params (CurrentSightPointComponents :type Array%20of%20Actor%20Object%20References))
  (if (> (Utilities|Array|Length CurrentSightPointComponents) 0)
    (Variables|SightPoint|SetCurrentSightIndex (Math|Integer|%(Integer) (+ (Variables|SightPoint|GetCurrentSightIndex) 1) (Utilities|Array|Length CurrentSightPointComponents)))
    (Utilities|FlowControl|Sequence
      (:then_0
        (for _array_element CurrentSightPointComponents
          (bind _component (Class|BPIPublicWeaponInterface|GetSelectADSComponent(Message) _array_element))
          (bind _widget (Default|GetWidget _component))
          (Default|EventClosePlay _widget)))
      (:then_1
        (bind _component_2 (Class|BPIPublicWeaponInterface|GetSelectADSComponent(Message) (Utilities|Array|Get(acopy) CurrentSightPointComponents (Variables|SightPoint|GetCurrentSightIndex))))
        (bind _widget_2 (Default|GetWidget _component_2))
        (Default|EventStartPlay _widget_2)))))

(fn GetCurrentSightPointComponent
  (bind _sightcopm (Get|GetSightPointComponent true))
  (for _array_element _sightcopm
    (bind _component (Class|BPIPublicWeaponInterface|GetSelectADSComponent(Message) _array_element))
    (Utilities|IsValid _component
      (:Is%20Valid
        (if (Variables|/Game/WeaponCustomSystem/Blueprints/Weapon/CustomComponent/BP_SelectADSComponent.BP_SelectADSComponent_C|GetStatus _component)
          (bind _customcomponent (Class|BPIPublicWeaponInterface|GetCustomComponent(Message) _array_element))
          (return _customcomponent))))))

(fn SwichtActionComponent
  (params (CurrentActionComponents :type Array%20of%20Actor%20Object%20References))
  ;[1 1 1] ToggleAction
  (if (> (Utilities|Array|Length CurrentActionComponents) 0)
    (Variables|ActionComponent|SetActionIndex (Math|Integer|%(Integer) (+ (Variables|ActionComponent|GetActionIndex) 1) (Utilities|Array|Length CurrentActionComponents)))
    (Utilities|FlowControl|Sequence
      (:then_0
        (for _array_element CurrentActionComponents
          (bind _component (Class|BPIPublicWeaponInterface|GetActionComponent(Message) _array_element))
          (bind _widget (Default|GetWidget _component))
          (Default|EventClosePlay _widget)))
      (:then_1
        (bind _component_2 (Class|BPIPublicWeaponInterface|GetActionComponent(Message) (Utilities|Array|Get(acopy) CurrentActionComponents (Variables|ActionComponent|GetActionIndex))))
        (bind _widget_2 (Default|GetWidget _component_2))
        (Default|EventStartPlay _widget_2)))))

(fn SetAimStatus
  (params (IsADS :type Boolean))
  (Variables|ADS|SetIsADS IsADS))

(fn ClearWeapon
  (Spawn|ClearChild (Variables|Default|GetRootTransformActor))
  (Variables|Default|SetRootTransformActor 0)
  (Utilities|Array|Clear (Variables|Default|GetWeaponComponents))
  (Utilities|Array|Clear (Variables|ActionComponent|GetActionWeaponComponents))
  (Utilities|Array|Clear (Variables|SightPoint|GetSightPointWeaponComponents))
  (Variables|ADS|SetIsADS false)
  (Variables|ActionComponent|SetActionIndex 0)
  (Variables|SightPoint|SetCurrentSightIndex 0))

(fn ClearChild
  (params (CurrentActor :type Actor%20Object%20Reference))
  (Utilities|IsValid CurrentActor
    (:Is%20Valid
      (Utilities|FlowControl|Sequence
        (:then_0
          (LocalVariables|SetL_AttachedActors (Actor|GetAttachedActors CurrentActor true))
          (for _array_element (LocalVariables|GetL_AttachedActors)
            (Spawn|ClearChild _array_element)))
        (:then_1
          (Actor|DestroyActor CurrentActor))))))

(fn GetWeaponData
  (return (Variables|Default|GetCurrentWeaponData)))