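; Weapon customization component that represents one part's mesh and its attachment sockets, plus references to its connect-point and pin widgets.
; SetInfo stores the mesh components, then spawns a BP_TransformActor on each configured socket so slot positions can change dynamically.
; The owning actor can attach to such a transform actor, and socket data setters track IDs and offsets.
; Socket queries use the static, skeletal or poseable mesh, with conversions into root or owner space.
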(event Custom|Event_SetConnectPointWidgets
  (params (PointWidgets :type Array%20of%20User%20Widget%20Object%20References))
  (Variables|Widget|SetConnectPointWidgets PointWidgets))

(event Custom|Event_SetPinWidgets
  (params (PinWidgets :type Array%20of%20User%20Widget%20Object%20References))
  (Variables|Widget|SetPinWidgets PinWidgets))

(event EventBeginPlay)

(event EventTick
  (params (DeltaSeconds :type Float%20%28single-precision%29)))

(fn SetInfo
  (params (SkeletalMeshComponent :type Skeletal%20Mesh%20Component%20Object%20Reference) (StaticMeshComponent :type Static%20Mesh%20Component%20Object%20Reference) (PoseableMeshComponent :type Poseable%20Mesh%20Component%20Object%20Reference))
  (Variables|Info|SetSkeletalMeshComponent SkeletalMeshComponent)
  (Variables|Info|SetStaticMeshComponent StaticMeshComponent)
  (Variables|Info|SetPoseableMeshComponent PoseableMeshComponent)
  (Attach|SpawnSocketTransfromActor))

(fn GetMeshComponent
  (Utilities|IsValid (Variables|/Script/Engine.StaticMeshComponent|GetStaticMesh (Variables|Info|GetStaticMeshComponent))
    (:Is%20Valid
      (return (Variables|Info|GetStaticMeshComponent)))
    (:Is%20Not%20Valid
      (Utilities|IsValid (Variables|/Script/Engine.SkinnedMeshComponent|GetSkeletalMesh (Variables|Info|GetSkeletalMeshComponent))
        (:Is%20Valid
          (return (Variables|Info|GetSkeletalMeshComponent)))
        (:Is%20Not%20Valid
          (return (Variables|Info|GetPoseableMeshComponent)))))))

(fn GetSocketLocation
  (params (Name :type Name :default "None"))
  (bind _meshcomponent (Info|GetMeshComponent))
  (Utilities|IsValid _meshcomponent
    (:Is%20Valid
      (if (Transformation|DoesSocketExist _meshcomponent Name)
        (return (Transformation|GetSocketLocation _meshcomponent Name))
        (else
          _)))
    (:Is%20Not%20Valid
      _))
  (return "0, 0, 0"))

(fn SetWeaponComponentSocketData
  (params (SocketData :type S%20Weapon%20Component%20Socket%20Data%20Structure) (Index :type Integer))
  (bind (_slider_leftsocketname _slider_rightsocketname _currentid _nextid _relativelocation) (Utilities|Struct|BreakS_WeaponComponentSocketData SocketData))
  (Utilities|Struct|SetmembersinS_WeaponComponentSocketData (Utilities|Array|Get(acopy) (Variables|Info|GetWeaponComponentSocketData) Index) _currentid _nextid _relativelocation))

(fn GetConnectPointWidgets
  (return (Variables|Widget|GetConnectPointWidgets)))

(fn GetConfigSocketLocation
  (params (Config :type S%20Weapon%20Component%20Socket%20Data%20Structure))
  (bind _transformactor (Utilities|Struct|BreakS_WeaponComponentSocketData Config))
  (Utilities|IsValid _transformactor
    (:Is%20Valid
      (return (Transformation|GetActorLocation _transformactor)))))

(fn GetPinWidgets
  (return (Variables|Widget|GetPinWidgets)))

(fn GetWeaponComponentSocketData
  (return (Variables|Info|GetWeaponComponentSocketData)))

(fn AttachtoTransfromActor
  (params (TransformActorRootComponent :type Scene%20Component%20Object%20Reference))
  (Transformation|AttachComponentToComponent (Info|GetParentActor) TransformActorRootComponent "None" "KeepRelative" "KeepRelative" "KeepRelative" true))

(fn SpawnSocketTransfromActor
  ;[1 1 1] 用于动态改变插槽位置
  ; For changing slot position dynamically
  (for _index (range 0 (- (Utilities|Array|Length (Variables|Info|GetWeaponComponentSocketData)) 1))
    (LocalVariables|SetL_Index _index)
    (bind _returnvalue (Game|SpawnActorfromClass "/Game/WeaponCustomSystem/Blueprints/Weapon/BP_TransformActor.BP_TransformActor_C" (Math|Transform|MakeTransform "0, 0, 0" "0, 0, 0" "1,1,1") "Undefined" 0 0))
    (Transformation|AttachComponentToComponent _returnvalue (Info|GetMeshComponent) (.WeaponSocketName (Utilities|Struct|BreakS_WeaponComponentSocketData (Utilities|Array|Get(acopy) (Variables|Info|GetWeaponComponentSocketData) (LocalVariables|GetL_Index)))) "KeepRelative" "KeepRelative" "KeepWorld" true)
    (Utilities|Struct|SetmembersinS_WeaponComponentSocketData (Utilities|Array|Get(acopy) (Variables|Info|GetWeaponComponentSocketData) (LocalVariables|GetL_Index)) _returnvalue)))

(fn GetParentActor
  (return (Components|GetOwner)))

(fn GetSocketRootComponent
  (params (Config :type S%20Weapon%20Component%20Socket%20Data%20Structure))
  (return (Variables|/Script/Engine.Actor|GetRootComponent (.TransformActor (Utilities|Struct|BreakS_WeaponComponentSocketData Config)))))

(fn SetCurrentIDSocketData
  (params (ID :type Integer))
  (for _index (range 0 (- (Utilities|Array|Length (Variables|Info|GetWeaponComponentSocketData)) 1))
    (Utilities|Struct|SetmembersinS_WeaponComponentSocketData (Utilities|Array|Get(acopy) (Variables|Info|GetWeaponComponentSocketData) _index) ID)))

(fn SetNextIDSocketData
  (params (NextID :type Integer) (Index :type Integer))
  (Utilities|Struct|SetmembersinS_WeaponComponentSocketData (Utilities|Array|Get(acopy) (Variables|Info|GetWeaponComponentSocketData) Index) NextID))

(fn SetRelativeLocationSocketData
  (params (Index :type Integer) (RelativeLocation :type Vector))
  (Utilities|Struct|SetmembersinS_WeaponComponentSocketData (Utilities|Array|Get(acopy) (Variables|Info|GetWeaponComponentSocketData) Index) RelativeLocation))

(fn FindTransfromActorbySocketData
  (params (SocketData :type S%20Weapon%20Component%20Socket%20Data%20Structure))
  (bind (_weaponcomponenttype _weaponmatchcode _weaponsocketname) (Utilities|Struct|BreakS_WeaponComponentSocketData SocketData))
  (for _array_element (Variables|Info|GetWeaponComponentSocketData)
    (if (Math|Boolean|ANDBoolean (== (.WeaponComponentType (Utilities|Struct|BreakS_WeaponComponentSocketData _array_element)) _weaponcomponenttype) (== (.WeaponMatchCode (Utilities|Struct|BreakS_WeaponComponentSocketData _array_element)) _weaponmatchcode) (Utilities|Name|Equal(Name) (.WeaponSocketName (Utilities|Struct|BreakS_WeaponComponentSocketData _array_element)) _weaponsocketname))
      (return (.TransformActor (Utilities|Struct|BreakS_WeaponComponentSocketData _array_element))))))

(fn GetSocketRotation
  (params (Name :type Name))
  (bind _meshcomponent (Info|GetMeshComponent))
  (Utilities|IsValid _meshcomponent
    (:Is%20Valid
      (if (Transformation|DoesSocketExist _meshcomponent Name)
        (return (Transformation|GetSocketRotation _meshcomponent Name))
        (else
          _)))
    (:Is%20Not%20Valid
      _))
  (return "0, 0, 0"))

(fn HasSocket
  (params (InSocketName :type Name))
  (Utilities|IsValid (Info|GetMeshComponent)
    (:Is%20Valid
      (return (Transformation|DoesSocketExist (Info|GetMeshComponent) InSocketName)))
    (:Is%20Not%20Valid
      (return false))))

(fn GetRelativeSocketLocationRoot
  (params (Name :type Name) (RotateVector :type Rotator :default "0,0.000000,0"))
  (return (Math|Vector|RotateVector (Math|Transform|InverseTransformLocation (Transformation|GetActorTransform (Variables|Parent|GetRootParentActor)) (Transform|GetSocketLocation Name)) RotateVector)))

(fn GetRelativeSocketRotationRoot
  (params (Name :type Name) (RotateVector :type Rotator :default "0,0.000000,0"))
  (return (Math|Rotator|CombineRotators (Math|Transform|InverseTransformRotation (Transformation|GetActorTransform (Variables|Parent|GetRootParentActor)) (Transform|GetSocketRotation Name)) RotateVector)))

(fn GetRelativeSocketLocationSelf
  (params (Name :type Name) (RotateVector :type Rotator :default "0,0.000000,0"))
  (return (Math|Vector|RotateVector (Math|Transform|InverseTransformLocation (Transformation|GetActorTransform (Components|GetOwner)) (Transform|GetSocketLocation Name)) RotateVector)))

(fn ConveLocationtoRelativeLocationRoot
  (params (RotateVector :type Rotator :default "0,0.000000,0") (Location :type Vector))
  (return (Math|Vector|RotateVector (Math|Transform|InverseTransformLocation (Transformation|GetActorTransform (Variables|Parent|GetRootParentActor)) Location) RotateVector)))