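; BP_ClothingComponent turns a clothing mesh's custom sockets into attachment points for the weapon customization system.
; SetInfo stores skeletal, static and poseable mesh references, then spawns a BP_TransformActor_Clothing snapped to each "CWM_" socket on the active mesh.
; GetMeshComponent picks that mesh, preferring static, then skeletal, then poseable.
; The spawned actors are tracked so customization widgets can be shown or weapons destroyed across all of them.
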(event EventBeginPlay)

(event EventTick
  (params (DeltaSeconds :type Float%20%28single-precision%29)))

(fn SpawnSocketTransfromActor
  (Utilities|FlowControl|Sequence
    (:then_0
      ;[1 1 1] 获取自定义的插槽
      ; Get a custom socket
      (for _array_element (Transformation|GetAllSocketNames (Info|GetMeshComponent))
        (if (Utilities|String|Contains (Utilities|String|ToString(Name) _array_element) "CWM_")
          (Utilities|Array|Add (Variables|Default|GetCWMS) _array_element))))
    (:then_1
      (for _array_element_2 (Variables|Default|GetCWMS)
        (bind _returnvalue (Game|SpawnActorfromClass "/Game/WeaponCustomSystem/Blueprints/Weapon/BP_TransformActor_Clothing.BP_TransformActor_Clothing_C" (Math|Transform|MakeTransform "0, 0, 0" "0, 0, 0" "1,1,1") "Undefined" 0 0))
        (LocalVariables|SetL_CurrentTransformActor _returnvalue)
        (Transformation|AttachComponentToComponent (LocalVariables|GetL_CurrentTransformActor) (Info|GetMeshComponent) _array_element_2 "SnapToTarget" "SnapToTarget" "SnapToTarget" true)
        (Default|SetInfo (LocalVariables|GetL_CurrentTransformActor) _array_element_2)
        (Utilities|Array|Add (Variables|Default|GetTransformActors) (LocalVariables|GetL_CurrentTransformActor))))))

(fn GetMeshComponent
  (Utilities|IsValid (Variables|Default|GetStaticMeshComponent)
    (:Is%20Valid
      (Utilities|IsValid (Variables|/Script/Engine.StaticMeshComponent|GetStaticMesh (Variables|Default|GetStaticMeshComponent))
        (:Is%20Valid
          (return (Variables|Default|GetStaticMeshComponent)))
        (:Is%20Not%20Valid
          (Utilities|IsValid (Variables|/Script/Engine.SkinnedMeshComponent|GetSkeletalMesh (Variables|Default|GetSkeletalMeshComponent)) :!label _label
            (:Is%20Valid
              _)
            (:Is%20Not%20Valid
              (return (Variables|Default|GetPoseableMeshComponent)))))))
    (:Is%20Not%20Valid
      (Utilities|IsValid (Variables|Default|GetSkeletalMeshComponent)
        (:Is%20Valid
          (goto _label))
        (:Is%20Not%20Valid
          (return (Variables|Default|GetPoseableMeshComponent))))))
  (return (Variables|Default|GetSkeletalMeshComponent)))

(fn SetInfo
  (params (SkeletalMeshComponent :type Skeletal%20Mesh%20Component%20Object%20Reference) (StaticMeshComponent :type Static%20Mesh%20Component%20Object%20Reference) (PoseableMeshComponent :type Poseable%20Mesh%20Component%20Object%20Reference))
  (Variables|Default|SetSkeletalMeshComponent SkeletalMeshComponent)
  (Variables|Default|SetStaticMeshComponent StaticMeshComponent)
  (Variables|Default|SetPoseableMeshComponent PoseableMeshComponent)
  (Attach|SpawnSocketTransfromActor))

(fn RemoveAllWeapon
  (for _array_element (Variables|Default|GetTransformActors)
    (bind _asbp_transform_actor_clothing (Utilities|Casting|CastToBP_TransformActor_Clothing _array_element))
    (Default|DestroyWeapon _asbp_transform_actor_clothing)))

(fn ShowCustomWidget
  (params (Min :type Float%20%28single-precision%29) (Max :type Float%20%28single-precision%29))
  (for _array_element (Variables|Default|GetTransformActors)
    (bind _asbp_transform_actor_clothing (Utilities|Casting|CastToBP_TransformActor_Clothing _array_element))
    (Default|SpawnWidget _asbp_transform_actor_clothing Min Max)))