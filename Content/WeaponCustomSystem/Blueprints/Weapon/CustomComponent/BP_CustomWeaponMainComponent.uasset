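; Main component actor of a customizable weapon, handling its fire audio and tracking sight and silencer attachments.
; On BeginPlay it messages the player character to clear the melee-equipped flag.
; Shoot and empty-ammo sounds play only while the weapon is in character hands, and an attached silencer mutes the shoot sound.
; A counter check approves only the first sight install, and a getter exposes the main component.
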(event EventBeginPlay
  (|CallParentFunction)
  (CallFunction|SetMeleWeaponBool))

(event Collision|EventActorBeginOverlap
  (params (OtherActor :type Actor%20Object%20Reference))
  (|CallParentFunction OtherActor) ; 此节点被禁用，将不会被调用。\n从引脚连出引线来编译功能。
)

(event EventTick
  (params (DeltaSeconds :type Float%20%28single-precision%29))
  (|CallParentFunction DeltaSeconds) ; 此节点被禁用，将不会被调用。\n从引脚连出引线来编译功能。
)

(event EventWeaponinCharacterHands?
  (params (InChaacterHands? :type Boolean))
  (Variables|Default|SetWeaponInCharacteHands? InChaacterHands?))

(event EventShootAudioEvent
  (if (Variables|Default|GetWeaponInCharacteHands?)
    (if (not (Variables|Default|GetSilencerAttached?))
      (Audio|PlaySoundatLocation (Variables|Default|GetShootSound) (Transformation|GetActorLocation) "0, 0, 0" 1.0 1.0 0.0 0 0 0))))

(event EventEmptyAmmoAudioEvent
  (if (Variables|Default|GetWeaponInCharacteHands?)
    (Audio|PlaySoundatLocation (Variables|Default|GetEmptyAmmoSound) (Transformation|GetActorLocation) "0, 0, 0" 1.0 1.0 0.0 0 0 0)))

(event EventSilencerAttachedInterface
  (Variables|Default|SetSilencerAttached? true))

(fn ConstructionScript
  (|CallParentFunction))

(fn GetMainComponent
  (return (Variables|Default|GetBP_MainComponent)))

(fn CheckSightCountBeforeInstall
  (if (== (Variables|Default|GetSightCount) 0)
    (Variables|Default|SetSightCount (+ (Variables|Default|GetSightCount) 1))
    (return true)
    (else
      (return false))))

(fn SetMeleWeaponBool
  (Class|PlayerInterface|MeleWeaponEquipSetter(Message) (Game|GetPlayerCharacter 0) false)
  (return))