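; BP_BasePendant is a base weapon-customization attachment that provides a switchable flashlight.
; On BeginPlay it creates a dynamic material instance from the static mesh's slot 0 material and assigns it to slot 1.
; ToggleFlashlight shows or hides the Light and drives that material's "Param" scalar high or to zero to match.
; A query function reports whether the flashlight is on from the Light's visibility.
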(event EventBeginPlay
  (|CallParentFunction)
  (bind _returnvalue (Rendering|Material|CreateDynamicMaterialInstance (Rendering|Material|GetMaterial (Variables|Default|GetStaticMesh) 0) "None" :!class /Script/Engine.KismetMaterialLibrary))
  (bind _output_get (Variables|Default|SetMAT _returnvalue))
  (Rendering|Material|SetMaterial (Variables|Default|GetStaticMesh) 1 _output_get))

(event Collision|EventActorBeginOverlap
  (params (OtherActor :type Actor%20Object%20Reference))
  (|CallParentFunction OtherActor) ; This node is disabled and will not be called.\nDrag off pins to build functionality.
)

(event EventTick
  (params (DeltaSeconds :type Float%20%28single-precision%29))
  (|CallParentFunction DeltaSeconds) ; This node is disabled and will not be called.\nDrag off pins to build functionality.
)

(fn ConstructionScript
  (|CallParentFunction))

(fn ToggleFlashlight
  (params (bNewVisibility :type Boolean))
  (Rendering|SetVisibility (Variables|Default|GetLight) bNewVisibility false)
  (if bNewVisibility
    (Rendering|Material|SetScalarParameterValue (Variables|Default|GetMAT) "Param" 1e+03 :!class /Script/Engine.MaterialInstanceDynamic)
    (else
      (Rendering|Material|SetScalarParameterValue (Variables|Default|GetMAT) "Param" 0.0 :!class /Script/Engine.MaterialInstanceDynamic))))

(fn FashliteActivated?
  (return (Rendering|IsVisible (Variables|Default|GetLight))))