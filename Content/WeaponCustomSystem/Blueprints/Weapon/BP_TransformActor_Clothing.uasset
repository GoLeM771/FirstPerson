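; Clothing attach-point actor that spawns customized weapons or pendants on a character socket and remembers them in the CharacterClothing save.
; Preset spawns rebuild the component tree from saved preset data, mapping socket IDs to actors under a root transform actor.
; SetInfo restores the saved preset for its socket, while removal recursively destroys attached actors.
; SpawnWidget adds a side-offset focus actor and shows a selection button after a random delay.
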(event Custom|Event_SpawnWidget
  (params (Duration :type Float%20%28single-precision%29))
  (Utilities|FlowControl|Delay Duration)
  (Utilities|IsValid self
    (:Is%20Valid
      (bind _returnvalue (UserInterface|CreateWidget "/Game/WeaponCustomSystem/Blueprints/UI/ClothingComponent/BPW_ClothingComponentButton.BPW_ClothingComponentButton_C"))
      (Default|SetInfo _returnvalue self)
      (UserInterface|SetWidget (Variables|Default|GetWidget) _returnvalue))))

(event EventBeginPlay
  (|CallParentFunction) ; This node is disabled and will not be called.\nDrag off pins to build functionality.
)

(event Collision|EventActorBeginOverlap
  (params (OtherActor :type Actor%20Object%20Reference))
  (|CallParentFunction OtherActor) ; This node is disabled and will not be called.\nDrag off pins to build functionality.
)

(event EventTick
  (params (DeltaSeconds :type Float%20%28single-precision%29))
  (|CallParentFunction DeltaSeconds) ; This node is disabled and will not be called.\nDrag off pins to build functionality.
)

(fn ConstructionScript
  (|CallParentFunction))

(fn SetInfo
  (params (SocketName :type Name))
  (Variables|Default|SetSocketName SocketName)
  ;[1 1 1] Reback
  (bind _asbpsg_character_clothing (Utilities|Casting|CastToBPSG_CharacterClothing (CallFunction|GetSaveGame "CharacterClothing" 0 "/Game/WeaponCustomSystem/Blueprints/SaveGame/BPSG_CharacterClothing.BPSG_CharacterClothing_C")))
  (bind (_find _element) (Default|FindDatabySocketName _asbpsg_character_clothing (Variables|Default|GetSocketName)))
  (if _find
    (if (.IsSpawn (Utilities|Struct|BreakS_CharacterClothingData _element))
      (bind _roottransformactor (Weapon|SpawnWeaponbyPresetName (.PresetName (Utilities|Struct|BreakS_CharacterClothingData _element))))
      (Transformation|AttachActorToActor _roottransformactor self "None" "SnapToTarget" "SnapToTarget" "SnapToTarget" true))))

(fn SpawnWeapon
  (params (PresetIndex :type Integer))
  (Utilities|FlowControl|Sequence
    (:then_0
      (Utilities|FlowControl|Sequence
        (:then_0
          ;[1 1 1] (获取SaveGame，然后生成一个基础的武器组件)
          ; Get SaveGame and generate a basic weapon component
          (bind _asnew_fps_save_game (Utilities|Casting|CastToNew_FPS_SaveGame (CallFunction|GetSaveGame "GigahruchRogueLike" 0 "/Game/Blueprints/SaveGameBlueprint/New_FPS_SaveGame.New_FPS_SaveGame_C")))
          (LocalVariables|SetL_SaveGame _asnew_fps_save_game)
          (bind _presetdataarrey (Default|GetPresetData (LocalVariables|GetL_SaveGame)))
          (LocalVariables|SetL_PresetData (Utilities|Array|Get(acopy) _presetdataarrey PresetIndex))
          (Variables|Default|SetPresetName (.PresetName (Utilities|Struct|BreakS_PresetData (LocalVariables|GetL_PresetData)))))
        (:then_1
          (bind _returnvalue (Game|SpawnActorfromClass "/Game/WeaponCustomSystem/Blueprints/Weapon/BP_TransformActor.BP_TransformActor_C" (Math|Transform|MakeTransform "0, 0, 0" "0, 0, 0" "1,1,1") "Undefined" 0 0))
          (Variables|Default|SetRootTransformActor _returnvalue)
          (bind _returnvalue_2 (Game|SpawnActorfromClass (.BaseWeaponComponentClass (Utilities|Struct|BreakS_PresetData (LocalVariables|GetL_PresetData))) (Math|Transform|MakeTransform "0, 0, 0" "0, 0, 0" "1,1,1") "Undefined" 0 0))
          (bind _output_get (Variables|Default|SetCurrentWeaponMainComponent _returnvalue_2))
          (Utilities|Array|Add (LocalVariables|GetL_WeaponComponents) _output_get)
          (Utilities|Map|Add (LocalVariables|GetL_Index_Actor) 0 (Variables|Default|GetCurrentWeaponMainComponent))
          (Transformation|AttachActorToActor (Variables|Default|GetCurrentWeaponMainComponent) (Variables|Default|GetRootTransformActor) "None" "KeepRelative" "KeepRelative" "KeepRelative" true))
        (:then_2
          (for _array_element (.WeaponComponentSpawnDatas (Utilities|Struct|BreakS_PresetData (LocalVariables|GetL_PresetData)))
            (LocalVariables|SetL_WeaponComponentSpawnData _array_element)
            (Utilities|FlowControl|Sequence
              (:then_0
                ;[1 1 1] (通过CurrentID找到WeaponComponent，该WeaponComponent就是接下来要被附着的WeaponComponent)
                ; WeaponComponent is found by CurrentID, which is the WeaponComponent to be attached next
                (LocalVariables|SetL_WeaponComponent (.Value (Utilities|Map|Find (LocalVariables|GetL_Index_Actor) (Utilities|Struct|BreakS_WeaponComponentSocketData (Utilities|Struct|BreakS_WeaponComponentSpawnData (LocalVariables|GetL_WeaponComponentSpawnData)))))))
              (:then_1
                ;[1 1 1] （获取附着点的Actor,然后修改相对位置）
                ; Get the actor of the attachment point and modify the relative position
                (bind _customcomponent (Class|BPIPublicWeaponInterface|GetCustomComponent(Message) (LocalVariables|GetL_WeaponComponent)))
                (bind _transformactor (Default|FindTransfromActorbySocketData _customcomponent (Utilities|Struct|BreakS_WeaponComponentSpawnData (LocalVariables|GetL_WeaponComponentSpawnData))))
                (bind _output_get_2 (LocalVariables|SetL_TransformActor _transformactor))
                (Transformation|AddActorWorldOffset _output_get_2 (* (Utilities|Struct|BreakS_WeaponComponentSocketData (Utilities|Struct|BreakS_WeaponComponentSpawnData (LocalVariables|GetL_WeaponComponentSpawnData))) -1.0)))
              (:then_2
                ;[1 1 1] （生成组件并附着到上面获取的Actor中）
                ; Generate a component and attach it to the Actor obtained above
                (bind _returnvalue_3 (Game|SpawnActorfromClass (.ComponentClass (Utilities|Struct|BreakS_WeaponComponentData (Utilities|Struct|BreakS_WeaponComponentSpawnData (LocalVariables|GetL_WeaponComponentSpawnData)))) (Math|Transform|MakeTransform "0, 0, 0" "0, 0, 0" "1,1,1") "Undefined" 0 0))
                (LocalVariables|SetL_CurrentPinWeaponComponent _returnvalue_3)
                (Utilities|FlowControl|Sequence
                  (:then_0
                    (bind _customcomponent_2 (Class|BPIPublicWeaponInterface|GetCustomComponent(Message) (LocalVariables|GetL_CurrentPinWeaponComponent)))
                    (Default|AttachtoTransfromActor _customcomponent_2 (Variables|/Script/Engine.Actor|GetRootComponent (LocalVariables|GetL_TransformActor))))
                  (:then_1
                    ;[1 1 1] Reback Save Data
                    (CallFunction|UpdateWeaponComponentData (LocalVariables|GetL_WeaponComponentSpawnData) (LocalVariables|GetL_CurrentPinWeaponComponent)))
                  (:then_2
                    (Utilities|Array|Add (LocalVariables|GetL_WeaponComponents) (LocalVariables|GetL_CurrentPinWeaponComponent)))))
              (:then_3
                ;[1 1 1] 添加数据
                ; adding data
                (Utilities|Map|Add (LocalVariables|GetL_Index_Actor) (Utilities|Struct|BreakS_WeaponComponentSocketData (Utilities|Struct|BreakS_WeaponComponentSpawnData (LocalVariables|GetL_WeaponComponentSpawnData))) (LocalVariables|GetL_CurrentPinWeaponComponent))))))
        (:then_3
          ;[1 1 1] 基本上用来获取相对位置
          ; Basically used to get the relative position
          (for _array_element_2 (LocalVariables|GetL_WeaponComponents)
            (bind _customcomponent_3 (Class|BPIPublicWeaponInterface|GetCustomComponent(Message) _array_element_2))
            (Variables|/Game/WeaponCustomSystem/Blueprints/Weapon/CustomComponent/BP_CustomComponent.BP_CustomComponent_C|SetRootParentActor _customcomponent_3 (Variables|Default|GetRootTransformActor))))
        (:then_4
          ;[1 1 1] 保存身上的挂件或武器到savegame
          ; Save your pendant or weapon to savegame
          (bind _asbpsg_character_clothing (Utilities|Casting|CastToBPSG_CharacterClothing (CallFunction|GetSaveGame "CharacterClothing" 0 "/Game/WeaponCustomSystem/Blueprints/SaveGame/BPSG_CharacterClothing.BPSG_CharacterClothing_C")))
          (LocalVariables|SetL_CharacterClothing_SaveGame _asbpsg_character_clothing)
          (Default|AddCharacterClothingData (LocalVariables|GetL_CharacterClothing_SaveGame) (Utilities|Struct|MakeS_CharacterClothingData (Variables|Default|GetSocketName) true (Variables|Default|GetPresetName)))
          (CallFunction|UpdateSaveGame "CharacterClothing" 0 (LocalVariables|GetL_CharacterClothing_SaveGame)))))
    (:then_1
      (Variables|Default|SetWeaponComponents (LocalVariables|GetL_WeaponComponents))
      (return (LocalVariables|GetL_WeaponComponents) (Variables|Default|GetRootTransformActor)))))

(fn RemoveWeapon
  (Utilities|IsValid (Variables|Default|GetRootTransformActor)
    (:Is%20Valid
      (Utilities|FlowControl|Sequence
        (:then_0
          (Weapon|FindAttachedActors (Variables|Default|GetRootTransformActor))
          (Variables|Default|SetRootTransformActor 0)
          (Variables|Default|SetCurrentWeaponMainComponent 0)
          (Utilities|Array|Clear (Variables|Default|GetWeaponComponents)))
        (:then_1
          ;[1 1 1] 保存身上的挂件或武器到savegame
          ; Save your pendant or weapon to savegame
          (bind _asbpsg_character_clothing (Utilities|Casting|CastToBPSG_CharacterClothing (CallFunction|GetSaveGame "CharacterClothing" 0 "/Game/WeaponCustomSystem/Blueprints/SaveGame/BPSG_CharacterClothing.BPSG_CharacterClothing_C")))
          (LocalVariables|SetL_CharacterClothing_SaveGame _asbpsg_character_clothing)
          (Default|AddCharacterClothingData (LocalVariables|GetL_CharacterClothing_SaveGame) (Utilities|Struct|MakeS_CharacterClothingData (Variables|Default|GetSocketName) false (Variables|Default|GetPresetName)))
          (CallFunction|UpdateSaveGame "CharacterClothing" 0 (LocalVariables|GetL_CharacterClothing_SaveGame)))))))

(fn FindAttachedActors
  (params (CurrentActor :type Actor%20Object%20Reference))
  (Utilities|FlowControl|Sequence
    (:then_0
      (LocalVariables|SetL_CurrentAttachedActors (Actor|GetAttachedActors CurrentActor true))
      (for _array_element (LocalVariables|GetL_CurrentAttachedActors)
        (Weapon|FindAttachedActors _array_element)))
    (:then_1
      (Actor|DestroyActor CurrentActor))))

(fn SpawnFocusActor
  (bind _returnvalue (Transformation|GetActorLocation))
  (bind _returnvalue_2 (Transformation|GetActorRightVector))
  (bind _returnvalue_3 (* _returnvalue_2 5e+01))
  (bind _returnvalue_4 (+ _returnvalue _returnvalue_3))
  (bind _returnvalue_5 (Game|SpawnActorfromClass "/Game/WeaponCustomSystem/Blueprints/Weapon/BP_TransformActor.BP_TransformActor_C" (Math|Transform|MakeTransform "0, 0, 0" "0, 0, 0" "1,1,1") "Undefined" 0 0))
  (Variables|Default|SetFocusTransformActor _returnvalue_5)
  (Transformation|SetActorLocationAndRotation (Variables|Default|GetFocusTransformActor) _returnvalue_4 (Math|Rotator|FindLookatRotation _returnvalue_4 (Transformation|GetActorLocation)))
  (Transformation|AttachActorToActor (Variables|Default|GetFocusTransformActor) self "None" "KeepWorld" "KeepWorld" "SnapToTarget" true))

(fn SpawnWidget
  (params (Min :type Float%20%28single-precision%29) (Max :type Float%20%28single-precision%29))
  (Spawn|SpawnFocusActor)
  (CallFunction|EventSpawnWidget (Math|Random|RandomFloatinRange Min Max)))

(fn DestroyWeapon
  (Utilities|FlowControl|Sequence
    (:then_0
      (Utilities|IsValid (Variables|Default|GetRootTransformActor)
        (:Is%20Valid
          (Weapon|FindAttachedActors (Variables|Default|GetRootTransformActor))
          (Utilities|Array|Clear (Variables|Default|GetWeaponComponents)))))
    (:then_1
      (Actor|DestroyActor (Variables|Default|GetFocusTransformActor))
      (Actor|DestroyActor))))

(fn SpawnWeaponbyPresetName
  (params (PresetName :type String))
  (Variables|Default|SetPresetName PresetName)
  (Utilities|FlowControl|Sequence
    (:then_0
      (Utilities|FlowControl|Sequence
        (:then_0
          ;[1 1 1] (获取SaveGame，然后生成一个基础的武器组件)
          ; Get SaveGame and generate a basic weapon component
          (bind _asnew_fps_save_game (Utilities|Casting|CastToNew_FPS_SaveGame (CallFunction|GetSaveGame "GigahruchRogueLike" 0 "/Game/Blueprints/SaveGameBlueprint/New_FPS_SaveGame.New_FPS_SaveGame_C")))
          (LocalVariables|SetL_SaveGame _asnew_fps_save_game)
          (bind _presetdataarrey (Default|GetPresetData (LocalVariables|GetL_SaveGame)))
          (bind _newparam (Info|FindPresetDatabyName (Variables|Default|GetPresetName) _presetdataarrey))
          (LocalVariables|SetL_PresetData _newparam))
        (:then_1
          (bind _returnvalue (Game|SpawnActorfromClass "/Game/WeaponCustomSystem/Blueprints/Weapon/BP_TransformActor.BP_TransformActor_C" (Math|Transform|MakeTransform "0, 0, 0" "0, 0, 0" "1,1,1") "Undefined" 0 0))
          (Variables|Default|SetRootTransformActor _returnvalue)
          (bind _returnvalue_2 (Game|SpawnActorfromClass (.BaseWeaponComponentClass (Utilities|Struct|BreakS_PresetData (LocalVariables|GetL_PresetData))) (Math|Transform|MakeTransform "0, 0, 0" "0, 0, 0" "1,1,1") "Undefined" 0 0))
          (bind _output_get (Variables|Default|SetCurrentWeaponMainComponent _returnvalue_2))
          (Utilities|Array|Add (LocalVariables|GetL_WeaponComponents) _output_get)
          (Utilities|Map|Add (LocalVariables|GetL_Index_Actor) 0 (Variables|Default|GetCurrentWeaponMainComponent))
          (Transformation|AttachActorToActor (Variables|Default|GetCurrentWeaponMainComponent) (Variables|Default|GetRootTransformActor) "None" "KeepRelative" "KeepRelative" "KeepRelative" true))
        (:then_2
          (for _array_element (.WeaponComponentSpawnDatas (Utilities|Struct|BreakS_PresetData (LocalVariables|GetL_PresetData)))
            (LocalVariables|SetL_WeaponComponentSpawnData _array_element)
            (Utilities|FlowControl|Sequence
              (:then_0
                ;[1 1 1] (通过CurrentID找到WeaponComponent，该WeaponComponent就是接下来要被附着的WeaponComponent)
                ; WeaponComponent is found by CurrentID, which is the WeaponComponent to be attached next
                (LocalVariables|SetL_WeaponComponent (.Value (Utilities|Map|Find (LocalVariables|GetL_Index_Actor) (Utilities|Struct|BreakS_WeaponComponentSocketData (Utilities|Struct|BreakS_WeaponComponentSpawnData (LocalVariables|GetL_WeaponComponentSpawnData)))))))
              (:then_1
                ;[1 1 1] （获取附着点的Actor,然后修改相对位置）
                ; Get the actor of the attachment point and modify the relative position
                (bind _customcomponent (Class|BPIPublicWeaponInterface|GetCustomComponent(Message) (LocalVariables|GetL_WeaponComponent)))
                (bind _transformactor (Default|FindTransfromActorbySocketData _customcomponent (Utilities|Struct|BreakS_WeaponComponentSpawnData (LocalVariables|GetL_WeaponComponentSpawnData))))
                (bind _output_get_2 (LocalVariables|SetL_TransformActor _transformactor))
                (Transformation|AddActorWorldOffset _output_get_2 (* (Utilities|Struct|BreakS_WeaponComponentSocketData (Utilities|Struct|BreakS_WeaponComponentSpawnData (LocalVariables|GetL_WeaponComponentSpawnData))) -1.0)))
              (:then_2
                ;[1 1 1] （生成组件并附着到上面获取的Actor中）
                ; Generate a component and attach it to the Actor obtained above
                (bind _returnvalue_3 (Game|SpawnActorfromClass (.ComponentClass (Utilities|Struct|BreakS_WeaponComponentData (Utilities|Struct|BreakS_WeaponComponentSpawnData (LocalVariables|GetL_WeaponComponentSpawnData)))) (Math|Transform|MakeTransform "0, 0, 0" "0, 0, 0" "1,1,1") "Undefined" 0 0))
                (LocalVariables|SetL_CurrentPinWeaponComponent _returnvalue_3)
                (Utilities|FlowControl|Sequence
                  (:then_0
                    (bind _customcomponent_2 (Class|BPIPublicWeaponInterface|GetCustomComponent(Message) (LocalVariables|GetL_CurrentPinWeaponComponent)))
                    (Default|AttachtoTransfromActor _customcomponent_2 (Variables|/Script/Engine.Actor|GetRootComponent (LocalVariables|GetL_TransformActor))))
                  (:then_1
                    ;[1 1 1] Reback Save Data
                    (CallFunction|UpdateWeaponComponentData (LocalVariables|GetL_WeaponComponentSpawnData) (LocalVariables|GetL_CurrentPinWeaponComponent)))
                  (:then_2
                    (Utilities|Array|Add (LocalVariables|GetL_WeaponComponents) (LocalVariables|GetL_CurrentPinWeaponComponent)))))
              (:then_3
                ;[1 1 1] 添加数据
                ; adding data
                (Utilities|Map|Add (LocalVariables|GetL_Index_Actor) (Utilities|Struct|BreakS_WeaponComponentSocketData (Utilities|Struct|BreakS_WeaponComponentSpawnData (LocalVariables|GetL_WeaponComponentSpawnData))) (LocalVariables|GetL_CurrentPinWeaponComponent))))))
        (:then_3
          ;[1 1 1] 基本上用来获取相对位置
          ; Basically used to get the relative position
          (for _array_element_2 (LocalVariables|GetL_WeaponComponents)
            (bind _customcomponent_3 (Class|BPIPublicWeaponInterface|GetCustomComponent(Message) _array_element_2))
            (Variables|/Game/WeaponCustomSystem/Blueprints/Weapon/CustomComponent/BP_CustomComponent.BP_CustomComponent_C|SetRootParentActor _customcomponent_3 (Variables|Default|GetRootTransformActor))))
        (:then_4
          ;[1 1 1] 保存身上的挂件或武器到savegame
          ; Save your pendant or weapon to savegame
          (bind _asbpsg_character_clothing (Utilities|Casting|CastToBPSG_CharacterClothing (CallFunction|GetSaveGame "CharacterClothing" 0 "/Game/WeaponCustomSystem/Blueprints/SaveGame/BPSG_CharacterClothing.BPSG_CharacterClothing_C")))
          (LocalVariables|SetL_CharacterClothing_SaveGame _asbpsg_character_clothing)
          (Default|AddCharacterClothingData (LocalVariables|GetL_CharacterClothing_SaveGame) (Utilities|Struct|MakeS_CharacterClothingData (Variables|Default|GetSocketName) true (Variables|Default|GetPresetName)))
          (CallFunction|UpdateSaveGame "CharacterClothing" 0 (LocalVariables|GetL_CharacterClothing_SaveGame)))))
    (:then_1
      (Variables|Default|SetWeaponComponents (LocalVariables|GetL_WeaponComponents))
      (return (LocalVariables|GetL_WeaponComponents) (Variables|Default|GetRootTransformActor)))))

(fn FindPresetDatabyName
  (params (IN_PresetName :type String) (IN_PresetData :type Array%20of%20S%20Preset%20Data%20Structures))
  (for _array_element IN_PresetData
    (bind _output_get (LocalVariables|SetL_Preset _array_element))
    (if (Utilities|Enum|Equal(Enum) (.PresetName (Utilities|Struct|BreakS_PresetData _output_get)) IN_PresetName)
      (return (LocalVariables|GetL_Preset)))))