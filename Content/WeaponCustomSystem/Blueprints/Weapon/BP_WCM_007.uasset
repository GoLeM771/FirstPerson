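; BP_WCM_007 is a Blueprint in the weapon customization system that drives a toggleable MK18 front sight.
; When its action component fires ToggleAction, it casts the skeletal mesh's anim instance to the front sight AnimBlueprint and passes the status to that blueprint's Toggle.
; It adds no other logic: the default events are disabled and construction only calls the parent.
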(event ToggleAction(BP_ActionComponent)
  (params (Status :type Boolean))
  (bind _assk_mk18_front_sight_skeleton_anim_blueprint (Utilities|Casting|CastToSK_MK18_FrontSight_Skeleton_AnimBlueprint (Components|SkeletalMesh|GetAnimInstance (Variables|Default|GetSkeletalMesh))))
  (Default|Toggle _assk_mk18_front_sight_skeleton_anim_blueprint Status))

(event EventBeginPlay
  (|CallParentFunction) ; 此节点被禁用，将不会被调用。\n从引脚连出引线来编译功能。
)

(event Collision|EventActorBeginOverlap
  (params (OtherActor :type Actor%20Object%20Reference))
  (|CallParentFunction OtherActor) ; 此节点被禁用，将不会被调用。\n从引脚连出引线来编译功能。
)

(event EventTick
  (params (DeltaSeconds :type Float%20%28single-precision%29))
  (|CallParentFunction DeltaSeconds) ; 此节点被禁用，将不会被调用。\n从引脚连出引线来编译功能。
)

(fn ConstructionScript
  (|CallParentFunction))