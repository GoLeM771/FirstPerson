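; Pawn for previewing and customizing a weapon, with a spring-arm zoom camera and mouse dragging.
; Spawns the weapon under a centered TransformActor and feeds both to the component panel widget.
; ShowHand gates clamped hand IK offset and rotation input, but the switch into hand view and free weapon rotation are disconnected.
; Exit timelines animate the weapon, then clear the panel; possession passes to a spawned custom character or back through PlayerInterface.
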(event Custom|Event_ColseHand
  ;[1 1 1] 切换观察模式
  ; Switch observation mode. Пока показ в руках персонажа отключен
  ;;[1 1 1] 第三人称模式
  ;; TPS
  (Utilities|FlowControl|Sequence
    (:then_0
      (Rendering|SetVisibility (Variables|Default|GetSkeletalMesh) false false)
      (Transformation|DetachFromActor (Variables|组件|GetTransformActor) "KeepWorld" "KeepWorld" "KeepWorld")
      (Transformation|SetActorLocationAndRotation (Variables|组件|GetTransformActor) "0, 0, 0" "0,180.000000, 0")
      (Transformation|SetRelativeLocation (Variables|Default|GetCamera) "0, 0, 0" false false)
      (Variables|IK|SetIKRotation "0, 0, 0")
      (Variables|IK|SetRelativeSightLoction "0, 0, 0")
      (Variables|IK|SetTargetSightPointLocation (Math|Vector|MakeVector 0.0 0.0 0.0))
      (Variables|/Script/Engine.SpringArmComponent|SetTargetArmLength (Variables|Default|GetSpringArm) 1.5e+02)
      (Variables|Data|SetTargetArmLength 7e+01)
      (CallFunction|SetTransformActortoWeaponCenter))
    (:then_1
      (Variables|Data|SetShowHand false))))

(event Custom|Event_MoveWeaponByMouse
  (bind _returnvalue (Game|GetPlayerController 0))
  (bind _returnvalue_2 (Game|GetPlayerController 0))
  (bind (_deltax _deltay) (Class|PlayerController|GetInputMouseDelta _returnvalue))
  (bind (_deltax_2 _deltay_2) (Class|PlayerController|GetInputMouseDelta _returnvalue_2))
  ;[1 1 1] Move
  (Utilities|IsValid (Variables|组件|GetTransformActor)
    (:Is%20Valid
      (if (Game|Player|IsInputKeyDown (Game|GetPlayerController 0) "LeftMouseButton")
        (if (Variables|Data|GetShowHand)
          ;;[1 1 1] Hand move
          (Variables|IK|SetTargetSightPointOffset (Math|Vector|ClampVectorSize (+ (* (+ (* (Math|Vector|GetUpVector (Pawn|GetControlRotation :!class /Script/Engine.Pawn)) _deltay) (* (Math|Vector|GetRightVector (Pawn|GetControlRotation :!class /Script/Engine.Pawn)) (* _deltax -1.0))) 0.2) (Variables|IK|GetTargetSightPointOffset)) -4.0 4.0))
          (Variables|IK|SetTargetSightPointLocation (+ (Variables|IK|GetBaseTargetSightPointLocation) (Variables|IK|GetTargetSightPointOffset)))
          (else
            ;;[1 1 1] Weapon move
            (Transformation|AddActorWorldOffset (Variables|组件|GetTransformActor) (* (+ (* (Math|Vector|GetUpVector (Pawn|GetControlRotation :!class /Script/Engine.Pawn)) _deltay_2) (* (Math|Vector|GetRightVector (Pawn|GetControlRotation :!class /Script/Engine.Pawn)) _deltax_2)) 0.2))))))))

(event Custom|Event_SwitchToCustomCharacter
  ;[1 1 1] 切换到自定义角色
  ; Switch to custom character
  (Rendering|SetVisibility (Variables|Default|GetSkeletalMesh) false false)
  (bind _returnvalue (Game|SpawnActorfromClass "/Game/WeaponCustomSystem/Blueprints/Character/BP_CustomCharacter.BP_CustomCharacter_C" (Math|Transform|MakeTransform "400.000000, 0, 0" "0, 0, 0" "1,1,1") "Undefined" 0 0))
  (Variables|Default|SetCustomCharacter _returnvalue)
  (bind _asplayer_controller (Utilities|Casting|CastToPlayerController (Pawn|GetController)))
  (Game|Player|SetViewTargetwithBlend _asplayer_controller (Variables|Default|GetCustomCharacter) 1.0 "VTBlend_Cubic" 0.0 false)
  (Widget|RemovefromParent (Variables|Widget|GetBPW_WeaponComponentPanel))
  (bind _alpha (Timeline|Timeline_0 PlayFromStart)
    (:Update
      (Transformation|SetActorLocation (Variables|组件|GetTransformActor) (Math|Vector|Lerp(Vector) (Transformation|GetActorLocation (Variables|组件|GetTransformActor)) "0.000000,-10.000000,0.000000" _alpha) false false)
      (Transformation|SetActorRotation (Variables|组件|GetTransformActor) (Math|Rotator|Lerp(Rotator) (Transformation|GetActorRotation (Variables|组件|GetTransformActor)) "0,-90.000000, 0" _alpha))
      (Transformation|SetActorLocation (Variables|Default|GetCustomCharacter) (Math|Vector|Lerp(Vector) (Transformation|GetActorLocation (Variables|Default|GetCustomCharacter)) "0, 0, 0" _alpha) false false))
    (:Finished
      (Default|ClearWeaponComponents (Variables|Widget|GetBPW_WeaponComponentPanel))
      (Variables|Widget|SetBPW_WeaponComponentPanel 0)
      (Variables|组件|SetTransformActor 0)
      (Variables|组件|SetWeapon 0)
      (Pawn|Possess (Pawn|GetController) (Variables|Default|GetCustomCharacter))
      (Actor|DestroyActor))))

(event Custom|DestroyWeaponPreview
  ;[1 1 1] Переписать
  (Utilities|FlowControl|Sequence
    (:then_0
      (Rendering|SetVisibility (Variables|Default|GetSkeletalMesh) false false)
      (Widget|RemovefromParent (Variables|Widget|GetBPW_WeaponComponentPanel))
      (bind _alpha (Timeline|Timeline_1 PlayFromStart)
        (:Update
          (Transformation|SetActorLocation (Variables|组件|GetTransformActor) (Math|Vector|Lerp(Vector) (Transformation|GetActorLocation (Variables|组件|GetTransformActor)) "0.000000,-10.000000,0.000000" _alpha) false false)
          (Transformation|SetActorRotation (Variables|组件|GetTransformActor) (Math|Rotator|Lerp(Rotator) (Transformation|GetActorRotation (Variables|组件|GetTransformActor)) "0,-90.000000, 0" _alpha)))
        (:Finished
          (Default|ClearWeaponComponents (Variables|Widget|GetBPW_WeaponComponentPanel))
          (Variables|Widget|SetBPW_WeaponComponentPanel 0)
          (Variables|组件|SetTransformActor 0)
          (Variables|组件|SetWeapon 0))))
    (:then_1
      (bind _outactors (Actor|GetAllActorswithInterface "/Game/Blueprints/Interfaces/PlayerInterface.PlayerInterface_C"))
      (for _array_element _outactors
        (Class|PlayerInterface|PossessBack(Message) _array_element (Pawn|GetController))))))

(event EventBeginPlay
  (if (Variables|Default|GetInHubLocationSpawn?)
    (Transformation|SetRelativeLocation (Variables|Default|GetScene self) (Variables|Default|GetWeaponLocatoin) false true)))

(event EventDestroyWeaponKostil
  ;[1 1 1] Переписать
  (CallFunction|DestroyWeaponPreview))

(event EventTick
  (params (DeltaSeconds :type Float%20%28single-precision%29))
  (bind _returnvalue (Game|GetPlayerController 0))
  (bind (_deltax _deltay) (Class|PlayerController|GetInputMouseDelta _returnvalue))
  ;[1 1 1] 计算手部旋转值
  ; Calculate hand rotation value
  (Utilities|FlowControl|Sequence
    (:then_0
      (if (Game|Player|IsInputKeyDown (Game|GetPlayerController 0) "RightMouseButton")
        (Utilities|IsValid (Variables|组件|GetTransformActor)
          (:Is%20Valid
            (if (Variables|Data|GetShowHand)
              ;;[1 1 1] 控制武器旋转,手部控制
              ;; Controlling hand rotation
              (Variables|IK|SetIKRotation (Math|Rotator|MakeRotator (Math|Float|ClampAngle (.roll (Math|Transform|InverseTransformRotation (Math|Transform|MakeTransform (Transformation|GetActorLocation (Variables|组件|GetTransformActor)) (Math|Rotator|MakeRotator 0.0 (* _deltay -1.0) _deltax) "1,1,1") (Variables|IK|GetIKRotation))) -2e+01 2e+01) (Math|Float|ClampAngle (.pitch (Math|Transform|InverseTransformRotation (Math|Transform|MakeTransform (Transformation|GetActorLocation (Variables|组件|GetTransformActor)) (Math|Rotator|MakeRotator 0.0 (* _deltay -1.0) _deltax) "1,1,1") (Variables|IK|GetIKRotation))) -2e+01 2e+01) (Math|Float|ClampAngle (.yaw (Math|Transform|InverseTransformRotation (Math|Transform|MakeTransform (Transformation|GetActorLocation (Variables|组件|GetTransformActor)) (Math|Rotator|MakeRotator 0.0 (* _deltay -1.0) _deltax) "1,1,1") (Variables|IK|GetIKRotation))) -6e+01 2e+01))))))))
    (:then_1
      (CallFunction|EventMoveWeaponbyMouse))))

(event Input|MouseEvents|MouseWheelAxis
  (params (AxisValue :type Float%20%28single-precision%29))
  ;[1 1 1] Lerp Arm Length
  (Variables|/Script/Engine.SpringArmComponent|SetTargetArmLength (Variables|Default|GetSpringArm) (Math|Float|Clamp(Float) (Math|Interpolation|FInterpTo (Variables|/Script/Engine.SpringArmComponent|GetTargetArmLength (Variables|Default|GetSpringArm)) (Variables|Data|GetTargetArmLength) (Utilities|Time|GetWorldDeltaSeconds) 1e+01) 1e+01 1.5e+02)))

(event Input|MouseEvents|MouseWheelUp
  (params (Key :type Key%20Structure :default "None"))
  ;[1 1 1] Lerp Arm Length
  (:Pressed
    (if (not (Variables|Data|GetShowHand))
      (Variables|Data|SetTargetArmLength (+ -5.0 (Variables|/Script/Engine.SpringArmComponent|GetTargetArmLength (Variables|Default|GetSpringArm)))))))

(event Input|MouseEvents|MouseWheelDown
  (params (Key :type Key%20Structure :default "None"))
  ;[1 1 1] Lerp Arm Length
  (:Pressed
    (if (not (Variables|Data|GetShowHand))
      (Variables|Data|SetTargetArmLength (+ 5.0 (Variables|/Script/Engine.SpringArmComponent|GetTargetArmLength (Variables|Default|GetSpringArm)))))))

(event Input|KeyboardEvents|R
  (params (Key :type Key%20Structure :default "None"))
  ;[1 1 1] 切换观察模式
  ; Switch observation mode. Пока показ в руках персонажа отключен
)

(fn ConstructionScript)

(fn CalculateIKLocation
  (Variables|IK|SetIKRotation "0, 0, 0")
  (bind _customcomponent (Class|BPIPublicWeaponInterface|GetCustomComponent(Message) (Variables|组件|GetWeapon)))
  (LocalVariables|SetL_CurrentCustomComponent _customcomponent)
  ;[1 1 1] 定点位置
  ; SightPointLocation
  (Variables|IK|SetRelativeSightLoction (+ (Default|ConveLocationtoRelativeLocationRoot (LocalVariables|GetL_CurrentCustomComponent) "0,90.000000,0" (.Origin (Collision|GetActorBounds (Variables|组件|GetWeapon) false false))) (Math|Vector|RotateVector (.Location (Math|Transform|BreakTransform (Transformation|GetSocketTransform (Variables|Default|GetSkeletalMesh) "VB GunSocket" "RTS_ParentBoneSpace"))) (.Rotation (Math|Transform|BreakTransform (Transformation|GetSocketTransform (Variables|Default|GetSkeletalMesh) "VB Ik_SightPoint_R" "RTS_Component"))))))
  (Variables|IK|SetIKRotation "0,-60.000000, 0")
  (bind _output_get (Variables|IK|SetBaseTargetSightPointLocation (Math|Vector|MakeVector (.X (Math|Vector|BreakVector (- (.OutPosition (Class|SkinnedMeshComponent|TransformtoBoneSpace (Variables|Default|GetSkeletalMesh) "root" "0, 0, 0" "0, 0, 0")) (+ (.Location (Math|Transform|BreakTransform (Transformation|GetSocketTransform (Variables|Default|GetSkeletalMesh) "VB Ik_SightPoint_R" "RTS_Component"))) (Variables|IK|GetRelativeSightLoction))))) -1e+01 (.Z (Math|Vector|BreakVector (- (.OutPosition (Class|SkinnedMeshComponent|TransformtoBoneSpace (Variables|Default|GetSkeletalMesh) "root" "0, 0, 0" "0, 0, 0")) (+ (.Location (Math|Transform|BreakTransform (Transformation|GetSocketTransform (Variables|Default|GetSkeletalMesh) "VB Ik_SightPoint_R" "RTS_Component"))) (Variables|IK|GetRelativeSightLoction))))))))
  (Variables|IK|SetTargetSightPointLocation _output_get))

(fn InitBaseWeaponComponentLocal
  (params (BaseWeaponComponentClass :type Actor%20Class%20Reference))
  (bind _returnvalue (Game|SpawnActorfromClass BaseWeaponComponentClass (Math|Transform|MakeTransform (Variables|Default|GetWeaponLocatoin) "0, 0, 0" "1,1,1") "Undefined" 0 0))
  (Variables|组件|SetWeapon _returnvalue)
  (Utilities|FlowControl|Sequence
    (:then_0
      (Utilities|IsValid (Variables|组件|GetTransformActor)
        (:Is%20Valid
          (CallFunction|EventColseHand)
          (Actor|DestroyActor (Variables|组件|GetTransformActor)))))
    (:then_1
      (bind _returnvalue_2 (Game|SpawnActorfromClass "/Game/WeaponCustomSystem/Blueprints/Weapon/BP_TransformActor.BP_TransformActor_C" (Math|Transform|MakeTransform (Variables|Default|GetWeaponLocatoin) "0, 0, 0" "1,1,1") "Undefined" 0 0))
      (Variables|组件|SetTransformActor _returnvalue_2))
    (:then_2
      (Transformation|AttachActorToActor (Variables|组件|GetWeapon) (Variables|组件|GetTransformActor) "None" "KeepRelative" "KeepRelative" "KeepRelative" true)
      (Transformation|SetActorLocationAndRotation (Variables|组件|GetTransformActor) (Variables|Default|GetWeaponLocatoin) "0,180.000000, 0")
      (CallFunction|SetTransformActortoWeaponCenter))
    (:then_3
      (Utilities|IsValid (Variables|Widget|GetBPW_WeaponComponentPanel)
        (:Is%20Valid
          (if (UserInterface|Viewport|IsinViewport (Variables|Widget|GetBPW_WeaponComponentPanel))
            _
            (else
              (UserInterface|Viewport|AddtoViewport (Variables|Widget|GetBPW_WeaponComponentPanel) 1))))
        (:Is%20Not%20Valid
          (bind _returnvalue_3 (UserInterface|CreateWidget "/Game/WeaponCustomSystem/Blueprints/UI/BPW_WeaponComponentPanel.BPW_WeaponComponentPanel_C"))
          (Variables|Widget|SetBPW_WeaponComponentPanel _returnvalue_3)
          (UserInterface|Viewport|AddtoViewport (Variables|Widget|GetBPW_WeaponComponentPanel) 1)))
      (Variables|/Game/WeaponCustomSystem/Blueprints/UI/BPW_WeaponComponentPanel.BPW_WeaponComponentPanel_C|SetTransformActor (Variables|Widget|GetBPW_WeaponComponentPanel) (Variables|组件|GetTransformActor))
      (Default|AddWeaponComponents (Variables|Widget|GetBPW_WeaponComponentPanel) (Variables|组件|GetWeapon)))
    (:then_4
      (return true))))

(fn SetTransformActortoWeaponCenter
  (if (Variables|Default|GetInHubLocationSpawn?)
    (Transformation|SetActorRelativeLocation (.Origin (Collision|GetActorBounds (Variables|组件|GetWeapon) false false)))
    (else
      (Transformation|SetActorRelativeLocation (Variables|组件|GetWeapon) (* (.Origin (Collision|GetActorBounds (Variables|组件|GetWeapon) false false)) "1.000000,1.000000,-1.000000"))))
  (return))

(fn SetTransformActortoOringPoint
  (Transformation|SetActorRelativeLocation (Variables|组件|GetWeapon)))

(fn ClampVector
  (params (Vector :type Vector) (Min :type Float%20%28single-precision%29) (Max :type Float%20%28single-precision%29))
  (bind (_x _y _z) (Math|Vector|BreakVector Vector))
  (return (Math|Vector|MakeVector (Math|Float|Clamp(Float) _x Min Max) (Math|Float|Clamp(Float) _y Min Max) (Math|Float|Clamp(Float) _z Min Max))))

(fn DebugWeaponBaseActorLocationInfo
  (Development|PrintString (Utilities|String|Append "Camera location: " (Utilities|String|ToString(Vector) (Transformation|GetActorLocation)) " Weapon location: " (Utilities|String|ToString(Vector) (Transformation|GetActorLocation (Variables|组件|GetWeapon)))) true true "(R=0.000000,G=0.660000,B=1.000000,A=1.000000)" 0.0)
  (Development|PrintString (Utilities|String|Append "WeaponActorRotation: " (Utilities|String|ToString(Rotator) (Transformation|GetActorRotation (Variables|组件|GetWeapon)))) true true "(R=0.000000,G=0.660000,B=1.000000,A=1.000000)" 0.0))

(fn GetOwnedWeaponComponentData
  (return 0))

(fn GetWeaponCenterLocation
  (Utilities|IsValid (Variables|组件|GetTransformActor)
    (:Is%20Valid
      (return (.Origin (Collision|GetActorBounds (Variables|组件|GetWeapon) false false))))
    (:Is%20Not%20Valid
      (return "0, 0, 0"))))

(fn GetWeaponComponentTable
  (return 0))

(fn InitBaseWeaponComponent
  (params (BaseWeaponComponentClass :type Actor%20Class%20Reference))
  (bind _newparam (CallFunction|InitBaseWeaponComponentLocal BaseWeaponComponentClass))
  (return _newparam))

(fn IsFollowCharacterCamera
  (return true))