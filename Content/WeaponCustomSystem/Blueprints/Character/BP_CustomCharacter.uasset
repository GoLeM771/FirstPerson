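; BP_CustomCharacter is the preview character for a customization screen, with orbit-style mouse controls for inspecting it.
; BeginPlay hands the skeletal mesh to BPClothingComponent, shows its custom widget, adds the customization panel and enables cursor input.
; Right-drag yaws the mesh, left-drag moves the spring arm vertically and the wheel zooms, all smoothed by interpolation.
; Weapon-related functions are stubs returning defaults, except IsFollowCharacterCamera, which returns true.
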(event EventBeginPlay
  (Default|SetInfo (Variables|Default|GetBP_ClothingComponent) (Variables|Default|GetSkeletalMesh))
  (Default|ShowCustomWidget (Variables|Default|GetBP_ClothingComponent) 1.5 2.5)
  (Variables|/Script/Engine.PlayerController|SetbShowMouseCursor (Game|GetPlayerController 0) true)
  (Input|SetInputModeGameandUI (Game|GetPlayerController 0) 0 "DoNotLock" true)
  (bind _returnvalue (UserInterface|CreateWidget "/Game/WeaponCustomSystem/Blueprints/UI/ClothingComponent/BPW_CustomCharacterPanel.BPW_CustomCharacterPanel_C"))
  (UserInterface|Viewport|AddtoViewport _returnvalue 0))

(event Collision|EventActorBeginOverlap
  (params (OtherActor :type Actor%20Object%20Reference)))

(event Input|MouseEvents|MouseWheelAxis
  (params (AxisValue :type Float%20%28single-precision%29))
  ;[1 1 1] Comment
  (Variables|/Script/Engine.SpringArmComponent|SetTargetArmLength (Variables|Default|GetSpringArm) (Math|Float|Clamp(Float) (Math|Interpolation|FInterpTo (Variables|/Script/Engine.SpringArmComponent|GetTargetArmLength (Variables|Default|GetSpringArm)) (Variables|Default|GetArmLengthNew) (Utilities|Time|GetWorldDeltaSeconds) 5.0) 1e+01 6e+02)))

(event Input|MouseEvents|MouseWheelUp
  (params (Key :type Key%20Structure))
  ;[1 1 1] Comment
  (:Pressed
    (Variables|Default|SetArmLengthNew (+ -3e+01 (Variables|/Script/Engine.SpringArmComponent|GetTargetArmLength (Variables|Default|GetSpringArm))))))

(event Input|MouseEvents|MouseWheelDown
  (params (Key :type Key%20Structure))
  ;[1 1 1] Comment
  (:Pressed
    (Variables|Default|SetArmLengthNew (+ 3e+01 (Variables|/Script/Engine.SpringArmComponent|GetTargetArmLength (Variables|Default|GetSpringArm))))))

(event Custom|Event_Update
  ;[1 1 1] Comment
  (Transformation|SetRelativeLocation (Variables|Default|GetSpringArm) (Math|Interpolation|VInterpTo (Variables|/Script/Engine.SceneComponent|GetRelativeLocation (Variables|Default|GetSpringArm)) (Variables|Default|GetSpringArmLocation) (Utilities|Time|GetWorldDeltaSeconds) 6.0) false false)
  (Transformation|SetWorldRotation (Variables|Default|GetSkeletalMesh) (Math|Interpolation|RInterpTo (Transformation|GetWorldRotation (Variables|Default|GetSkeletalMesh)) (Variables|Default|GetCharacterRotation) (Utilities|Time|GetWorldDeltaSeconds) 6.0) false false))

(event Custom|Event_MoveCameraByMouse
  ;[1 1 1] Comment
  (if (Game|Player|IsInputKeyDown (Game|GetPlayerController 0) "LeftMouseButton")
    (Variables|Default|SetSpringArmLocation (- (Variables|Default|GetSpringArmLocation) (Math|Vector|MakeVector 0.0 0.0 (.DeltaY (Class|PlayerController|GetInputMouseDelta (Game|GetPlayerController 0))))))))

(event Custom|Event_RotatorCharacterByMouse
  ;[1 1 1] 控制角色旋转
  ; Controlling Character rotation
  (if (Game|Player|IsInputKeyDown (Game|GetPlayerController 0) "RightMouseButton")
    (Variables|Default|SetCharacterRotation (Math|Rotator|MakeRotator 0.0 0.0 (- (.Yaw (Math|Rotator|BreakRotator (Variables|Default|GetCharacterRotation))) (.DeltaX (Class|PlayerController|GetInputMouseDelta (Game|GetPlayerController 0))))))))

(event EventTick
  (params (DeltaSeconds :type Float%20%28single-precision%29))
  (Utilities|FlowControl|Sequence
    (:then_0
      (CallFunction|EventRotatorCharacterbyMouse))
    (:then_1
      (CallFunction|EventMoveCamerabyMouse))
    (:then_2
      (CallFunction|EventUpdate))))

(fn ConstructionScript)

(fn GetOwnedWeaponComponentData
  (return 0))

(fn GetWeaponCenterLocation
  (return "0, 0, 0"))

(fn GetWeaponComponentTable
  (return 0))

(fn InitBaseWeaponComponent
  (params (BaseWeaponComponentClass :type Actor%20Class%20Reference))
  (return false))

(fn IsFollowCharacterCamera
  (return true))