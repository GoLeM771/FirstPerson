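; Blueprint function library of shared helpers for the weapon customization system, save games and weighted random rolls.
; It converts world positions into a skeletal mesh's root-socket space and restores saved spawn data onto a weapon's hand, action and custom components.
; Save helpers load a slot, or create and write one if missing.
; Loot, room modifier and body-part modification pickers share a cumulative-weight random selection.
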(fn WorldSpacetoPawnComponentSapce
  (params (CurrentWorldSpace :type Vector) (CurrentSkeletalComponent :type Skeletal%20Mesh%20Component%20Object%20Reference))
  (bind _returnvalue (Transformation|GetSocketTransform CurrentSkeletalComponent "root" "RTS_World"))
  (Utilities|IsValid CurrentSkeletalComponent
    (:Is%20Valid
      (return (Math|Vector|UnrotateVector (- CurrentWorldSpace (.location _returnvalue)) (.rotation _returnvalue))))
    (:Is%20Not%20Valid
      (return CurrentWorldSpace))))

(fn UpdateWeaponComponentData
  (params (CurrentSpawnData :type S%20Weapon%20Component%20Spawn%20Data%20Structure) (CurrentWeaponComponent :type Actor%20Object%20Reference))
  (Utilities|FlowControl|Sequence
    (:then_0
      ;[1 1 1] Reback Save Data
      (bind _component (Class|BPIPublicWeaponInterface|GetHandCopmonent(Message) CurrentWeaponComponent))
      (Utilities|IsValid _component
        (:Is%20Valid
          (|SetBy-RefVar (Variables|/Game/WeaponCustomSystem/Blueprints/Weapon/CustomComponent/BP_HandCustomComponent.BP_HandCustomComponent_C|GetHandCopmonentData _component) (Utilities|Struct|BreakS_WeaponComponentSpawnData CurrentSpawnData)))))
    (:then_1
      (bind _component_2 (Class|BPIPublicWeaponInterface|GetActionComponent(Message) CurrentWeaponComponent))
      (Utilities|IsValid _component_2
        (:Is%20Valid
          (bind _output_get (Variables|/Game/WeaponCustomSystem/Blueprints/Weapon/CustomComponent/BP_ActionComponent.BP_ActionComponent_C|SetStatus _component_2 (Utilities|Struct|BreakS_WeaponComponentSpawnData CurrentSpawnData)))
          (Default|CallToggleAction _component_2 _output_get))))
    (:then_2
      (bind _customcomponent (Class|BPIPublicWeaponInterface|GetCustomComponent(Message) CurrentWeaponComponent))
      (Variables|/Game/WeaponCustomSystem/Blueprints/Weapon/CustomComponent/BP_CustomComponent.BP_CustomComponent_C|SetWeaponComponentData _customcomponent (Utilities|Struct|BreakS_WeaponComponentSpawnData CurrentSpawnData)))))

(fn GetSaveGame
  (params (SlotName :type String) (UserIndex :type Integer) (SaveGameClass :type Save%20Game%20Class%20Reference))
  (bind _returnvalue (SaveGame|DoesSaveGameExist SlotName UserIndex))
  (if _returnvalue
    (bind _returnvalue_2 (SaveGame|LoadGamefromSlot SlotName UserIndex))
    (LocalVariables|SetL_SaveGame _returnvalue_2)
    (return (LocalVariables|GetL_SaveGame))
    (else
      (bind _returnvalue_3 (SaveGame|CreateSaveGameObject SaveGameClass))
      (LocalVariables|SetL_SaveGame _returnvalue_3)
      (SaveGame|UpdateSaveGame SlotName UserIndex (LocalVariables|GetL_SaveGame))
      (return (LocalVariables|GetL_SaveGame)))))

(fn UpdateSaveGame
  (params (SlotName :type String) (UserIndex :type Integer) (SaveGameObject :type Save%20Game%20Object%20Reference))
  (SaveGame|SaveGametoSlot SaveGameObject SlotName UserIndex))

(fn DropRandomLoot
  (params (LootToDrop :type Array%20of%20S%20Loot%20Structures))
  (LocalVariables|SetLootArrey LootToDrop)
  (for _array_element (LocalVariables|GetLootArrey)
    (LocalVariables|SetSumOfLootWeaight (+ (.DropChance (Utilities|Struct|BreakS_Loot _array_element)) (LocalVariables|GetSumOfLootWeaight))))
  (LocalVariables|SetRandomValue (Math|Random|RandomFloatinRange 0.0 (LocalVariables|GetSumOfLootWeaight)))
  (for _array_element_2 (LocalVariables|GetLootArrey)
    (if (<= (LocalVariables|GetRandomValue) (.DropChance (Utilities|Struct|BreakS_Loot _array_element_2)))
      (return (.class (.PickupContent (Utilities|Struct|BreakS_Loot _array_element_2))))
      (else
        (LocalVariables|SetRandomValue (- (LocalVariables|GetRandomValue) (.DropChance (Utilities|Struct|BreakS_Loot _array_element_2))))))))

(fn RandomRoomModification
  (params (RoomModyfArrey1 :type Array%20of%20S%20Room%20Modification%20Structures))
  (LocalVariables|SetRoomModyfArrey RoomModyfArrey1)
  (for _array_element (LocalVariables|GetRoomModyfArrey)
    (LocalVariables|SetSumOfLootWeaight (+ (Utilities|Struct|BreakS_RoomModification _array_element) (LocalVariables|GetSumOfLootWeaight))))
  (LocalVariables|SetRandomValue (Math|Random|RandomFloatinRange 0.0 (LocalVariables|GetSumOfLootWeaight)))
  (for _array_element_2 (LocalVariables|GetRoomModyfArrey)
    (if (<= (LocalVariables|GetRandomValue) (.ModificatorChance (Utilities|Struct|BreakS_RoomModification _array_element_2)))
      (return (.E_Modifycator (Utilities|Struct|BreakS_RoomModification _array_element_2)))
      (else
        (LocalVariables|SetRandomValue (- (LocalVariables|GetRandomValue) (.ModificatorChance (Utilities|Struct|BreakS_RoomModification _array_element_2))))))))

(fn SelectBodyPartModyfications
  (params (ModyfStruct :type Array%20of%20S%20Body%20Part%20Modification%20Structures))
  (LocalVariables|SetModyfArrey ModyfStruct)
  (for _array_element (LocalVariables|GetModyfArrey)
    (LocalVariables|SetSumOfLootWeaight (+ (Utilities|Struct|Breaks_BodyPartModification _array_element) (LocalVariables|GetSumOfLootWeaight))))
  (LocalVariables|SetRandomValue (Math|Random|RandomFloatinRange 0.0 (LocalVariables|GetSumOfLootWeaight)))
  (for _array_element_2 (LocalVariables|GetModyfArrey)
    (if (<= (LocalVariables|GetRandomValue) (.Veight (Utilities|Struct|Breaks_BodyPartModification _array_element_2)))
      (return (.Modifycation (Utilities|Struct|Breaks_BodyPartModification _array_element_2)))
      (else
        (LocalVariables|SetRandomValue (- (LocalVariables|GetRandomValue) (.Veight (Utilities|Struct|Breaks_BodyPartModification _array_element_2))))))))