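; Player controller for the weapon customization system that owns the weapon component data and drives a radial weapon selection menu.
; BeginPlay copies every row of the weapon data table into the owned weapon list, exposed through getter functions alongside several stub functions.
; Holding Left Alt shows the radial menu and locks look input.
; Releasing it reads the hovered slot, removes the menu and tells the character to switch weapons via an interface message.
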(event EventBeginPlay
  (bind _table (CallFunction|GetWeaponComponentTable))
  (bind _outrownames (DataTable|GetDataTableRowNames _table))
  (for _array_element _outrownames
    (bind _table_2 (CallFunction|GetWeaponComponentTable))
    (bind _returnvalue (Utilities|GetDataTableRow _table_2 _array_element)
      (:then
        (Utilities|Array|Add (Variables|Default|GetOwned_Weapon_Data) _returnvalue)))))

(event EventTick
  (params (DeltaSeconds :type Float%20%28single-precision%29)))

(event Input|KeyboardEvents|LeftAlt
  (params (Key :type Key%20Structure :default "None"))
  (:Pressed
    (Variables|Default|GetSelectionWeel
      (:then
        _)
      (:else
        (bind _returnvalue (UserInterface|CreateWidget "/Game/Blueprints/UI/RadialMenu.RadialMenu_C" self))
        (bind _output_get (Variables|Default|SetSelectionWeel _returnvalue))))
    (UserInterface|Viewport|AddtoViewport _output_get 0)
    ;[1 1 1] Дизейблим вращение башкой персонажа
    (Input|SetIgnoreLookInput true))
  (:Released
    (bind _selectionweel (Variables|Default|GetSelectionWeel)
      (:then
        ;[1 1 1] Перед уничтожением берём слот на который смотрит курсор
        (Variables|Default|SetWeaponIndex (Variables|/Game/GenericRadialMenus/UMG/UMG_RadialMenu.UMG_RadialMenu_C|GetIndex (Variables|/Game/Blueprints/UI/RadialMenu.RadialMenu_C|GetSelectionMenu _selectionweel)))
        (Widget|RemovefromParent _selectionweel)
        (Variables|Default|SetSelectionWeel 0)
        (Input|SetIgnoreLookInput false)
        ;[1 1 1] Говорим игроку поменять оружие
        (Class|PlayerInterface|SwitchWeapontoInterface(Message) (Game|GetPlayerCharacter 0) (Variables|Default|GetWeaponIndex)))
      (:else))))

(fn ConstructionScript)

(fn GetOwnedWeaponComponentData
  (return (Variables|Default|GetOwned_Weapon_Data)))

(fn GetWeaponCenterLocation
  (return "0, 0, 0"))

(fn GetWeaponComponentTable
  (return "/Game/WeaponCustomSystem/Blueprints/Data/DT_WeaponDataTable.DT_WeaponDataTable"))

(fn InitBaseWeaponComponent
  (params (BaseWeaponComponentClass :type Actor%20Class%20Reference))
  (return false))

(fn IsFollowCharacterCamera
  (return false))