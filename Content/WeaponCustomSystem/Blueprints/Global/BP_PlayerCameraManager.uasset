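; Player camera manager for the weapon customization system that switches the player view between the default camera and an eye-socket view.
; Each camera update asks the controlled pawn whether follow-character camera is on and, if so, defers to the parent update.
; Otherwise it places the camera at the skeletal mesh's Eye socket, using control rotation instead of socket rotation so the view follows player input, with a fixed FOV.
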(event EventBeginPlay)

(event Collision|EventActorBeginOverlap
  (params (OtherActor :type Actor%20Object%20Reference)))

(event EventTick
  (params (DeltaSeconds :type Float%20%28single-precision%29)))

(fn ConstructionScript)

(fn BlueprintUpdateCamera
  (params (CameraTarget :type Actor%20Object%20Reference))
  (bind _returnvalue (Game|Player|GetOwningPlayerController))
  (bind _returnvalue_2 (Pawn|GetControlledPawn _returnvalue))
  (bind _returnvalue_3 (Actor|GetComponentbyClass _returnvalue_2 "/Script/Engine.SkeletalMeshComponent"))
  ;[1 1 1] 检测是否关闭跟随角色相机，如果关闭了，那么就去计算摄像机的位置。我们不需要Socket的旋转，因为它的旋转并不是玩家输入的旋转。
  ; Check whether the following character camera is turned off, if it is turned off, then calculate the position of the camera. We don't need the rotation of Socket, because its rotation is not the rotation input by the player.
  (LocalVariables|SetL_CameraTarget CameraTarget)
  (Utilities|IsValid (Pawn|GetControlledPawn (Game|Player|GetOwningPlayerController))
    (:Is%20Valid
      (bind _return (Class|BPIPublicInformation|IsFollowCharacterCamera(Message) (Pawn|GetControlledPawn (Game|Player|GetOwningPlayerController))))
      (if _return
        (bind (_newcameralocation _newcamerarotation _newcamerafov _returnvalue_4) (|CallParentFunction (LocalVariables|GetL_CameraTarget)))
        (return _newcameralocation _newcamerarotation _newcamerafov _returnvalue_4)
        (else
          (Utilities|IsValid _returnvalue_3
            (:Is%20Valid
              (return (Transformation|GetSocketLocation _returnvalue_3 "Eye") (Pawn|GetControlRotation (Game|Player|GetOwningPlayerController) :!class /Script/Engine.Controller) 9e+01 true))))))))