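; Respirator system that runs a minutes-and-seconds countdown for the player's TPCharacter while activated.
; Tick uses a one-second Delay to step the timer, borrowing from minutes when seconds run out.
; At zero, it reduces a character stat slightly every frame through ModifyStat.
; A separate ContaminatedAir function, not called here, lowers CurrentAir by the contamination speed and prints the value.
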(event EventBeginPlay
  (bind _astpcharacter (Utilities|Casting|CastToTPCharacter (Game|GetPlayerCharacter 0)))
  (Variables|Default|SetCharRef _astpcharacter))

(event EventTick
  (params (DeltaSeconds :type Float%20%28single-precision%29))
  (if (Variables|Default|GetActivaited)
    (if (and (== (Variables|Default|GetSeckonds) 0) (== (Variables|Default|GetMinuts) 0))
      (Default|ModifyStat (Variables|Default|GetCharRef) -0.001 "NewEnumerator0")
      (else
        (Utilities|FlowControl|Delay 1.0)
        (Variables|Default|SetSeckonds (- (Variables|Default|GetSeckonds) 1))
        (if (<= (Variables|Default|GetSeckonds) -1)
          (Variables|Default|SetMinuts (- (Variables|Default|GetMinuts) 1))
          (Variables|Default|SetSeckonds 59))))))

(fn ContaminatedAir
  (bind _output_get (Variables|Default|SetCurrentAir (- (Variables|Default|GetCurrentAir) (Variables|Default|GetContaminatedSpeed))))
  (Development|PrintString (Utilities|String|ToString(Float) _output_get) true true "(R=0.000000,G=0.660000,B=1.000000,A=1.000000)" 0.0))