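; RespStartTrigger is a trigger volume that switches a character's respirator system on and off.
; When a TPCharacter begins overlapping its Box component, it sets the Activaited flag on that character's ResperatorSyastem to true, and ending the overlap sets it to false.
; Both responses run only while the trigger's Enabled flag is true.
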(event OnComponentBeginOverlap(Box)
  (params (OverlappedComponent :type Primitive%20Component%20Object%20Reference) (OtherActor :type Actor%20Object%20Reference) (OtherComp :type Primitive%20Component%20Object%20Reference) (OtherBodyIndex :type Integer) (bFromSweep :type Boolean) (SweepResult :type Hit%20Result%20Structure%20%28by%20ref%29))
  (if (Variables|Default|GetEnabled?)
    (bind _astpcharacter (Utilities|Casting|CastToTPCharacter OtherActor))
    (Variables|/Game/Blueprints/ResperatorTrigger/ResperatorSyastem.ResperatorSyastem_C|SetActivaited (Variables|/Game/Blueprints/TPCharacter.TPCharacter_C|GetResperatorSyastem _astpcharacter) true)))

(event OnComponentEndOverlap(Box)
  (params (OverlappedComponent :type Primitive%20Component%20Object%20Reference) (OtherActor :type Actor%20Object%20Reference) (OtherComp :type Primitive%20Component%20Object%20Reference) (OtherBodyIndex :type Integer))
  (if (Variables|Default|GetEnabled?)
    (bind _astpcharacter (Utilities|Casting|CastToTPCharacter OtherActor))
    (Variables|/Game/Blueprints/ResperatorTrigger/ResperatorSyastem.ResperatorSyastem_C|SetActivaited (Variables|/Game/Blueprints/TPCharacter.TPCharacter_C|GetResperatorSyastem _astpcharacter) false)))

(event EventBeginPlay)

(event Collision|EventActorBeginOverlap
  (params (OtherActor :type Actor%20Object%20Reference)))

(event EventTick
  (params (DeltaSeconds :type Float%20%28single-precision%29)))

(fn ConstructionScript)