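; Respirator system that runs a minutes-and-seconds air countdown while activated and penalises the player when it runs out.
; Tick uses a one-second Delay to count down; at zero it lowers a player stat every tick through an interface message.
; Chained DoOnce gates switch the player's breathing audio between having air, no air and stopped.
; A separate ContaminatedAir function subtracts from CurrentAir and prints it, but nothing here calls it.
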(event EventBeginPlay)

(event EventTick
  (params (DeltaSeconds :type Float%20%28single-precision%29))
  (if (Variables|Default|GetActivaited)
    (if (and (== (Variables|Default|GetSeckonds) 0) (== (Variables|Default|GetMinuts) 0))
      (Class|PlayerInterface|ModifyStatInterface(Message) (Game|GetPlayerCharacter 0) -0.001 "NewEnumerator0")
      (Utilities|FlowControl|DoOnce false :!label _label
        (:Completed
          (Class|PlayerInterface|PlayBreatheAudio?(Message) (Game|GetPlayerCharacter 0) true false)
          (goto _label_3 Reset)))
      (else
        (Utilities|FlowControl|Delay 1.0)
        (Variables|Default|SetSeckonds (- (Variables|Default|GetSeckonds) 1))
        (if (<= (Variables|Default|GetSeckonds) -1)
          (Variables|Default|SetMinuts (- (Variables|Default|GetMinuts) 1))
          (Variables|Default|SetSeckonds 59))
        (Utilities|FlowControl|DoOnce false :!label _label_2
          (:Completed
            (Class|PlayerInterface|PlayBreatheAudio?(Message) (Game|GetPlayerCharacter 0) true true)
            (goto _label_3 Reset)))))
    (else
      (Utilities|FlowControl|DoOnce false :!label _label_3
        (:Completed
          (Class|PlayerInterface|PlayBreatheAudio?(Message) (Game|GetPlayerCharacter 0) false false)
          (Utilities|FlowControl|Sequence
            (:then_0
              (goto _label_2 Reset))
            (:then_1
              (goto _label Reset))))))))

(fn ContaminatedAir
  (bind _output_get (Variables|Default|SetCurrentAir (- (Variables|Default|GetCurrentAir) (Variables|Default|GetContaminatedSpeed))))
  (Development|PrintString (Utilities|String|Append "CurrentAir: " (Utilities|String|ToString(Float) _output_get)) true true "(R=0.000000,G=0.660000,B=1.000000,A=1.000000)" 0.0))