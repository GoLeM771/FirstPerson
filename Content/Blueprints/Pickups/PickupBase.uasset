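; Base pickup actor that grants the player a configured stat: health, armor, ammo, bombs or respirator filter minutes.
; Interaction, or overlap when AutoPickup is set, calls AddStat, which switches on StatsToAdd and uses player or gun interface messages.
; Health and armor pickups stay when the stat is full; ammo and bombs keep leftovers until used up.
; Overlap and radius events drive interaction registration, a label widget and custom-depth highlighting.
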(event OnComponentBeginOverlap(InteracteableArea)
  (params (OverlappedComponent :type Primitive%20Component%20Object%20Reference) (OtherActor :type Actor%20Object%20Reference) (OtherComp :type Primitive%20Component%20Object%20Reference) (OtherBodyIndex :type Integer) (bFromSweep :type Boolean) (SweepResult :type Hit%20Result%20Structure%20%28by%20ref%29))
  (Class|PickupInteract|RegisterInteracteable(Message) OtherActor self)
  (CallFunction|SetHighlite true))

(event OnComponentEndOverlap(InteracteableArea)
  (params (OverlappedComponent :type Primitive%20Component%20Object%20Reference) (OtherActor :type Actor%20Object%20Reference) (OtherComp :type Primitive%20Component%20Object%20Reference) (OtherBodyIndex :type Integer))
  (Class|PickupInteract|UnregisterInteracteable(Message) OtherActor self)
  (CallFunction|SetHighlite false))

(event EventBeginPlay
  (bind _widget (Variables|Default|GetWidget))
  (Utilities|FlowControl|Delay 1.0)
  (switch Utilities|FlowControl|Switch|SwitchonE_Stat (Variables|Default|GetStatsToAdd)
    (:NewEnumerator0
      (Class|ElevatorInterface|SetWidgetText(Message) _widget "Healts"))
    (:NewEnumerator1
      (Class|ElevatorInterface|SetWidgetText(Message) _widget "Armor"))
    (:NewEnumerator2
      (Class|ElevatorInterface|SetWidgetText(Message) _widget "AKSU Ammo"))
    (:NewEnumerator7
      (Class|ElevatorInterface|SetWidgetText(Message) _widget "Filters"))))

(event Collision|EventActorBeginOverlap
  (params (OtherActor :type Actor%20Object%20Reference))
  (if (Variables|Default|GetAutoPickup)
    (if (Utilities|DoesObjectImplementInterface OtherActor "/Game/Blueprints/Interfaces/PlayerInterface.PlayerInterface_C")
      (CallFunction|AddStat))))

(event EventInteraction
  (CallFunction|AddStat))

(event EventOnEnterPlayerPickupRadius
  (Rendering|SetVisibility (Variables|Default|GetWidget) true false)
  (CallFunction|SetHighlite true))

(event EventOnLeavePlayerPickupRadius
  (Rendering|SetVisibility (Variables|Default|GetWidget) false false)
  (CallFunction|SetHighlite false))

(fn ConstructionScript)

(fn SetHighlite
  (params (Highlight? :type Boolean))
  (Rendering|SetRenderCustomDepth (Variables|Default|GetPickUpModel) Highlight?))

(fn AddStat
  (bind _outactors (Actor|GetAllActorswithInterface "/Game/Blueprints/Interfaces/GunInterface.GunInterface_C"))
  (LocalVariables|SetLocalGunReference (Utilities|Array|Get(acopy) _outactors))
  (switch Utilities|FlowControl|Switch|SwitchonE_Stat (Variables|Default|GetStatsToAdd)
    (:NewEnumerator0
      (bind (_currenthealth _maxhealth) (Class|PlayerInterface|CurrentHealthGetter(Message) (Game|GetPlayerCharacter 0)))
      (if (not (== _currenthealth _maxhealth))
        (Class|PlayerInterface|ModifyStatInterface(Message) (Game|GetPlayerCharacter 0) (Variables|Default|GetAddStats) (Variables|Default|GetStatsToAdd) :!label _label)
        (Actor|DestroyActor)))
    (:NewEnumerator1
      (bind (_currentarmor _maxarmor) (Class|PlayerInterface|CurrentArmorGetter(Message) (Game|GetPlayerCharacter 0)))
      (if (not (== _currentarmor _maxarmor))
        (goto _label)))
    (:NewEnumerator2
      ;[1 1 1] Для нового персонажа. Подбор патронов для глока
      (bind _returnammo (Class|PlayerInterface|AddAmmoInterface(Message) (Game|GetPlayerCharacter 0) (Variables|Default|GetAmmoToAdd) "/Game/WeaponCustomSystem/Blueprints/Weapon/BP_WCM_GLOCK17_Body.BP_WCM_GLOCK17_Body_C"))
      (bind _output_get (Variables|Default|SetAmmoToAdd _returnammo))
      (if (== _output_get 0)
        (Actor|DestroyActor)))
    (:NewEnumerator3
      (bind _ammotoadd (Class|GunInterface|AddAmmoInterface(Message) (LocalVariables|GetLocalGunReference) (Variables|Default|GetAmmoToAdd)))
      (Variables|Default|SetAmmoToAdd _ammotoadd)
      (if (== _ammotoadd 0)
        (Actor|DestroyActor)))
    (:NewEnumerator4
      (bind _ammotoadd_2 (Class|GunInterface|AddAmmoInterface(Message) (LocalVariables|GetLocalGunReference) (Variables|Default|GetAmmoToAdd)))
      (Variables|Default|SetAmmoToAdd _ammotoadd_2)
      (if (== _ammotoadd_2 0)
        (Actor|DestroyActor)))
    (:NewEnumerator6
      (bind (_currentbomb _maxbomb) (Class|PlayerInterface|CurrentBombGetter(Message) (Game|GetPlayerCharacter 0)))
      (if (<= (+ _currentbomb (Variables|Default|GetBombToAdd)) _maxbomb)
        (Class|PlayerInterface|CurrentBombSetter(Message) (Game|GetPlayerCharacter 0) (+ _currentbomb (Variables|Default|GetBombToAdd)))
        (Actor|DestroyActor)
        (else
          (Variables|Default|SetBombToAdd (- (Variables|Default|GetBombToAdd) (- _maxbomb _currentbomb)))
          (Class|PlayerInterface|CurrentBombSetter(Message) (Game|GetPlayerCharacter 0) _maxbomb))))
    (:NewEnumerator7
      (bind _respsystemref (Class|PlayerInterface|ResperatorSystemGetter(Message) (Game|GetPlayerCharacter 0)))
      (Variables|/Game/Blueprints/ResperatorTrigger/ResperatorSyastem.ResperatorSyastem_C|SetMinuts _respsystemref (+ (Variables|/Game/Blueprints/ResperatorTrigger/ResperatorSyastem.ResperatorSyastem_C|GetMinuts _respsystemref) (Variables|Default|GetMinutsToAdd)))
      (Actor|DestroyActor))
    (:NewEnumerator8
      (bind _ammotoadd_3 (Class|GunInterface|AddAmmoInterface(Message) (LocalVariables|GetLocalGunReference) (Variables|Default|GetAmmoToAdd)))
      (Variables|Default|SetAmmoToAdd _ammotoadd_3)
      (if (== _ammotoadd_3 0)
        (Actor|DestroyActor)))))