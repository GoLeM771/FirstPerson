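; AmmoPickup is a pickup Blueprint whose only active event logic here is on-screen debug output.
; Every Tick calls DebugInfo, which prints whether the PickUpModel component is visible and the actor's current world location.
; BeginPlay and ActorBeginOverlap are disabled placeholders and the construction script only calls its parent, so this graph defines no ammo or collection logic.
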(event EventBeginPlay
  (|CallParentFunction) ; This node is disabled and will not be called.\nDrag off pins to build functionality.
)

(event Collision|EventActorBeginOverlap
  (params (OtherActor :type Actor%20Object%20Reference))
  (|CallParentFunction OtherActor) ; This node is disabled and will not be called.\nDrag off pins to build functionality.
)

(event EventTick
  (params (DeltaSeconds :type Float%20%28single-precision%29))
  (CallFunction|DebugInfo))

(fn ConstructionScript
  (|CallParentFunction))

(fn DebugInfo
  (Development|PrintString (Utilities|String|Append "SM is visiable? " (Utilities|String|ToString(Boolean) (Rendering|IsVisible (Variables|Default|GetPickUpModel self)))) true true "(R=1.000000,G=0.106016,B=0.016356,A=1.000000)" 0.0)
  (Development|PrintString (Utilities|String|Append "PickupLocation: " (Utilities|String|ToString(Vector) (Transformation|GetActorLocation))) true true "(R=1.000000,G=0.000000,B=0.764042,A=1.000000)" 0.0))