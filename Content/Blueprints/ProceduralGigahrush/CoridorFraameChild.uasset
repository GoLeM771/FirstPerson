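; Child corridor frame piece for the procedural Gigahrush generator that can randomly host an enemy bug nest.
; On BeginPlay it runs the parent logic, then fills SocketArray with its four room and stayer sockets.
; A random roll up to SpawnNestChance must hit exactly 3, then after a one-second delay SpawnBot places a BugNest at the SpawnEnemy location.
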(event EventBeginPlay
  (|CallParentFunction)
  (Variables|Default|SetSocketArray (Utilities|Array|MakeArray (Variables|Default|GetRoomSocket) (Variables|Default|GetAnotherRoomSocet) (Variables|Default|GetAnotherSuperSecretRoomSocet) (Variables|Default|GetStayerSocet)))
  (if (== (Math|Random|RandomIntegerinRange 0 (Variables|Default|GetSpawnNestChance)) 3)
    (Utilities|FlowControl|Delay 1.0)
    (CallFunction|SpawnBot (Math|Conversions|ToTransform(Vector) (Transformation|GetWorldLocation (Variables|Default|GetSpawnEnemy))) "/Game/Bot/FlootBug/BugNest.BugNest_C")))

(event Collision|EventActorBeginOverlap
  (params (OtherActor :type Actor%20Object%20Reference))
  (|CallParentFunction OtherActor) ; This node is disabled and will not be called.\nDrag off pins to build functionality.
)

(event EventTick
  (params (DeltaSeconds :type Float%20%28single-precision%29))
  (|CallParentFunction DeltaSeconds) ; This node is disabled and will not be called.\nDrag off pins to build functionality.
)

(fn ConstructionScript
  (|CallParentFunction))