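; Corridor segment of the procedural Gigahrush level that spawns a random room at one of two sockets and registers the matching super-secret-room socket with the manager.
; Its trigger starts a timed zerg rush, recursively spawning player-rushing AI from frames gathered among last-element corridors on floor 2.
; The first trigger switches the level to emergency lighting, and Tick counts down the timer and restores normal lights.
; Room-based rush logic is left disconnected.
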(event OnComponentBeginOverlap(SpawnEnemy)
  (params (OverlappedComponent :type Primitive%20Component%20Object%20Reference) (OtherActor :type Actor%20Object%20Reference) (OtherComp :type Primitive%20Component%20Object%20Reference) (OtherBodyIndex :type Integer) (bFromSweep :type Boolean) (SweepResult :type Hit%20Result%20Structure%20%28by%20ref%29))
  ;[1 1 1] При пересечении коллизии начинаем зерграш
  (if (Variables|Default|GetCanSpawnEnemy?)
    (Variables|Default|SetZergRush? true)
    (CallFunction|ZergRush)
    (Utilities|FlowControl|DoOnce false
      (:Completed
        (CallFunction|Emergency)))))

(event OnComponentBeginOverlap(Cube)
  (params (OverlappedComponent :type Primitive%20Component%20Object%20Reference) (OtherActor :type Actor%20Object%20Reference) (OtherComp :type Primitive%20Component%20Object%20Reference) (OtherBodyIndex :type Integer) (bFromSweep :type Boolean) (SweepResult :type Hit%20Result%20Structure%20%28by%20ref%29))
  (if (== (Utilities|GetClass OtherActor) "/Game/Blueprints/ProceduralGigahrush/Perekrestok.Perekrestok_C")
    (Variables|Default|SetPerekrestokIsNear? true)
    (else
      (Variables|Default|SetPerekrestokIsNear? false))))

(event Custom|FindNearCoridorFarameToSpwnEnemy
  ;[1 1 1] Выбор фрейма коридора где будут спавниться враги
  (bind _outactors (Actor|GetAllActorsOfClass "CoridorFrame_C"))
  (for _array_element _outactors
    (if (and (Variables|/Game/Blueprints/ProceduralGigahrush/BaseGigahruchElement.BaseGigahruchElement_C|GetLastElement? _array_element) (== (Variables|/Game/Blueprints/ProceduralGigahrush/BaseGigahruchElement.BaseGigahruchElement_C|GetFloorNumber _array_element) 2))
      (Utilities|Array|Add (Variables|Default|GetCoridorFrameToSpawnProps) _array_element))))

(event Custom|ZergRush
  ;[1 1 1] Рекурсия. Зерграш.
  (if (>= (Variables|Default|GetZergRushTimer) 0)
    (for _array_element (Variables|Default|GetCoridorFrameToSpawnProps)
      (CallFunction|SpawnProps _array_element))
    (Utilities|FlowControl|Delay (Variables|Default|GetTimeBetweenSpawnEnemy))
    (CallFunction|ZergRush)))

(event EventBeginPlay
  (bind _gigahruchmanager (Variables|Default|GetGigahruchManager))
  (bind _gigahruchmanager_2 (Variables|Default|GetGigahruchManager))
  (|CallParentFunction)
  (if (Math|Random|RandomBool)
    (CallFunction|SpawnRoom (Variables|Default|GetAnotherRoomSocet))
    (Utilities|IsValid _gigahruchmanager
      (:Is%20Valid
        (Utilities|Array|Add (Variables|/Game/Blueprints/ProceduralGigahrush/GigahruchManager.GigahruchManager_C|GetSoketToSpawnSuperSecretRoom _gigahruchmanager) (Variables|Default|GetAnotherSuperSecretRoomSocet)))
      (:Is%20Not%20Valid
        (Development|PrintString "No gigahrush manager" :!label _label)))
    (else
      (CallFunction|SpawnRoom (Variables|Default|GetRoomSocket))
      (Utilities|IsValid _gigahruchmanager_2
        (:Is%20Valid
          (Utilities|Array|Add (Variables|/Game/Blueprints/ProceduralGigahrush/GigahruchManager.GigahruchManager_C|GetSoketToSpawnSuperSecretRoom _gigahruchmanager_2) (Variables|Default|GetSuperSecretRoomSocet)))
        (:Is%20Not%20Valid
          (goto _label))))))

(event Collision|EventActorBeginOverlap
  (params (OtherActor :type Actor%20Object%20Reference)))

(event EventTick
  (params (DeltaSeconds :type Float%20%28single-precision%29))
  ;[1 1 1] ЗерграшТаймер + дебагинфо
  (if (Variables|Default|GetZergRush?)
    (if (>= (Variables|Default|GetZergRushTimer) 0)
      (Development|PrintString (Utilities|String|Append "ZergRush timer: " (Utilities|String|ToString(Integer) (Variables|Default|GetZergRushTimer))) true true "(R=0.000000,G=0.660000,B=1.000000,A=1.000000)" 0.0)
      (Utilities|FlowControl|Delay 1.0)
      (Variables|Default|SetZergRushTimer (- (Variables|Default|GetZergRushTimer) 1))
      (else
        (Variables|Default|SetZergRush? false)
        (CallFunction|EmergencyOff)))))

(fn ConstructionScript)

(fn SpawnRoom
  (params (Parent :type Scene%20Component%20Object%20Reference))
  (bind _roomclasstospawn (Variables|Default|GetRoomClassToSpawn))
  (bind _returnvalue (Game|SpawnActorfromClass (Utilities|Array|Get(acopy) _roomclasstospawn (Math|Random|RandomIntegerinRange 0 (- (Utilities|Array|Length _roomclasstospawn) 1))) (Math|Transform|MakeTransform "0, 0, 0") "Undefined" 0 (Variables|Default|GetFloorNumber) false (Variables|Default|GetGameDificulty) "NewEnumerator0" false 0))
  (Transformation|AttachComponentToComponent _returnvalue Parent "None" "SnapToTarget" "SnapToTarget" "SnapToTarget" true))

(fn SpawnProps
  (bind _returnvalue (Game|SpawnActorfromClass "/Game/Bot/Zombie/AICharacter.AICharacter_C" (Transformation|GetWorldTransform (Variables|Default|GetPlayerStarter)) "AlwaysSpawn" 0 2e+01 0 5.0 0))
  (Default|ZergPlayer _returnvalue))

(fn Emergency
  (bind _outactors (Actor|GetAllActorsOfClass "/Game/Geometry/Props/Models/EmergencyLampActor.EmergencyLampActor_C"))
  (for _array_element _outactors
    (Default|EnableEmergency _array_element))
  (bind _outactors_2 (Actor|GetAllActorsOfClass "/Game/Geometry/Props/Models/Bulb.Bulb_C"))
  (for _array_element_2 _outactors_2
    (Default|DisaibleLight _array_element_2)))

(fn EmergencyOff
  (bind _outactors (Actor|GetAllActorsOfClass "/Game/Geometry/Props/Models/EmergencyLampActor.EmergencyLampActor_C"))
  (for _array_element _outactors
    (Default|DisableEmergency _array_element))
  (bind _outactors_2 (Actor|GetAllActorsOfClass "/Game/Geometry/Props/Models/Bulb.Bulb_C"))
  (for _array_element_2 _outactors_2
    (Default|EnableLight _array_element_2)))