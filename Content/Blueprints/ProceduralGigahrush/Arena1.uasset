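; Arena1 room piece for the procedural Gigahrush level, with a destructible wall and minimap representation.
; On BeginPlay it initializes the wall's material; in Debug it also spawns a secret room at its socket and makes the wall damageable.
; The first player overlap with MiniMapCollision reveals its paper sprites and sends element info to the minimap.
; CloseRoomHoles is deliberately overridden empty because this piece closes no holes.
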(event OnComponentBeginOverlap(MiniMapCollision)
  (params (OverlappedComponent :type Primitive%20Component%20Object%20Reference) (OtherActor :type Actor%20Object%20Reference) (OtherComp :type Primitive%20Component%20Object%20Reference) (OtherBodyIndex :type Integer) (bFromSweep :type Boolean) (SweepResult :type Hit%20Result%20Structure%20%28by%20ref%29))
  (if (Utilities|DoesObjectImplementInterface OtherActor "/Game/Blueprints/Interfaces/PlayerInterface.PlayerInterface_C")
    (Utilities|FlowControl|DoOnce false
      (:Completed
        (Rendering|SetVisibility (Variables|Default|GetPaperSprite) true false)
        (CallFunction|SendElementInfotoMinimap)))))

(event EventBeginPlay
  (|CallParentFunction)
  (CallFunction|InitializeDestructableWall (Variables|Default|GetMaterialToDestructableWall))
  (if (Variables|Default|GetDebug?)
    (CallFunction|SpawnSecretRoominCoridor (Variables|Default|GetSuperSecretRoomSocet))
    (Class|EnemyInterface|CanbeDamagedBoolSetter(Message) (Variables|/Script/Engine.ChildActorComponent|GetChildActor (Variables|Default|GetDestructableWall)) true)))

(event Collision|EventActorBeginOverlap
  (params (OtherActor :type Actor%20Object%20Reference))
  (|CallParentFunction OtherActor) ; This node is disabled and will not be called.\nDrag off pins to build functionality.
)

(event EventTick
  (params (DeltaSeconds :type Float%20%28single-precision%29))
  (|CallParentFunction DeltaSeconds) ; This node is disabled and will not be called.\nDrag off pins to build functionality.
)

(fn ConstructionScript
  (|CallParentFunction))

(fn CloseRoomHoles
  ;[1 1 1] Этот фрейм никакие дыры не закрывает, поэтому я переписал функцию и сделал её пустой
  (return))

(fn TurnOffPaperSpriteVisibility
  (Rendering|SetVisibility (Variables|Default|GetPaperSprite) false false)
  (return))

(fn TurnonPaperSpriteVisibility
  (Rendering|SetVisibility (Variables|Default|GetPaperSprite) true false)
  (return))