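; Procedural spawner for a Gigahrush level that builds a corridor chain on BeginPlay, with its length randomized by game difficulty.
; Each corridor frame snaps to the previous one's out socket and receives floor number, difficulty and a last-element flag.
; After two frames, a random roll can add a crossroads (perekrestok), which ends the chain unless PerekrestokInt blocks it.
; Afterwards it registers its super-secret-room socket with the GigahruchManager.
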(event Custom|CoridorSpawn
  (while (>= (Variables|Default|GetSpawnInt) 0)
    (CallFunction|SpawnFrame (Variables|Default|GetSocet))
    (if (>= (Variables|Default|GetPerekrestokInt) 2)
      (Variables|Default|SetSpawnInt (- (Variables|Default|GetSpawnInt) 1) :!label _label)
      (elif (Math|Random|RandomBool)
        (goto _label)
        (elif (Variables|Default|GetCanSpawnPerekrestok?)
          (CallFunction|SpawnPerekrestok (Variables|Default|GetSocet))
          (else
            (goto _label)))))))

(event EventBeginPlay
  (bind _gigahruchmanager (Variables|Default|GetGigahruchManager))
  (|CallParentFunction)
  (CallFunction|RandomizeCorridorPart)
  (CallFunction|CoridorSpawn)
  (Utilities|IsValid _gigahruchmanager
    (:Is%20Valid
      (Utilities|Array|Add (Variables|/Game/Blueprints/ProceduralGigahrush/GigahruchManager.GigahruchManager_C|GetSoketToSpawnSuperSecretRoom _gigahruchmanager) (Variables|Default|GetSocetToSuperSecretRoom)))
    (:Is%20Not%20Valid
      (Development|PrintString "No gigahrush manager"))))

(event Collision|EventActorBeginOverlap
  (params (OtherActor :type Actor%20Object%20Reference)))

(event EventTick
  (params (DeltaSeconds :type Float%20%28single-precision%29)))

(fn ConstructionScript)

(fn SpawnFrame
  (params (Parent :type Scene%20Component%20Object%20Reference))
  (Utilities|IsValid Parent
    (:Is%20Valid
      (LocalVariables|SetLocalSocet Parent))
    (:Is%20Not%20Valid
      (LocalVariables|SetLocalSocet (Variables|Default|GetImprovisedSocet))))
  (bind _returnvalue (Game|SpawnActorfromClass "/Game/Blueprints/ProceduralGigahrush/CoridorFraameChild.CoridorFraameChild_C" (Transformation|GetWorldTransform (LocalVariables|GetLocalSocet)) "Undefined" 0 false (Variables|Default|GetFloorNumber) (CallFunction|SpawnLastElement?) (Variables|Default|GetGameDificulty) "NewEnumerator0" false 0))
  (Transformation|AttachComponentToComponent _returnvalue (LocalVariables|GetLocalSocet) "None" "SnapToTarget" "SnapToTarget" "SnapToTarget" true)
  (Variables|Default|SetSocet (Variables|/Game/Blueprints/ProceduralGigahrush/CoridorFrame_Base.CoridorFrame_Base_C|GetOutSocet _returnvalue))
  (bind _output_get (Variables|Default|SetToPerekrestokSpawn (+ (Variables|Default|GetToPerekrestokSpawn) 1)))
  (if (>= _output_get 2)
    (Variables|Default|SetCanSpawnPerekrestok? true))
  (return (Variables|/Game/Blueprints/ProceduralGigahrush/CoridorFrame_Base.CoridorFrame_Base_C|GetOutSocet _returnvalue)))

(fn RandomizeCorridorPart
  (switch Utilities|FlowControl|Switch|SwitchonGameDificulty (Variables|Default|GetGameDificulty)
    (:NewEnumerator0
      (Variables|Default|SetSpawnInt (Math|Random|RandomIntegerinRange 3 6)))
    (:NewEnumerator1
      (Variables|Default|SetSpawnInt (Math|Random|RandomIntegerinRange 6 8)))
    (:NewEnumerator2
      (Variables|Default|SetSpawnInt (Math|Random|RandomIntegerinRange 5 7)))))

(fn SpawnPerekrestok
  (params (Socet :type Scene%20Component%20Object%20Reference))
  (Utilities|IsValid Socet
    (:Is%20Valid
      (LocalVariables|SetLocalSocet Socet))
    (:Is%20Not%20Valid
      (LocalVariables|SetLocalSocet (Variables|Default|GetImprovisedSocet))))
  (bind _returnvalue (Game|SpawnActorfromClass "/Game/Blueprints/ProceduralGigahrush/Perekrestok.Perekrestok_C" (Transformation|GetWorldTransform (LocalVariables|GetLocalSocet)) "Undefined" 0 (Variables|Default|GetFloorNumber) (CallFunction|SpawnLastElement?) (Variables|Default|GetGameDificulty) "NewEnumerator0" false 0))
  (Transformation|AttachComponentToComponent _returnvalue (LocalVariables|GetLocalSocet) "None" "SnapToTarget" "SnapToTarget" "SnapToTarget" true)
  (Variables|Default|SetSocet (Utilities|Array|Get(acopy) (Variables|/Game/Blueprints/ProceduralGigahrush/Perekrestok.Perekrestok_C|GetOutSocketArrey _returnvalue) (Math|Random|RandomIntegerinRange 0 2)))
  (Variables|Default|SetSpawnInt -1)
  (return (Utilities|Array|Get(acopy) (Variables|/Game/Blueprints/ProceduralGigahrush/Perekrestok.Perekrestok_C|GetOutSocketArrey _returnvalue) (Math|Random|RandomIntegerinRange 0 2))))

(fn SpawnLastElement?
  (if (== (Variables|Default|GetSpawnInt) 0)
    (return true)
    (else
      (return false))))