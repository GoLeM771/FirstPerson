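; Base corridor segment for the procedural Gigahrush level, spawning random rooms on its sockets and minimap-revealed by the player.
; BeginPlay fills one or two room sockets, plugs others with placeholders and offers a secret-room socket to the manager.
; While hole closing is active, sphere overlaps seal open ends and destroy disconnected frames.
; A trigger starts a timed zombie rush via recursive delayed events, keeping emergency lighting on until all rush zombies die.
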(event OnComponentBeginOverlap(SpawnEnemy)
  (params (OverlappedComponent :type Primitive%20Component%20Object%20Reference) (OtherActor :type Actor%20Object%20Reference) (OtherComp :type Primitive%20Component%20Object%20Reference) (OtherBodyIndex :type Integer) (bFromSweep :type Boolean) (SweepResult :type Hit%20Result%20Structure%20%28by%20ref%29))
  ;[1 1 1] При пересечении коллизии начинаем зерграш
  (Utilities|FlowControl|DoOnce false
    (:Completed
      (if (Variables|Default|GetCanSpawnEnemy?)
        (CallFunction|ZergRushStartTimerEvent)
        (Variables|Default|SetZergRush? true)
        (CallFunction|ZergRush)
        (CallFunction|Emergency)))))

(event OnComponentBeginOverlap(MiniMapCollision)
  (params (OverlappedComponent :type Primitive%20Component%20Object%20Reference) (OtherActor :type Actor%20Object%20Reference) (OtherComp :type Primitive%20Component%20Object%20Reference) (OtherBodyIndex :type Integer) (bFromSweep :type Boolean) (SweepResult :type Hit%20Result%20Structure%20%28by%20ref%29))
  (Utilities|Casting|CastToTPCharacter OtherActor)
  (Utilities|FlowControl|DoOnce false
    (:Completed
      (Rendering|SetVisibility (Variables|Default|GetPaperSprite) true false))))

(event Custom|OnCloseHoleEventStarted
  ;[1 1 1] На всякий случай автоотключение проверки коллизий и спавна заглушек
  (Utilities|FlowControl|Delay 5.0)
  (Variables|Default|SetStartClosingHoles? false))

(event Custom|ZergRush
  ;[1 1 1] Рекурсия. Зерграш.
  (if (Variables|Default|GetZergRush?)
    (for _array_element (Variables|Default|GetCoridorFrameToSpawnProps)
      (CallFunction|SpawnEnem _array_element true))
    (Utilities|FlowControl|Delay (Variables|Default|GetTimeBetweenSpawnEnemy))
    (CallFunction|ZergRush)
    (else
      (Development|PrintString "Stop spawn enemy" true true "(R=1.000000,G=0.118760,B=0.956838,A=1.000000)" 1e+01))))

(event Custom|CheckZergrushEnd
  ;[1 1 1] Рекурсивная функция. Если убиты все враги алярм выключается
  (Utilities|Array|Clear (Variables|Default|GetAiArrey))
  (bind _outactors (Actor|GetAllActorsOfClass "/Game/Bot/BaseEnemyCharacter/BaseZombieCharacter.BaseZombieCharacter_C"))
  (for _array_element _outactors
    (if (not (Variables|/Game/Bot/BaseEnemyCharacter/BaseZombieCharacter.BaseZombieCharacter_C|GetIsDead? _array_element))
      (if (Variables|/Game/Bot/BaseEnemyCharacter/BaseZombieCharacter.BaseZombieCharacter_C|GetZergRushSpwn? _array_element)
        (Utilities|Array|Add (Variables|Default|GetAiArrey) _array_element))))
  (if (Utilities|Array|IsValidIndex (Variables|Default|GetAiArrey))
    (Utilities|FlowControl|Delay 1.0)
    (CallFunction|CheckZergrushEnd)
    (else
      (CallFunction|EmergencyOff))))

(event Custom|FindNearCoridorFarameToSpwnEnemy
  ;[1 1 1] Выбор фрейма коридора где будут спавниться враги
  (bind _outactors (Actor|GetAllActorsOfClass "CoridorFrame_Base_C"))
  (for _array_element _outactors
    (if (Math|Boolean|ANDBoolean (Variables|/Game/Blueprints/ProceduralGigahrush/BaseGigahruchElement.BaseGigahruchElement_C|GetLastElement? _array_element) (== (Variables|/Game/Blueprints/ProceduralGigahrush/BaseGigahruchElement.BaseGigahruchElement_C|GetFloorNumber _array_element) 2) (Variables|CoridorFrame_Base_C|GetCanSpawnFromHere? _array_element))
      (Utilities|Array|Add (Variables|Default|GetCoridorFrameToSpawnProps) _array_element))))

(event Custom|DestroySelf
  ;[1 1 1] Самоуничтожить себя и всё что я заспавнил
  (for _array_element (Variables|Default|GetMySpawnedActors)
    (Utilities|IsValid _array_element
      (:Is%20Valid
        (Actor|DestroyActor _array_element))))
  (Actor|DestroyActor))

(event Custom|CheckInnerSocetCollision
  (bind _result (CallFunction|SphereTraceCheckCollision (Variables|Default|GetinnerSocet)))
  (if (not _result)
    (Development|PrintString (Utilities|String|Append "I need destroyed: " (Utilities|GetDisplayName self)) true true "(R=1.000000,G=0.000000,B=0.087363,A=1.000000)" 1e+01)
    (CallFunction|DestroySelf)))

(event Custom|ZergRushStartTimerEvent
  (Utilities|FlowControl|Delay 1.0)
  (Variables|Default|SetZergRushTimer (- (Variables|Default|GetZergRushTimer) 1))
  (if (<= (Variables|Default|GetZergRushTimer) 0)
    (Variables|Default|SetZergRush? false)
    (CallFunction|CheckZergrushEnd)
    (else
      (CallFunction|ZergRushStartTimerEvent))))

(event EventBeginPlay
  (bind _roomsocket (Variables|Default|GetRoomSocket))
  (bind _anotherroomsocet (Variables|Default|GetAnotherRoomSocet))
  (bind _roomsocket_2 (Variables|Default|GetRoomSocket))
  ;[1 1 1] Спавн комнат и плейсхолддеров
  (|CallParentFunction)
  (Utilities|FlowControl|Delay 1.0)
  (CallFunction|FillSocetArrey)
  (if (Variables|Default|GetDebug?)
    (CallFunction|SpawnRoom)
    (else
      (if (> (Math|Random|RandomIntegerinRange 0 10) 1)
        (Variables|Default|SetRoomSoket? false)
        (CallFunction|SpawnRoom _anotherroomsocet)
        (Utilities|Array|RemoveItem (Variables|Default|GetSocketArrey) _anotherroomsocet)
        (CallFunction|SpawnRoom _roomsocket_2)
        (Utilities|Array|RemoveItem (Variables|Default|GetSocketArrey) _roomsocket_2)
        (CallFunction|CloseRoomHoles)
        (else
          (Variables|Default|SetRoomSoket? true)
          (CallFunction|SpawnRoom _roomsocket)
          (Utilities|Array|RemoveItem (Variables|Default|GetSocketArrey) _roomsocket)
          (CallFunction|CloseRoomHoles)))
      (CallFunction|SendSockettoSpawnSecretRoom (Variables|Default|GetAnotherSuperSecretRoomSocet)))))

(event EventTick
  (params (DeltaSeconds :type Float%20%28single-precision%29))
  (bind _zergrushtimer (Variables|Default|GetZergRushTimer))
  ;[1 1 1] ЗерграшТаймер + дебагинфо + проверка на коллизию и закрытие дырок
  (Utilities|FlowControl|Sequence
    (:then_0
      (if (Variables|Default|GetStartClosingHoles?)
        (CallFunction|SphereTraceCheckCollision (Variables|Default|GetOutSocet))
        (CallFunction|CheckInnerSocetCollision)
        (Utilities|FlowControl|DoOnce false
          (:Completed
            (CallFunction|OnCloseHoleEventStarted)))))
    (:then_1
      (if (Variables|Default|GetZergRush?)
        (if (>= _zergrushtimer 0)
          (Development|PrintString (Utilities|String|Append "ZergRush timer: " (Utilities|String|ToString(Integer) _zergrushtimer)) true true "(R=0.000000,G=0.660000,B=1.000000,A=1.000000)" 0.0))))))

(fn ConstructionScript)

(fn SpawnRoom
  (params (Parent :type Scene%20Component%20Object%20Reference))
  (bind _returnvalue (Math|Transform|MakeTransform "0, 0, 0"))
  (if (Variables|Default|GetCanSpawnRoom?)
    (bind _output_get (LocalVariables|SetLocalRoomClass (CallFunction|GetRandomRoomClass)))
    (if (== _output_get "/Game/Blueprints/ProceduralGigahrush/ROOM_Sclad.ROOM_Sclad_C")
      (bind _returnvalue_2 (Game|SpawnActorfromClass (LocalVariables|GetLocalRoomClass) _returnvalue "Undefined" 0 false false (Variables|Default|GetFloorNumber) (Variables|Default|GetLastElement?) (Variables|Default|GetGameDificulty) "NewEnumerator0" (Variables|Default|GetDebug?) (Variables|Default|GetSpawnIterations) 0))
      (Utilities|Array|Add (Variables|Default|GetMySpawnedActors) _returnvalue_2)
      (Transformation|AttachComponentToComponent _returnvalue_2 Parent "None" "SnapToTarget" "SnapToTarget" "SnapToTarget" true)
      (Variables|Default|SetSpawnedRoomReference _returnvalue_2)
      (Variables|/Game/Blueprints/ProceduralGigahrush/Room_Parent.Room_Parent_C|SetCoridorFrameReference (Variables|Default|GetSpawnedRoomReference) self)
      (return)
      (else
        (bind _returnvalue_3 (Game|SpawnActorfromClass (LocalVariables|GetLocalRoomClass) _returnvalue "Undefined" 0 false false (Variables|Default|GetFloorNumber) (Variables|Default|GetLastElement?) (Variables|Default|GetGameDificulty) "NewEnumerator0" (Variables|Default|GetDebug?) (Variables|Default|GetSpawnIterations) 0))
        (Utilities|Array|Add (Variables|Default|GetMySpawnedActors) _returnvalue_3)
        (Transformation|AttachComponentToComponent _returnvalue_3 Parent "None" "SnapToTarget" "SnapToTarget" "SnapToTarget" true)
        (Variables|Default|SetSpawnedRoomReference _returnvalue_3)
        (Variables|/Game/Blueprints/ProceduralGigahrush/Room_Parent.Room_Parent_C|SetCoridorFrameReference (Variables|Default|GetSpawnedRoomReference) self)
        (return)))
    (else
      (return))))

(fn SpawnEnem
  (params (ZergRushSpwn? :type Boolean))
  (bind _returnvalue (Game|SpawnActorfromClass "/Game/Bot/BaseEnemyCharacter/BaseZombieCharacter.BaseZombieCharacter_C" (Transformation|GetWorldTransform (Variables|Default|GetPlayerStarter)) "AdjustIfPossibleButAlwaysSpawn" 0 (Variables|Default|GetPlayerRef) 0 ZergRushSpwn? 0))
  (Default|ZergPlayer _returnvalue))

(fn Emergency
  (bind _outactors (Actor|GetAllActorsOfClass "/Game/Geometry/Props/Models/EmergencyLampActor.EmergencyLampActor_C"))
  (for _array_element _outactors
    (Default|EnableEmergency _array_element))
  (bind _outactors_2 (Actor|GetAllActorsOfClass "/Game/Geometry/Props/Models/Bulb.Bulb_C"))
  (for _array_element_2 _outactors_2
    (Default|DisaibleLight _array_element_2)))

(fn EmergencyOff
  (bind _outactors (Actor|GetAllActorsOfClass "/Game/Geometry/Props/Models/EmergencyLampActor.EmergencyLampActor_C"))
  (for _array_element _outactors
    (Default|DisableEmergency _array_element))
  (bind _outactors_2 (Actor|GetAllActorsOfClass "/Game/Geometry/Props/Models/Bulb.Bulb_C"))
  (for _array_element_2 _outactors_2
    (Default|EnableLight _array_element_2)))

(fn RespawnRoom
  (if (Variables|Default|GetRoomWasRespawned?)
    (CallFunction|DestroyRoom)
    (Development|PrintString "Cant respawn room, destroy room" true true "(R=1.000000,G=0.000000,B=0.000000,A=1.000000)" 1e+01)
    (else
      (CallFunction|DestroyRoom)
      (if (Variables|Default|GetRoomSoket?)
        (CallFunction|SpawnRoom (Variables|Default|GetAnotherRoomSocet))
        (else
          (CallFunction|SpawnRoom (Variables|Default|GetRoomSocket))))
      (Variables|Default|SetRoomWasRespawned? true)
      (Development|PrintString "Room was respawned" true true "(R=1.000000,G=0.000000,B=0.000000,A=1.000000)" 1e+01))))

(fn DestroyRoom
  (bind _spawnedroomreference (Variables|Default|GetSpawnedRoomReference))
  (for _array_element (Variables|/Game/Blueprints/ProceduralGigahrush/Room_Parent.Room_Parent_C|GetSpawnedRoomArrey _spawnedroomreference)
    (Utilities|IsValid _array_element
      (:Is%20Valid
        (Actor|DestroyActor _array_element))))
  (Utilities|IsValid _spawnedroomreference
    (:Is%20Valid
      (Actor|DestroyActor _spawnedroomreference))
    (:Is%20Not%20Valid
      _))
  (return))

(fn SpawnPlaceHolder
  (params (parent :type Scene%20Component%20Object%20Reference))
  (if (not (== (Variables|Default|GetStairSocket) parent))
    (bind _returnvalue (Game|SpawnActorfromClass "/Game/Blueprints/ProceduralGigahrush/RoomPlaceholder.RoomPlaceholder_C" (Math|Transform|MakeTransform "0, 0, 0") "Undefined" 0 (Variables|Default|GetFloorNumber) (Variables|Default|GetLastElement?) (Variables|Default|GetGameDificulty) "NewEnumerator0" (Variables|Default|GetDebug?) (Variables|Default|GetSpawnIterations) 0))
    (Utilities|Array|Add (Variables|Default|GetMySpawnedActors) _returnvalue)
    (Transformation|AttachComponentToComponent _returnvalue parent "None" "SnapToTarget" "SnapToTarget" "SnapToTarget" true)
    (return _returnvalue)))

(fn GetRandomRoomClass
  (bind _roomclasstospawn (Variables|Default|GetRoomClassToSpawn))
  (return (Utilities|Array|Get(acopy) _roomclasstospawn (Math|Random|RandomIntegerinRange 0 (- (Utilities|Array|Length _roomclasstospawn) 1)))))

(fn FillSocetArrey
  (bind _socketarrey (Variables|Default|GetSocketArrey))
  (Utilities|Array|Add _socketarrey (Variables|Default|GetRoomSocket))
  (Utilities|Array|Add _socketarrey (Variables|Default|GetAnotherRoomSocet))
  (Utilities|Array|Add _socketarrey (Variables|Default|GetStayerSocet))
  (Utilities|Array|Add _socketarrey (Variables|Default|GetAnotherSuperSecretRoomSocet))
  (Utilities|Array|Add _socketarrey 0))

(fn CloseRoomHoles
  (for _array_element (Variables|Default|GetSocketArrey)
    (Utilities|IsValid _array_element
      (:Is%20Valid
        (CallFunction|SpawnPlaceHolder _array_element))))
  (return))

(fn SendSockettoSpawnSecretRoom
  (params (BoxCollision :type Scene%20Component%20Object%20Reference%20%28by%20ref%29))
  (bind _gigahruchmanager (Variables|Default|GetGigahruchManager))
  (Utilities|IsValid _gigahruchmanager
    (:Is%20Valid
      (Utilities|Array|Add (Variables|/Game/Blueprints/ProceduralGigahrush/GigahruchManager.GigahruchManager_C|GetSoketToSpawnSuperSecretRoom _gigahruchmanager) BoxCollision)
      (return))
    (:Is%20Not%20Valid
      (Development|PrintString (Utilities|String|Append (Utilities|GetDisplayName self) " Gigahrush manager is not valid"))
      (return))))

(fn CloseOutSocetHole
  (params (parent :type Scene%20Component%20Object%20Reference))
  (bind _returnvalue (CallFunction|SpawnPlaceHolder parent))
  (Transformation|AddActorLocalRotation _returnvalue (Math|Rotator|MakeRotator 0.0 0.0 9e+01) false false)
  (Transformation|SetActorScale3D _returnvalue "2.000000,2.000000,1.500000"))

(fn SphereTraceCheckCollision
  (params (OutSocetReference :type Scene%20Component%20Object%20Reference))
  (bind _returnvalue (Transformation|GetWorldLocation OutSocetReference))
  (bind _checkradius (Variables|Default|GetCheckRadius))
  (bind _returnvalue_2 (Collision|SphereOverlapActors _returnvalue _checkradius (Utilities|Array|MakeArray "ObjectTypeQuery1") "CoridorFrame_Base_C" (Utilities|Array|MakeArray self)))
  (Rendering|Debug|DrawDebugSphere _returnvalue _checkradius 12 "(R=1.000000,G=0.009454,B=0.000000,A=1.000000)" 0.0)
  (if _returnvalue_2
    (return true)
    (else
      (CallFunction|CloseOutSocetHole OutSocetReference)
      (return false))))

(fn SpawnBot
  (params (TransformForSpawn :type Transform) (NewParam1 :type Base%20Zombie%20Character%20Class%20Reference))
  (Game|SpawnActorfromClass NewParam1 TransformForSpawn "AlwaysSpawn" 0 0 0 true 0))

(fn SpawnNest
  (params (TransformForSpawn :type Transform) (NewParam1 :type Bug%20Nest%20Class%20Reference))
  (Game|SpawnActorfromClass NewParam1 TransformForSpawn "AlwaysSpawn" 0 0))