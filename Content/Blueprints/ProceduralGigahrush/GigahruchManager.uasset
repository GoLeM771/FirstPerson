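; Manager for the procedurally generated Gigahruch level, handling player placement, enemy trouble-spot activation and layout fix-ups.
; BeginPlay copies difficulty from LevelSpawner, then after a delay re-runs corridor collision traces to close holes.
; Events teleport the player to a random eligible element and activate one random floor-2 corridor, filtered by player distance, as enemy spawner, rebuilding navigation.
; A helper hands out free stair sockets; secret-room spawning is disconnected.
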(event Custom|SpawnPlayer
  (bind _gigahruchelementsshocanspawnplayer (Variables|Default|GetGigahruchElementsShoCanSpawnPlayer))
  (bind _returnvalue (Utilities|Array|Length _gigahruchelementsshocanspawnplayer))
  (bind _returnvalue_2 (- _returnvalue 1))
  (bind _returnvalue_3 (Math|Random|RandomIntegerinRange 0 _returnvalue_2))
  (bind _output (Utilities|Array|Get(acopy) _gigahruchelementsshocanspawnplayer _returnvalue_3))
  (bind _playerstarter (Variables|/Game/Blueprints/ProceduralGigahrush/BaseGigahruchElement.BaseGigahruchElement_C|GetPlayerStarter _output))
  (bind _returnvalue_4 (Transformation|GetWorldTransform _playerstarter))
  (bind (_location _rotation) (Math|Transform|BreakTransform _returnvalue_4))
  ;[1 1 1] Телепорт плеера
  (bind _outactors (Actor|GetAllActorsOfClass "/Game/Blueprints/ProceduralGigahrush/BaseGigahruchElement.BaseGigahruchElement_C"))
  (for _array_element _outactors
    (if (Variables|/Game/Blueprints/ProceduralGigahrush/BaseGigahruchElement.BaseGigahruchElement_C|GetCanSpawnPlayer? _array_element)
      (Utilities|Array|Add (Variables|Default|GetGigahruchElementsShoCanSpawnPlayer) _array_element)))
  (Transformation|Teleport (Game|GetPlayerCharacter 0) _location _rotation))

(event Custom|GetRandomCoridorFrameSpwner
  (bind _enemyspawnrearrey (Variables|Default|GetEnemySpawnreArrey))
  ;[1 1 1] Выбираем фрейм коридора который начнёт зерграш
  (bind _output_get (Variables|Default|SetEnemySpawnerCoridorFrme (Utilities|Array|Get(acopy) _enemyspawnrearrey (Math|Random|RandomIntegerinRange 0 (Utilities|Array|Length _enemyspawnrearrey)))))
  (Utilities|IsValid _output_get
    (:Is%20Valid
      (CallFunction|SelectTroublePlaceActivator (Variables|Default|GetEnemySpawnerCoridorFrme)))
    (:Is%20Not%20Valid
      (CallFunction|GetRandomCoridorFrameSpwner)))
  (Development|ExecuteConsoleCommand "RebuildNavigation" 0))

(event Custom|SelectTroublePlaceActivator
  (params (EnemySpawner :type Coridor%20Frame%20Base%20Object%20Reference))
  ;[1 1 1] Выбираем фрейм коридора который начнёт зерграш
  (Utilities|FlowControl|DoOnce false
    (:Completed
      (Development|PrintString (Utilities|GetDisplayName EnemySpawner))
      (Variables|/Game/Blueprints/ProceduralGigahrush/CoridorFrame_Base.CoridorFrame_Base_C|SetCanSpawnEnemy? EnemySpawner true)
      ;[1 1 1] Дебаг, что бы видеть коллизию
      (Development|SetHiddeninGame (Variables|/Game/Blueprints/ProceduralGigahrush/CoridorFrame_Base.CoridorFrame_Base_C|GetSpawnEnemy EnemySpawner) false false)
      (Default|FindNearCoridorFarametoSpwnEnemy EnemySpawner)
      (Development|PrintString (Utilities|String|Append "Trouble place activted in: " (Utilities|String|ToString(Vector) (Transformation|GetWorldLocation (Variables|/Game/Blueprints/ProceduralGigahrush/BaseGigahruchElement.BaseGigahruchElement_C|GetDefaultSceneRoot EnemySpawner))) " " (Utilities|GetDisplayName EnemySpawner)) true true "(R=0.000000,G=0.660000,B=1.000000,A=1.000000)" 4e+01))))

(event Custom|ActivateTroublePlace
  ;[1 1 1] Выбираем фрейм коридора который начнёт зерграш
  (Utilities|FlowControl|Delay 5.0)
  (bind _outactors (Actor|GetAllActorsOfClass "/Game/Blueprints/ProceduralGigahrush/CoridorFrame_Base.CoridorFrame_Base_C"))
  (for _array_element _outactors
    (if (and (Utilities|Enum|Equal(Enum) (Variables|/Game/Blueprints/ProceduralGigahrush/BaseGigahruchElement.BaseGigahruchElement_C|GetDistanceToPlayer _array_element) "NewEnumerator0") (== (Variables|/Game/Blueprints/ProceduralGigahrush/BaseGigahruchElement.BaseGigahruchElement_C|GetFloorNumber _array_element) 2))
      (Utilities|Array|Add (Variables|Default|GetEnemySpawnreArrey) _array_element)))
  (CallFunction|GetRandomCoridorFrameSpwner))

(event EventBeginPlay
  (Utilities|FlowControl|Delay 1.0)
  (Variables|Default|SetGameDificulty (Variables|/Game/Blueprints/ProceduralGigahrush/BaseGigahruchElement.BaseGigahruchElement_C|GetGameDificulty (Variables|Default|GetLevelSpawner)))
  (Utilities|FlowControl|Delay 2e+01)
  ;[1 1 1] На всякий случай ещё раз проверка коллизий у всех коридор фреймов и закрытие дыр
  (bind _outactors (Actor|GetAllActorsOfClass "/Game/Blueprints/ProceduralGigahrush/CoridorFrame_Base.CoridorFrame_Base_C"))
  (for _array_element _outactors
    (Default|SphereTraceCheckCollision _array_element (Variables|/Game/Blueprints/ProceduralGigahrush/CoridorFrame_Base.CoridorFrame_Base_C|GetOutSocet _array_element))))

(fn ConstructionScript)

(fn FindSocettoSpawnSecretRoom
  (params (SocetToSpawnSecretRoom :type Array%20of%20Scene%20Component%20Object%20References))
  (bind _output_get (LocalVariables|SetLocalSocetToSpawn (Utilities|Array|Get(acopy) SocetToSpawnSecretRoom (Math|Random|RandomIntegerinRange 0 (- (Utilities|Array|Length SocetToSpawnSecretRoom) 1)))))
  (Utilities|IsValid _output_get
    (:Is%20Valid
      (bind _asbase_gigahruch_element (Utilities|Casting|CastToBaseGigahruchElement (Components|GetOwner _output_get)))
      (return _output_get (Variables|/Game/Blueprints/ProceduralGigahrush/BaseGigahruchElement.BaseGigahruchElement_C|GetFloorNumber _asbase_gigahruch_element)))
    (:Is%20Not%20Valid
      (Development|PrintString "Cant spawn secret room" true true "(R=0.000000,G=0.660000,B=1.000000,A=1.000000)" 2e+01)
      (bind _output_get_2 (LocalVariables|SetLocalSocetToSpawn (Utilities|Array|Get(acopy) SocetToSpawnSecretRoom (Math|Random|RandomIntegerinRange 0 (- (Utilities|Array|Length SocetToSpawnSecretRoom) 1)))))
      (bind _asbase_gigahruch_element_2 (Utilities|Casting|CastToBaseGigahruchElement (Components|GetOwner _output_get_2)))
      (return _output_get_2 (Variables|/Game/Blueprints/ProceduralGigahrush/BaseGigahruchElement.BaseGigahruchElement_C|GetFloorNumber _asbase_gigahruch_element_2)))))

(fn SpawnSecretRoom)

(fn SpawnSuperSecretRoom)

(fn GetSocettoSpawnStayers
  (bind _localarreysocesttospawnstair (LocalVariables|GetLocalArreySocestToSpawnStair))
  (for _array_element (Variables|Default|GetFreeSocetArreyToSpawnStairs)
    (Utilities|IsValid _array_element
      (:Is%20Valid
        (Utilities|Array|Add (LocalVariables|GetLocalArreySocestToSpawnStair) _array_element))))
  (bind _output_get (LocalVariables|SetLocalSocetToSpawnStairs (Utilities|Array|Get(acopy) _localarreysocesttospawnstair (Math|Random|RandomIntegerinRange 0 (- (Utilities|Array|Length _localarreysocesttospawnstair) 1)))))
  (Utilities|Array|RemoveItem (Variables|Default|GetFreeSocetArreyToSpawnStairs) _output_get)
  (return (LocalVariables|GetLocalSocetToSpawnStairs)))