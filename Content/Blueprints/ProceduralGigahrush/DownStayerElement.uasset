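; Staircase element of the procedural Gigahrush level that opens wall holes at its connections and tracks the player's floor.
; On BeginPlay it runs a delayed sequence, destroying RoomPlaceholder actors around its inner socket, triggering same-floor corridor frames to close holes, then clearing the outer socket.
; Two minimap triggers switch the player's map and floor number to second or third floor.
; OnFloorSpawned asks LevelSpawnerWithLift to spawn the up stairs.
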(event OnComponentBeginOverlap(MiniMapCollision)
  (params (OverlappedComponent :type Primitive%20Component%20Object%20Reference) (OtherActor :type Actor%20Object%20Reference) (OtherComp :type Primitive%20Component%20Object%20Reference) (OtherBodyIndex :type Integer) (bFromSweep :type Boolean) (SweepResult :type Hit%20Result%20Structure%20%28by%20ref%29))
  (bind _returnvalue (Game|GetPlayerCharacter 0))
  (if (Utilities|DoesObjectImplementInterface OtherActor "/Game/Blueprints/Interfaces/PlayerInterface.PlayerInterface_C")
    (bind _map (Class|PlayerInterface|FullMapReferenceGetter(Message) _returnvalue))
    (Default|PlayerGotoSecondFloor _map)
    (Class|PlayerInterface|PlayeronFloorSetter(Message) _returnvalue 2)))

(event OnComponentBeginOverlap(MiniMapCollision1)
  (params (OverlappedComponent :type Primitive%20Component%20Object%20Reference) (OtherActor :type Actor%20Object%20Reference) (OtherComp :type Primitive%20Component%20Object%20Reference) (OtherBodyIndex :type Integer) (bFromSweep :type Boolean) (SweepResult :type Hit%20Result%20Structure%20%28by%20ref%29))
  (bind _returnvalue (Game|GetPlayerCharacter 0))
  (if (Utilities|DoesObjectImplementInterface OtherActor "/Game/Blueprints/Interfaces/PlayerInterface.PlayerInterface_C")
    (bind _map (Class|PlayerInterface|FullMapReferenceGetter(Message) _returnvalue))
    (Default|PlayerGotoThirdFloor _map)
    (Class|PlayerInterface|PlayeronFloorSetter(Message) _returnvalue 3)))

(event Custom|OpenWallHole
  (params (Target :type Scene%20Component%20Object%20Reference))
  (bind _returnvalue (Transformation|GetWorldLocation Target))
  (bind _outactors (Collision|SphereOverlapActors _returnvalue 2e+02 (Utilities|Array|MakeArray "ObjectTypeQuery1") "/Game/Blueprints/ProceduralGigahrush/RoomPlaceholder.RoomPlaceholder_C" (Utilities|Array|MakeArray self)))
  (Rendering|Debug|DrawDebugSphere _returnvalue 2e+02 12 "(R=1.000000,G=0.009454,B=0.000000,A=1.000000)" 0.0)
  (for _array_element _outactors
    (Actor|DestroyActor _array_element)))

(event Custom|StartCloasingAllHoles
  ;[1 1 1] Всё, что отнаследовано от coridor base начинает закрывать дыры в стенах
  (Utilities|FlowControl|DoOnce false
    (:Completed
      (bind _outactors (Actor|GetAllActorsOfClass "/Game/Blueprints/ProceduralGigahrush/CoridorFrame_Base.CoridorFrame_Base_C"))
      (for _array_element _outactors
        (if (== (Variables|/Game/Blueprints/ProceduralGigahrush/BaseGigahruchElement.BaseGigahruchElement_C|GetFloorNumber _array_element) (Variables|Default|GetFloorNumber))
          (Variables|/Game/Blueprints/ProceduralGigahrush/CoridorFrame_Base.CoridorFrame_Base_C|SetStartClosingHoles? _array_element true)))
      (Development|PrintString "Cloase holes event sended"))))

(event EventBeginPlay
  (|CallParentFunction)
  (Utilities|FlowControl|Delay 1.0)
  (CallFunction|OpenWallHole (Variables|Default|GetinnerSocet))
  (Utilities|FlowControl|Delay 1e+01)
  (CallFunction|StartCloasingAllHoles)
  (Utilities|FlowControl|Delay 1e+01)
  (CallFunction|OpenWallHole (Variables|Default|GetOutSocet)))

(event Collision|EventActorBeginOverlap
  (params (OtherActor :type Actor%20Object%20Reference))
  (|CallParentFunction OtherActor) ; This node is disabled and will not be called.\nDrag off pins to build functionality.
)

(event EventTick
  (params (DeltaSeconds :type Float%20%28single-precision%29))
  (|CallParentFunction DeltaSeconds) ; This node is disabled and will not be called.\nDrag off pins to build functionality.
)

(fn ConstructionScript
  (|CallParentFunction))

(fn OnFloorSpawned
  (bind _outactors (Actor|GetAllActorsOfClass "/Game/Blueprints/ProceduralGigahrush/LevelSpawnerWithLift.LevelSpawnerWithLift_C"))
  (Default|SpawnUpStairs (Utilities|Array|Get(acopy) _outactors)))