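; Crossroad corridor piece for the procedural Gigahrush level, with three out sockets and its own hole-closing logic replacing the inherited checks.
; Two seconds after BeginPlay, it sphere-checks each socket for neighboring corridor frames and attaches RoomPlaceholders to open ones.
; While flagged as respawned, Tick destroys it if no corridor surrounds PlayerStarter, also removing a UnitedCoridorFrame spawner's related parts.
; The first player overlap reveals its minimap sprites and reports it to the minimap.
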(event OnComponentBeginOverlap(MiniMapCollision)
  (params (OverlappedComponent :type Primitive%20Component%20Object%20Reference) (OtherActor :type Actor%20Object%20Reference) (OtherComp :type Primitive%20Component%20Object%20Reference) (OtherBodyIndex :type Integer) (bFromSweep :type Boolean) (SweepResult :type Hit%20Result%20Structure%20%28by%20ref%29))
  (if (Utilities|DoesObjectImplementInterface OtherActor "/Game/Blueprints/Interfaces/PlayerInterface.PlayerInterface_C")
    (Utilities|FlowControl|DoOnce false
      (:Completed
        (CallFunction|TurnonPaperSpriteVisibility)
        (CallFunction|SendElementInfotoMinimap)))))

(event Custom|CloseAllHoles
  (Utilities|FlowControl|DoOnce false
    (:Completed
      (for _array_element (Variables|Default|GetOutSocketArrey)
        (bind _closeholes (CallFunction|PerekrestokCheckCollision 2.5e+02 _array_element))
        (if _closeholes
          (CallFunction|PerekrestokSpawnPlaceholder _array_element)))
      (Development|PrintString (Utilities|String|Append (Utilities|GetDisplayName self) " close all holes") true true "(R=0.000000,G=0.660000,B=1.000000,A=1.000000)" 1e+01))))

(event EventBeginPlay
  (bind _outsocketarrey (Variables|Default|GetOutSocketArrey))
  (Utilities|Array|Add _outsocketarrey (Variables|Default|GetOutSocet_0))
  (Utilities|Array|Add _outsocketarrey (Variables|Default|GetOutSocet1))
  (Utilities|Array|Add _outsocketarrey (Variables|Default|GetOutSocet2))
  (|CallParentFunction)
  (Utilities|FlowControl|Delay 2.0)
  (CallFunction|CloseAllHoles)
  (if (not (Variables|Default|GetDebug?))
    (Variables|Default|SetFrameWasRespawned false)))

(event EventTick
  (params (DeltaSeconds :type Float%20%28single-precision%29))
  (if (Variables|Default|GetFrameWasRespawned)
    (bind _closeholes (CallFunction|PerekrestokCheckCollision 6e+02 (Variables|Default|GetPlayerStarter)))
    (if _closeholes
      ;[1 1 1] Удалить огрызок большой части, не забыть для каждого типа больших элементов перезаписывать функцию.
      (bind _asunited_coridor_frame (Utilities|Casting|CastToUnitedCoridorFrame (Variables|Default|GetActorWhoSpawnMe))
        (:then
          (Default|RemoveRelatedParts _asunited_coridor_frame))
        (:CastFailed
          _))
      (Actor|DestroyActor))))

(fn ConstructionScript)

(fn CloseRoomHoles
  ;[1 1 1] Этот фрейм никакие дыры не закрывает, поэтому я переписал функцию и сделал её пустой
  (return))

(fn PerekrestokSpawnPlaceholder
  (params (Parent :type Scene%20Component%20Object%20Reference))
  (bind _returnvalue (Game|SpawnActorfromClass "/Game/Blueprints/ProceduralGigahrush/RoomPlaceholder.RoomPlaceholder_C" (Math|Transform|MakeTransform "0, 0, 0") "Undefined" 0 (Variables|Default|GetFloorNumber) false (Variables|Default|GetGameDificulty) "NewEnumerator0" true 0 0))
  (Transformation|AttachComponentToComponent _returnvalue Parent "None" "SnapToTarget" "SnapToTarget" "SnapToTarget" true)
  (Transformation|AddActorLocalRotation _returnvalue "0,90.000000, 0" false false)
  (Transformation|SetActorScale3D _returnvalue "2.000000,2.000000,1.500000"))

(fn PerekrestokCheckCollision
  (params (SphereСруслRadius :type Float%20%28single-precision%29) (Target :type Scene%20Component%20Object%20Reference))
  (bind _returnvalue (Transformation|GetWorldLocation Target))
  (bind _returnvalue_2 (Collision|SphereOverlapActors _returnvalue SphereСруслRadius (Utilities|Array|MakeArray "ObjectTypeQuery1") "/Game/Blueprints/ProceduralGigahrush/CoridorFrame_Base.CoridorFrame_Base_C" (Utilities|Array|MakeArray self)))
  (Rendering|Debug|DrawDebugSphere _returnvalue SphereСруслRadius 12 "(R=1.000000,G=0.009454,B=0.000000,A=1.000000)" 0.0)
  (if _returnvalue_2
    (return false)
    (else
      (Variables|Default|SetStartClosingHoles? false)
      (return true))))

(fn SphereTraceCheckCollision
  (params (OutSocetReference :type Scene%20Component%20Object%20Reference))
  ;[1 1 1] Перекрёсток по другому будет закрывать коллизию
  (return false))

(fn TurnOffPaperSpriteVisibility
  (Rendering|SetVisibility (Variables|Default|GetPaperSprite) false true)
  (return))

(fn TurnonPaperSpriteVisibility
  (Rendering|SetVisibility (Variables|Default|GetPaperSprite) true true)
  (return))