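; Small composite corridor piece for the procedural Gigahrush level generator, built around child-actor corridor frames.
; While StartCheckCollision is set, Tick runs BigElementCheckCollision on ChildActor1 against corridor frames, and FillElementArrey registers that child's actor.
; SphereOverlapCheck tests for overlaps ignoring its own children, with debug drawing and logging.
; FindSocetToSpawnStairs returns immediately, leaving its free-socket registration for the level spawner unreachable.
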(event EventBeginPlay
  (|CallParentFunction) ; This node is disabled and will not be called.\nDrag off pins to build functionality.
)

(event Collision|EventActorBeginOverlap
  (params (OtherActor :type Actor%20Object%20Reference))
  (|CallParentFunction OtherActor) ; This node is disabled and will not be called.\nDrag off pins to build functionality.
)

(event EventTick
  (params (DeltaSeconds :type Float%20%28single-precision%29))
  (if (Variables|Default|GetStartCheckCollision?)
    (CallFunction|BigElementCheckCollision (Variables|Default|GetChildActor1) "/Game/Blueprints/ProceduralGigahrush/CoridorFrame_Base.CoridorFrame_Base_C")))

(fn ConstructionScript
  (|CallParentFunction))

(fn FillElementArrey
  (Utilities|Array|Add (Variables|Default|GetChildAActorsArrey) (Variables|/Script/Engine.ChildActorComponent|GetChildActor (Variables|Default|GetChildActor1)))
  (return))

(fn FindSocettoSpawnStairs
  (params (LevelSpawnerReference :type Level%20Spawner%20Object%20Reference))
  (return))

(fn SphereOverlapCheck
  (params (ActorClassFilter :type Object%20Class%20Reference) (CheckLocation :type Scene%20Component%20Object%20Reference) (SphereCheckerRadius :type Float%20%28single-precision%29))
  (bind _returnvalue (Transformation|GetWorldLocation CheckLocation))
  (bind (_outactors _returnvalue_2) (Collision|SphereOverlapActors _returnvalue SphereCheckerRadius (Utilities|Array|MakeArray "ObjectTypeQuery1") ActorClassFilter (Utilities|Array|MakeArray (Variables|/Script/Engine.ChildActorComponent|GetChildActor (Variables|Default|GetChildActor)) (Variables|/Script/Engine.ChildActorComponent|GetChildActor (Variables|Default|GetChildActor2)) (Variables|/Script/Engine.ChildActorComponent|GetChildActor (Variables|Default|GetChildActor4)) (Variables|/Script/Engine.ChildActorComponent|GetChildActor (Variables|Default|GetChildActor5)) (Variables|/Script/Engine.ChildActorComponent|GetChildActor (Variables|Default|GetChildActor1)))))
  (Rendering|Debug|DrawDebugSphere _returnvalue 1e+02 12 "(R=1.000000,G=0.009454,B=0.000000,A=1.000000)" 0.0)
  (for _array_element _outactors
    (Development|PrintString (Utilities|String|Append (Utilities|GetDisplayName self) " collision witch: " (Utilities|GetDisplayName _array_element)) true true "(R=0.000000,G=0.660000,B=1.000000,A=1.000000)" 2e+01))
  (return _returnvalue_2))