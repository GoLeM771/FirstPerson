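; Destructible placeholder prop for procedural Gigahrush rooms, with a static mesh, settable material and wall health, that accepts enemy-style damage.
; Simple and point damage events reduce health only while damage is enabled by a setter.
; At zero health it notifies its assigned room actor through DestroyPropsMessage, then destroys itself once.
; Enemy getter functions for body parts, coordinates, mesh, death and spawning are stubs returning defaults.
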(event EventSimpleDamageEnemy
  (params (Damage :type Float%20%28single-precision%29))
  (if (Variables|Default|GetCanBeDamaged?)
    (Variables|Default|SetWallHealth (- (Variables|Default|GetWallHealth) Damage))
    (if (<= (Variables|Default|GetWallHealth) 0.0)
      (Utilities|FlowControl|DoOnce false
        (:Completed
          (Class|GigahruchInterface|DestroyProps(Message) (Variables|Default|GetRoomActor))
          (Actor|DestroyActor))))))

(event Game|Damage|EventPointDamage
  (params (Damage :type Float%20%28single-precision%29) (DamageType :type Damage%20Type%20Object%20Reference) (HitLocation :type Vector :default "0, 0, 0") (HitNormal :type Vector :default "0, 0, 0") (HitComponent :type Primitive%20Component%20Object%20Reference) (BoneName :type Name :default "None") (ShotFromDirection :type Vector :default "0, 0, 0") (InstigatedBy :type Controller%20Object%20Reference) (DamageCauser :type Actor%20Object%20Reference) (HitInfo :type Hit%20Result%20Structure%20%28by%20ref%29))
  (if (Variables|Default|GetCanBeDamaged?)
    (Variables|Default|SetWallHealth (- (Variables|Default|GetWallHealth) Damage))
    (if (<= (Variables|Default|GetWallHealth) 0.0)
      (Utilities|FlowControl|DoOnce false
        (:Completed
          (Class|GigahruchInterface|DestroyProps(Message) (Variables|Default|GetRoomActor))
          (Actor|DestroyActor))))))

(event EventSetWallMaterial
  (params (MaterialToSet :type Material%20Interface%20Object%20Reference))
  (Rendering|Material|SetMaterial (Variables|Default|GetStaticMesh) 0 MaterialToSet))

(event EventCanbeDamagedBoolSetter
  (params (CanBeDamaged? :type Boolean))
  (Variables|Default|SetCanBeDamaged? CanBeDamaged?))

(event EventRoomReferenceSetter
  (params (ActorReference :type Actor%20Object%20Reference))
  (Variables|Default|SetRoomActor ActorReference))

(fn ConstructionScript)

(fn ArmsCoordinateGetter
  (return 0))

(fn BodyPartMassGetter
  (return 0.0))

(fn BodyPartsArreyGetter
  (return 0))

(fn CanSpawnEnemyGetter
  (return false))

(fn EnemySkeletalMeshGetter
  (return 0))

(fn HeadCoordinateGetter
  (return 0))

(fn IsDeadGetter
  (return false))

(fn TorsoCoordinateGetter
  (return 0))