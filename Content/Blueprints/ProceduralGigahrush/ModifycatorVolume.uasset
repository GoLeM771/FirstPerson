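; ModifycatorVolume is a trigger box that applies a room modifier to the player in the procedural Gigahrush level.
; Setter events supply the room reference and modifier type, the latter also enabling the volume.
; Overlaps report player presence to the room and toggle the respirator system, boosted walk speed or enemy spawning.
; A DoOnce guards entry effects and resets on exit for gas and speed, but not for enemy spawning.
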(event OnComponentBeginOverlap(Box)
  (params (OverlappedComponent :type Primitive%20Component%20Object%20Reference) (OtherActor :type Actor%20Object%20Reference) (OtherComp :type Primitive%20Component%20Object%20Reference) (OtherBodyIndex :type Integer) (bFromSweep :type Boolean) (SweepResult :type Hit%20Result%20Structure%20%28by%20ref%29))
  (bind _returnvalue (Game|GetPlayerCharacter 0))
  (if (Variables|Default|GetEnabled?)
    (if (Utilities|DoesObjectImplementInterface OtherActor "/Game/Blueprints/Interfaces/PlayerInterface.PlayerInterface_C")
      (CallFunction|PlayerinRoomBoolSetter true)
      (Utilities|FlowControl|DoOnce false
        (:Completed
          (switch Utilities|FlowControl|Switch|SwitchonRoomModificator (Variables|Default|GetRoomModifycator)
            (:NewEnumerator0
              (Class|PlayerInterface|ResperatorSystemActivateSetter(Message) _returnvalue true))
            (:NewEnumerator1
              (Class|GigahruchInterface|SeyRespawnerSpawnEnemy(Message) (Variables|Default|GetRoomRference)))
            (:NewEnumerator2
              (Class|PlayerInterface|SetCharacterMaxWolkSpeed(Message) _returnvalue (Variables|Default|GetBoostedWalkSpeed)))))))))

(event OnComponentEndOverlap(Box)
  (params (OverlappedComponent :type Primitive%20Component%20Object%20Reference) (OtherActor :type Actor%20Object%20Reference) (OtherComp :type Primitive%20Component%20Object%20Reference) (OtherBodyIndex :type Integer))
  (bind _returnvalue (Game|GetPlayerCharacter 0))
  (bind _returnvalue_2 (Game|GetPlayerCharacter 0))
  (if (Variables|Default|GetEnabled?)
    (if (Utilities|DoesObjectImplementInterface OtherActor "/Game/Blueprints/Interfaces/PlayerInterface.PlayerInterface_C")
      (CallFunction|PlayerinRoomBoolSetter false)
      (switch Utilities|FlowControl|Switch|SwitchonRoomModificator (Variables|Default|GetRoomModifycator)
        (:NewEnumerator0
          (Class|PlayerInterface|ResperatorSystemActivateSetter(Message) _returnvalue_2 false)
          (Utilities|FlowControl|DoOnce false) ; enters at Reset
        )
        (:NewEnumerator1
          (Class|GigahruchInterface|SeyRespawnerStopSpawn(Message) (Variables|Default|GetRoomRference)))
        (:NewEnumerator2
          (Class|PlayerInterface|SetCharacterMaxWolkSpeed(Message) _returnvalue_2 (Variables|Default|GetNormalWolkSpeed))
          (Utilities|FlowControl|DoOnce false) ; enters at Reset
        )))))

(event EventBeginPlay)

(event Collision|EventActorBeginOverlap
  (params (OtherActor :type Actor%20Object%20Reference)))

(event EventTick
  (params (DeltaSeconds :type Float%20%28single-precision%29)))

(event EventRoomModyfycatorSetter
  (params (RoomModyf :type RoomModificator%20Enum :default "NewEnumerator0"))
  (Variables|Default|SetRoomModifycator RoomModyf)
  (Variables|Default|SetEnabled? true))

(event EventRoomReferenceSetter
  (params (Room :type Actor%20Object%20Reference))
  (Variables|Default|SetRoomRference Room))

(fn ConstructionScript)

(fn PlayerinRoomBoolSetter
  (params (PlayerInRoom? :type Boolean))
  (bind _roomrference (Variables|Default|GetRoomRference))
  (Utilities|IsValid _roomrference
    (:Is%20Valid
      (Class|GigahruchInterface|PlayerinRoomSetter(Message) _roomrference PlayerInRoom?))
    (:Is%20Not%20Valid
      (Development|PrintString (Utilities|String|Append (Utilities|GetDisplayName self) " Room ref is not valid") true true "(R=0.000000,G=0.660000,B=1.000000,A=1.000000)" 2e+01)))
  (return))

(fn DistancetoPlayerGetter
  (return "NewEnumerator0"))

(fn FloorNumGetter
  (return 0))

(fn WorldLocationGetterInterface
  (return "0, 0, 0"))