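; Disabler_Button is an interactable button actor that switches off a referenced modificator volume.
; An overlap area registers and unregisters the button as an interactable with the overlapping actor.
; On interaction, gated by the built-in CanBeDamaged flag, it sends TurnOffModificatorMessage to a valid ModificatorVolumeRef and changes its text to "Pressed".
; PickupModelGetter exposes the Cube as its model.
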(event OnComponentBeginOverlap(InteracteableArea)
  (params (OverlappedComponent :type Primitive%20Component%20Object%20Reference) (OtherActor :type Actor%20Object%20Reference) (OtherComp :type Primitive%20Component%20Object%20Reference) (OtherBodyIndex :type Integer) (bFromSweep :type Boolean) (SweepResult :type Hit%20Result%20Structure%20%28by%20ref%29))
  (Class|PickupInteract|RegisterInteracteable(Message) OtherActor self))

(event OnComponentEndOverlap(InteracteableArea)
  (params (OverlappedComponent :type Primitive%20Component%20Object%20Reference) (OtherActor :type Actor%20Object%20Reference) (OtherComp :type Primitive%20Component%20Object%20Reference) (OtherBodyIndex :type Integer))
  (Class|PickupInteract|UnregisterInteracteable(Message) OtherActor self))

(event EventBeginPlay
  (|CallParentFunction) ; This node is disabled and will not be called.\nDrag off pins to build functionality.
)

(event Collision|EventActorBeginOverlap
  (params (OtherActor :type Actor%20Object%20Reference))
  (|CallParentFunction OtherActor) ; This node is disabled and will not be called.\nDrag off pins to build functionality.
)

(event EventTick
  (params (DeltaSeconds :type Float%20%28single-precision%29))
  (|CallParentFunction DeltaSeconds) ; This node is disabled and will not be called.\nDrag off pins to build functionality.
)

(event EventInteraction
  (params (Interacter :type Actor%20Object%20Reference))
  (bind _modificatorvolumeref (Variables|Default|GetModificatorVolumeRef))
  (if (Variables|Default|GetCanBeDamaged?)
    (Utilities|IsValid _modificatorvolumeref
      (:Is%20Valid
        (Class|GigahruchInterface|TurnOffModificator(Message) _modificatorvolumeref)
        (Rendering|Components|TextRender|SetText (Variables|Default|GetTextRender) (Utilities|Text|MakeLiteralText "Pressed"))))))

(fn ConstructionScript
  (|CallParentFunction))

(fn PickupModelGetter
  (return (Variables|Default|GetCube)))