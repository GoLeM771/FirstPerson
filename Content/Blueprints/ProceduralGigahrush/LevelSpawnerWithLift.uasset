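; Procedural map room with an elevator that spawns stairs and acts as a drop-off point for Civil quests.
; BeginPlay passes TargetLevel to the child elevator, spawns a secret-room placeholder and registers the room in the player's floor-two map list.
; OnFloorSpawned attaches down stairs to a free socket after a delay, and CloseRoomHoles is overridden empty to avoid extra placeholders.
; A Civil entering the SpawnEnemy volume increments matching quests and stops following.
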(event OnComponentBeginOverlap(SpawnEnemy)
  (params (OverlappedComponent :type Primitive%20Component%20Object%20Reference) (OtherActor :type Actor%20Object%20Reference) (OtherComp :type Primitive%20Component%20Object%20Reference) (OtherBodyIndex :type Integer) (bFromSweep :type Boolean) (SweepResult :type Hit%20Result%20Structure%20%28by%20ref%29))
  (bind _ascivil (Utilities|Casting|CastToCivil OtherActor))
  (bind _outactors (Actor|GetAllActorsOfClass "/Game/Blueprints/QuestSystem/Quests/bp_baseQuest.bp_baseQuest_C"))
  (for _array_element _outactors
    (bind _asbp_base_quest (Utilities|Casting|CastTobp_baseQuest _array_element)
      (:then
        (if (Utilities|Enum|Equal(Enum) (Variables|/Game/Blueprints/QuestSystem/Quests/bp_baseQuest.bp_baseQuest_C|GetQuestType _asbp_base_quest) (Variables|Default|GetQuestType))
          (Default|CountPlus _asbp_base_quest)
          (Variables|/Game/Bot/Civil/Civil.Civil_C|SetCanFollow _ascivil false)
          (else
            (Development|PrintString (Utilities|String|Append "Текущий квест " (Utilities|String|EnumtoString (Variables|/Game/Blueprints/QuestSystem/Quests/bp_baseQuest.bp_baseQuest_C|GetQuestType _asbp_base_quest)))))))
      (:CastFailed
        (Development|PrintString "CastFailed" true true "(R=0.000000,G=0.660000,B=1.000000,A=1.000000)" 1e+01)))))

(event Custom|SpawnDownStairs
  (Utilities|FlowControl|Delay 2.0)
  (bind _returnvalue (Game|SpawnActorfromClass "/Game/Blueprints/ProceduralGigahrush/DownStayerElement.DownStayerElement_C" (Math|Transform|MakeTransform "0, 0, 0") "Undefined" 0 false false 3 false (Variables|Default|GetGameDificulty) "NewEnumerator0" false 0 0))
  (bind _localsocettospawn1 (CallFunction|FindFreeSocettoSpawnStairs))
  (Transformation|AttachComponentToComponent _returnvalue _localsocettospawn1 "None" "SnapToTarget" "SnapToTarget" "SnapToTarget" true))

(event Custom|SpawnUpStairs
  (Utilities|FlowControl|Delay 2.0)
  (bind _returnvalue (Game|SpawnActorfromClass "/Game/Blueprints/ProceduralGigahrush/UpStayerElement.UpStayerElement_C" (Math|Transform|MakeTransform "0, 0, 0") "Undefined" 0 false false 1 false (Variables|Default|GetGameDificulty) "NewEnumerator0" false 0 0))
  (bind _localsocettospawn1 (CallFunction|FindFreeSocettoSpawnStairs))
  (Transformation|AttachComponentToComponent _returnvalue _localsocettospawn1 "None" "SnapToTarget" "SnapToTarget" "SnapToTarget" true))

(event EventBeginPlay
  (|CallParentFunction)
  (bind _asbp_elevator (Utilities|Casting|CastToBP_Elevator (Variables|/Script/Engine.ChildActorComponent|GetChildActor (Variables|Default|GetBP_Elevator))))
  (Variables|/Game/Blueprints/Elevator/BP_Elevator.BP_Elevator_C|SetTargetLevel _asbp_elevator (Variables|Default|GetTargetLevel))
  (Utilities|FlowControl|Delay 1.0)
  (CallFunction|SpawnPlaceHolder (Variables|Default|GetSocetToSuperSecretRoom))
  (bind _map (Class|PlayerInterface|FullMapReferenceGetter(Message) (Game|GetPlayerCharacter 0)))
  (Utilities|Array|Add (Variables|/Game/Blueprints/UI/MiniMap_v2/FullMap.FullMap_C|GetKnownElementOnFloorTwo _map) self))

(event Collision|EventActorBeginOverlap
  (params (OtherActor :type Actor%20Object%20Reference)))

(event EventTick
  (params (DeltaSeconds :type Float%20%28single-precision%29))
  (|CallParentFunction DeltaSeconds))

(fn ConstructionScript)

(fn OnFloorSpawned
  (CallFunction|SpawnDownStairs))

(fn CloseRoomHoles
  ;[1 1 1] Чтоб не спавнил лишние плейсхолдеры
  (return))

(fn TurnOffPaperSpriteVisibility
  (Rendering|SetVisibility (Variables|Default|GetPaperSprite) false true)
  (return))

(fn TurnonPaperSpriteVisibility
  (Rendering|SetVisibility (Variables|Default|GetPaperSprite) true true)
  (return))