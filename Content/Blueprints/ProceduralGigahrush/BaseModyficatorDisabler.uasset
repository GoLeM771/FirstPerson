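; BaseModyficatorDisabler is a damageable actor that switches off a room modifier in the procedural Gigahrush level.
; Setter events supply the modificator volume reference and the flag that allows damage.
; On point damage, if allowed and the reference is valid, it sends the turn-off message to the volume, swaps the cube material and changes its text to show the disabled state.
; The remaining getter functions are stubs returning defaults.
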(event EventBeginPlay)

(event Collision|EventActorBeginOverlap
  (params (OtherActor :type Actor%20Object%20Reference)))

(event EventTick
  (params (DeltaSeconds :type Float%20%28single-precision%29)))

(event Game|Damage|EventPointDamage
  (params (Damage :type Float%20%28single-precision%29) (DamageType :type Damage%20Type%20Object%20Reference) (HitLocation :type Vector :default "0, 0, 0") (HitNormal :type Vector :default "0, 0, 0") (HitComponent :type Primitive%20Component%20Object%20Reference) (BoneName :type Name :default "None") (ShotFromDirection :type Vector :default "0, 0, 0") (InstigatedBy :type Controller%20Object%20Reference) (DamageCauser :type Actor%20Object%20Reference) (HitInfo :type Hit%20Result%20Structure%20%28by%20ref%29))
  (bind _modificatorvolumeref (Variables|Default|GetModificatorVolumeRef))
  (if (Variables|Default|GetCanBeDamaged?)
    (Utilities|IsValid _modificatorvolumeref
      (:Is%20Valid
        (Class|GigahruchInterface|TurnOffModificator(Message) _modificatorvolumeref)
        (Rendering|Material|SetMaterial (Variables|Default|GetCube) 0 "/Game/Biomass/Materials/BaseMaterial_M.BaseMaterial_M")
        (Rendering|Components|TextRender|SetText (Variables|Default|GetTextRender) (Utilities|Text|MakeLiteralText "Room mod disabled"))))))

(event EventCanbeDamagedBoolSetter
  (params (CanBeDamaged? :type Boolean))
  (Variables|Default|SetCanBeDamaged? CanBeDamaged?))

(event EventRoomModyfReferenceSetter
  (params (RoomModyfRef :type Actor%20Object%20Reference))
  (Variables|Default|SetModificatorVolumeRef RoomModyfRef))

(fn ConstructionScript)

(fn ArmsCoordinateGetter
  (return 0))

(fn BodyPartMassGetter
  (return 0.0))

(fn BodyPartsArreyGetter
  (return 0))

(fn CanSpawnEnemyGetter
  (return false))

(fn DistancetoPlayerGetter
  (return "NewEnumerator0"))

(fn EnemySkeletalMeshGetter
  (return 0))

(fn FloorNumGetter
  (return 0))

(fn HeadCoordinateGetter
  (return 0))

(fn IsDeadGetter
  (return false))

(fn TorsoCoordinateGetter
  (return 0))

(fn WorldLocationGetterInterface
  (return "0, 0, 0"))