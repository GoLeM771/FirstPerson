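; Composite corridor segment for the procedural Gigahrush level, built from child-actor frames and a crossroad (Perekrestok).
; On BeginPlay it passes generation data to its children, then briefly sphere-checks two end frames on Tick against other corridor frames.
; A collision destroys that frame and flags the crossroad.
; After the check window, outside debug and while spawns remain, it asks the level spawner to respawn it on collision or continue from a random socket.
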(event Custom|StopSpawnEvent
  ;[1 1 1] Команда на респавн и команда перекрёстку начать проверку коллизий, если коллизит - удалить перекрёсток
  (Default|RespawnBigElement (Variables|Default|GetLevelSpawnerReference)))

(event EventBeginPlay
  (bind _levelspawnerreference (Variables|Default|GetLevelSpawnerReference))
  (|CallParentFunction)
  (CallFunction|FillElementArrey)
  (CallFunction|FillChildActorVariables)
  (Utilities|FlowControl|Delay 0.2)
  (Variables|Default|SetStartCheckCollision? true)
  (Utilities|FlowControl|Delay 1.0)
  (Variables|Default|SetStartCheckCollision? false)
  (if (not (Variables|Default|GetDebug?))
    (if (> (Variables|/Game/Blueprints/ProceduralGigahrush/LevelSpawner.LevelSpawner_C|GetSpawnInt _levelspawnerreference) 0)
      ;[1 1 1] Проверяется на event tick
      (if (Variables|Default|GetCollisiuonWitchEnotherActor?)
        (CallFunction|StopSpawnEvent)
        (else
          (Default|SpawnBigCoridorPart _levelspawnerreference (Default|GetRandomSocettoSpawn _levelspawnerreference)))))))

(event Collision|EventActorBeginOverlap
  (params (OtherActor :type Actor%20Object%20Reference))
  (|CallParentFunction OtherActor) ; This node is disabled and will not be called.\nDrag off pins to build functionality.
)

(event EventTick
  (params (DeltaSeconds :type Float%20%28single-precision%29))
  ;[1 1 1] Проверка на коллизии, если коллизит - удаляем коллизящий элемент и отсылаем команду на респавн
  (|CallParentFunction DeltaSeconds)
  (if (Variables|Default|GetStartCheckCollision?)
    (CallFunction|BigElementCheckCollision (Variables|Default|GetChildActor4) "/Game/Blueprints/ProceduralGigahrush/CoridorFrame_Base.CoridorFrame_Base_C")
    (CallFunction|BigElementCheckCollision (Variables|Default|GetChildActor5) "/Game/Blueprints/ProceduralGigahrush/CoridorFrame_Base.CoridorFrame_Base_C")))

(fn ConstructionScript
  (|CallParentFunction))

(fn GetSocettoSpawn
  (for _array_element (Variables|Default|GetChildAActorsArrey)
    (bind _ascoridor_frame_base (Utilities|Casting|CastToCoridorFrame_Base _array_element))
    (if (Variables|/Game/Blueprints/ProceduralGigahrush/CoridorFrame_Base.CoridorFrame_Base_C|GetCanSpawnFromHere? _ascoridor_frame_base)
      (Utilities|Array|Add (Variables|Default|GetSocketArrey) (Variables|/Game/Blueprints/ProceduralGigahrush/CoridorFrame_Base.CoridorFrame_Base_C|GetOutSocet _ascoridor_frame_base))))
  (return (Variables|Default|GetSocketArrey)))

(fn FillElementArrey
  (bind _childaactorsarrey (Variables|Default|GetChildAActorsArrey))
  (Utilities|Array|Add _childaactorsarrey (Variables|/Script/Engine.ChildActorComponent|GetChildActor (Variables|Default|GetChildActor5)))
  (Utilities|Array|Add _childaactorsarrey (Variables|/Script/Engine.ChildActorComponent|GetChildActor (Variables|Default|GetChildActor4)))
  (Utilities|Array|Add _childaactorsarrey (Variables|/Script/Engine.ChildActorComponent|GetChildActor (Variables|Default|GetChildActor2)))
  (Utilities|Array|Add _childaactorsarrey (Variables|/Script/Engine.ChildActorComponent|GetChildActor (Variables|Default|GetChildActor1)))
  (Utilities|Array|Add _childaactorsarrey (Variables|/Script/Engine.ChildActorComponent|GetChildActor (Variables|Default|GetChildActor)))
  (return))

(fn FillChildActorVariables
  (for _array_element (Variables|Default|GetChildAActorsArrey)
    (bind _asbase_gigahruch_element (Utilities|Casting|CastToBaseGigahruchElement _array_element))
    (Variables|/Game/Blueprints/ProceduralGigahrush/BaseGigahruchElement.BaseGigahruchElement_C|SetFloorNumber _asbase_gigahruch_element (Variables|Default|GetFloorNumber))
    (Variables|/Game/Blueprints/ProceduralGigahrush/BaseGigahruchElement.BaseGigahruchElement_C|SetSpawnIterations _asbase_gigahruch_element (Variables|Default|GetSpawnIterations))
    (Variables|/Game/Blueprints/ProceduralGigahrush/BaseGigahruchElement.BaseGigahruchElement_C|SetActorWhoSpawnMe _asbase_gigahruch_element self)
    (if (Variables|Default|GetLastElement?)
      (Variables|/Game/Blueprints/ProceduralGigahrush/BaseGigahruchElement.BaseGigahruchElement_C|SetLastElement? _asbase_gigahruch_element true)))
  (return))

(fn BigElementCheckCollision
  (params (CoridorFrameReference :type Child%20Actor%20Component%20Object%20Reference) (ActorClassFilter :type Object%20Class%20Reference))
  (bind _output_get (LocalVariables|SetLocalChildActor (Variables|/Script/Engine.ChildActorComponent|GetChildActor CoridorFrameReference)))
  (bind _ascoridor_frame_base (Utilities|Casting|CastToCoridorFrame_Base _output_get)
    (:then
      (Utilities|IsValid _ascoridor_frame_base
        (:Is%20Valid
          (bind _collision (CallFunction|SphereOverlapCheck ActorClassFilter (Variables|/Game/Blueprints/ProceduralGigahrush/CoridorFrame_Base.CoridorFrame_Base_C|GetOutSocet _ascoridor_frame_base) 3e+02))
          (if _collision
            (CallFunction|TellAboutCollision (Variables|Default|GetChildActor2) (LocalVariables|GetLocalChildActor))
            (return)
            (else
              (bind _collision_2 (CallFunction|SphereOverlapCheck ActorClassFilter (Variables|/Game/Blueprints/ProceduralGigahrush/CoridorFrame_Base.CoridorFrame_Base_C|GetSpawnEnemy _ascoridor_frame_base) 3e+02))
              (if _collision_2
                (CallFunction|TellAboutCollision (Variables|Default|GetChildActor2) (LocalVariables|GetLocalChildActor))
                (return)
                (else
                  (return))))))
        (:Is%20Not%20Valid
          _)))
    (:CastFailed
      _))
  (return))

(fn TellAboutCollision
  (params (PerekrestokActor :type Child%20Actor%20Component%20Object%20Reference) (ActorToDelete :type Actor%20Object%20Reference))
  (Variables|Default|SetStartCheckCollision? false)
  (Variables|Default|SetCollisiuonWitchEnotherActor? true)
  (bind _asperekrestok (Utilities|Casting|CastToPerekrestok (Variables|/Script/Engine.ChildActorComponent|GetChildActor PerekrestokActor))
    (:then
      (Variables|/Game/Blueprints/ProceduralGigahrush/Perekrestok.Perekrestok_C|SetFrameWasRespawned _asperekrestok true))
    (:CastFailed
      _))
  (bind _ascoridor_frame_base (Utilities|Casting|CastToCoridorFrame_Base ActorToDelete)
    (:then
      (Default|DestroySelf _ascoridor_frame_base))
    (:CastFailed
      _))
  (return))

(fn SphereOverlapCheck
  (params (ActorClassFilter :type Object%20Class%20Reference) (CheckLocation :type Scene%20Component%20Object%20Reference) (SphereCheckerRadius :type Float%20%28single-precision%29))
  (bind _returnvalue (Transformation|GetWorldLocation CheckLocation))
  (bind (_outactors _returnvalue_2) (Collision|SphereOverlapActors _returnvalue SphereCheckerRadius (Utilities|Array|MakeArray "ObjectTypeQuery1") ActorClassFilter (Variables|Default|GetChildAActorsArrey)))
  (Rendering|Debug|DrawDebugSphere _returnvalue SphereCheckerRadius 12 "(R=1.000000,G=0.009454,B=0.000000,A=1.000000)" 0.0)
  (for _array_element _outactors
    (Development|PrintString (Utilities|String|Append (Utilities|GetDisplayName self) " collision witch: " (Utilities|GetDisplayName _array_element)) true true "(R=0.000000,G=0.660000,B=1.000000,A=1.000000)" 2e+01))
  (return _returnvalue_2))

(fn RemoveRelatedParts
  ;[1 1 1] При удалении перекрёстка удалить связанную часть
  (Components|DestroyComponent (Variables|Default|GetChildActor5))
  (return))

(fn FindSocettoSpawnStairs
  (params (LevelSpawnerReference :type Level%20Spawner%20Object%20Reference))
  (bind _collisionchecker1 (Variables|Default|GetCollisionChecker1))
  (bind _collisionchecker2 (Variables|Default|GetCollisionChecker2))
  (Utilities|FlowControl|Sequence
    (:then_0
      (bind _collision (CallFunction|SphereOverlapCheck "/Game/Blueprints/ProceduralGigahrush/CoridorFrame_Base.CoridorFrame_Base_C" _collisionchecker1 2e+02))
      (if (not _collision)
        (Utilities|Array|Add (Variables|/Game/Blueprints/ProceduralGigahrush/LevelSpawner.LevelSpawner_C|GetFreeSocetToSpawn LevelSpawnerReference) _collisionchecker1)))
    (:then_1
      (bind _collision_2 (CallFunction|SphereOverlapCheck "/Game/Blueprints/ProceduralGigahrush/CoridorFrame_Base.CoridorFrame_Base_C" _collisionchecker2 2e+02))
      (if (not _collision_2)
        (Utilities|Array|Add (Variables|/Game/Blueprints/ProceduralGigahrush/LevelSpawner.LevelSpawner_C|GetFreeSocetToSpawn LevelSpawnerReference) _collisionchecker2)))
    (:then_2
      (return))))