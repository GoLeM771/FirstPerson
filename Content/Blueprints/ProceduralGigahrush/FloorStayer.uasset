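; FloorStayer procedurally builds a corridor layout for the Gigahrush generator on BeginPlay.
; It picks a random segment count based on how many FloorStayers exist, then chains CoridorFrame actors socket to socket.
; From the second frame on, it randomly inserts up to two crossroads (Perekrestok) of random type, rotating their out sockets.
; It finally registers two super secret room sockets with the GigahruchManager.
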(event Custom|CoridorSpawn
  (while (>= (Variables|Default|GetSpawnInt) 0)
    (CallFunction|SpawnFrame (Variables|Default|GetSocet))
    (if (>= (Variables|Default|GetPerekrestokInt) 2)
      _
      (elif (Math|Random|RandomBool)
        _
        (elif (Variables|Default|GetCanSpawnPerekrestok?)
          (CallFunction|SpawnPerekrestok (Variables|Default|GetSocet)))))
    (Variables|Default|SetSpawnInt (- (Variables|Default|GetSpawnInt) 1))))

(event EventBeginPlay
  (bind _outactors (Actor|GetAllActorsOfClass "/Game/Blueprints/ProceduralGigahrush/GigahruchManager.GigahruchManager_C"))
  (Variables|Default|SetGigahruchManager (Utilities|Array|Get(acopy) _outactors))
  (CallFunction|RandomizeCorridorPart)
  (CallFunction|CoridorSpawn)
  (Utilities|Array|Add (Variables|/Game/Blueprints/ProceduralGigahrush/GigahruchManager.GigahruchManager_C|GetSoketToSpawnSuperSecretRoom (Variables|Default|GetGigahruchManager)) (Variables|Default|GetSocetToSuperSecretRoom1))
  (Utilities|Array|Add (Variables|/Game/Blueprints/ProceduralGigahrush/GigahruchManager.GigahruchManager_C|GetSoketToSpawnSuperSecretRoom (Variables|Default|GetGigahruchManager)) (Variables|Default|GetSocetToSuperSecretRoom)))

(event Collision|EventActorBeginOverlap
  (params (OtherActor :type Actor%20Object%20Reference)))

(event EventTick
  (params (DeltaSeconds :type Float%20%28single-precision%29)))

(fn ConstructionScript)

(fn SpawnFrame
  (params (Parent :type Scene%20Component%20Object%20Reference))
  (Utilities|IsValid Parent
    (:Is%20Valid
      (LocalVariables|SetLocalSocet Parent))
    (:Is%20Not%20Valid
      (LocalVariables|SetLocalSocet (Variables|Default|GetImprovisedSocet))))
  (bind _returnvalue (Game|SpawnActorfromClass "/Game/Blueprints/ProceduralGigahrush/CoridorFrame.CoridorFrame_C" (Transformation|GetWorldTransform (LocalVariables|GetLocalSocet)) "Undefined" 0 (Variables|Default|GetGigahruchManager) 0))
  (Transformation|AttachComponentToComponent _returnvalue (LocalVariables|GetLocalSocet) "None" "SnapToTarget" "SnapToTarget" "SnapToTarget" true)
  (Variables|Default|SetSocet (Variables|/Game/Blueprints/ProceduralGigahrush/CoridorFrame.CoridorFrame_C|GetOutSocet _returnvalue))
  (bind _output_get (Variables|Default|SetToPerekrestokSpawn (+ (Variables|Default|GetToPerekrestokSpawn) 1)))
  (if (>= _output_get 2)
    (Variables|Default|SetCanSpawnPerekrestok? true))
  (return (Variables|/Game/Blueprints/ProceduralGigahrush/CoridorFrame.CoridorFrame_C|GetOutSocet _returnvalue)))

(fn RandomizeCorridorPart
  (bind _outactors (Actor|GetAllActorsOfClass "FloorStayer_C"))
  (switch int (Utilities|Array|Length _outactors)
    (:Default
      (Variables|Default|SetSpawnInt (Math|Random|RandomIntegerinRange 8 10) :!label _label))
    (:0
      (Development|PrintString "Not valid situation suka"))
    (:1
      (goto _label))
    (:2
      (Variables|Default|SetSpawnInt (Math|Random|RandomIntegerinRange 5 7)))
    (:3
      (Variables|Default|SetSpawnInt (Math|Random|RandomIntegerinRange 2 4)))))

(fn SpawnPerekrestok
  (params (Socet :type Scene%20Component%20Object%20Reference))
  (Utilities|IsValid Socet
    (:Is%20Valid
      (LocalVariables|SetLocalSocet Socet))
    (:Is%20Not%20Valid
      (LocalVariables|SetLocalSocet (Variables|Default|GetImprovisedSocet))))
  (bind _returnvalue (Game|SpawnActorfromClass (Utilities|Array|Get(acopy) (Variables|Default|GetPerekrestokType) (Math|Random|RandomIntegerinRange 0 1)) (Transformation|GetWorldTransform (LocalVariables|GetLocalSocet)) "Undefined" 0 0))
  (Transformation|AttachComponentToComponent _returnvalue (LocalVariables|GetLocalSocet) "None" "SnapToTarget" "SnapToTarget" "SnapToTarget" true)
  (Variables|Default|SetSocet (Variables|/Game/Blueprints/ProceduralGigahrush/Perekrestok.Perekrestok_C|GetOutSocet _returnvalue))
  (Variables|Default|SetPerekrestokInt (+ (Variables|Default|GetPerekrestokInt) 1))
  (Default|RotateOutSoket? _returnvalue)
  (return (Variables|/Game/Blueprints/ProceduralGigahrush/Perekrestok.Perekrestok_C|GetOutSocet _returnvalue)))