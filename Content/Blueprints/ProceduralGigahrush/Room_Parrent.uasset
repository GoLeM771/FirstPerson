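; Base room actor for the procedural Gigahrush level, which fills its sockets with sub-rooms.
; On BeginPlay it either spawns a SmallRoom on a random socket or offers one to GigahruchManager as a secret-room candidate, optionally adding a Sortir.
; Overlap with another room, reported through CheckCollisionWitchEnotherRoom, makes its corridor frame respawn the room.
; Helpers open the child-actor door, spawn props and spawn a secret room directly.
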(event Custom|CheckCollisionWitchEnotherRoom
  (params (Actor :type Actor%20Object%20Reference) (HitResult :type Hit%20Result%20Structure))
  (Utilities|Casting|CastToRoom_Parrent Actor)
  (if (not (== Actor self))
    (Development|PrintString (Utilities|String|Append "Collision witch: " (Utilities|GetDisplayName Actor) " and " (Utilities|GetDisplayName self)) true true "(R=1.000000,G=0.000000,B=0.000000,A=1.000000)" 15.0)
    (Variables|Default|SetCollisiuonWitchEnotherActor? true)
    (Rendering|Debug|DrawDebugSphere (.Location (Collision|BreakHitResult HitResult)) 1e+02 12 "(R=1.000000,G=0.000000,B=0.000000,A=1.000000)" 5e+01 1.0)
    (Default|RespawnRoom (Variables|Default|GetCoridorFrameReference))))

(event Custom|OpenDoor
  (bind _asin_door (Utilities|Casting|CastToInDoor (Variables|/Script/Engine.ChildActorComponent|GetChildActor (Variables|Default|GetDoorActor))))
  (Default|OpenDoor1 _asin_door))

(event EventBeginPlay
  (bind _gigahruchmanager (Variables|Default|GetGigahruchManager))
  (bind _sokettospawnsecretroom (Variables|/Game/Blueprints/ProceduralGigahrush/GigahruchManager.GigahruchManager_C|GetSoketToSpawnSecretRoom _gigahruchmanager))
  (|CallParentFunction)
  (if (Variables|Default|GetSpawnRoom?)
    (if (Math|Random|RandomBool)
      ;[1 1 1] Спавним 2ю комнату?
      (CallFunction|SpawnSecondRoom?)
      (if (Variables|Default|GetSpawnSortir?)
        (CallFunction|SpawnSortir))
      (else
        ;[1 1 1] Отправляем рандомный сокет на гигахрущ менеджер. На какой то из отправленых заспавнится секретная комната
        (Utilities|IsValid _gigahruchmanager :!label _label
          (:Is%20Valid
            (switch int (Math|Random|RandomIntegerinRange 0 2)
              (:Default
                (Utilities|Array|Add _sokettospawnsecretroom (Variables|Default|GetSmallRoomSocet1) :!label _label_2))
              (:0
                (goto _label_2))
              (:1
                (Utilities|Array|Add _sokettospawnsecretroom (Variables|Default|GetSmallRoomSocet2)))
              (:2
                (Utilities|Array|Add _sokettospawnsecretroom (Variables|Default|GetSmallRoomSocet3))))
            (if (Variables|Default|GetSpawnSortir?)
              (CallFunction|SpawnSortir)))
          (:Is%20Not%20Valid
            (Development|PrintString "no gigahrosh manager")))))
    (else
      (goto _label))))

(event Collision|EventActorBeginOverlap
  (params (OtherActor :type Actor%20Object%20Reference)))

(event EventTick
  (params (DeltaSeconds :type Float%20%28single-precision%29))
  (if (not (Variables|Default|GetDebug?))
    (Utilities|IsValid (Variables|Default|GetCoridorFrameReference)
      (:Is%20Not%20Valid
        (Development|PrintString "Coridor frame not valid" true true "(R=1.000000,G=0.000000,B=0.000000,A=1.000000)" 0.0)))))

(fn ConstructionScript)

(fn SpawnSecretRoom
  (switch int (Math|Random|RandomIntegerinRange 0 2)
    (:Default
      (Variables|Default|SetAttachToSocet (Variables|Default|GetSmallRoomSocet1) :!label _label))
    (:0
      (goto _label))
    (:1
      (Variables|Default|SetAttachToSocet (Variables|Default|GetSmallRoomSocet2)))
    (:2
      (Variables|Default|SetAttachToSocet (Variables|Default|GetSmallRoomSocet3))))
  (bind _returnvalue (Game|SpawnActorfromClass "/Game/Blueprints/ProceduralGigahrush/SecretRoom.SecretRoom_C" (Transformation|GetWorldTransform (Variables|Default|GetAttachToSocet)) "Undefined" 0 0 false "NewEnumerator0" "NewEnumerator0" false 0))
  (Transformation|AttachComponentToComponent _returnvalue (Variables|Default|GetAttachToSocet) "None" "SnapToTarget" "SnapToTarget" "SnapToTarget" true)
  (Development|PrintString (Utilities|String|Append "Room spawned in " (Utilities|String|ToString(Vector) (Transformation|GetWorldLocation (Variables|Default|GetAttachToSocet)))) true true "(R=0.000000,G=0.660000,B=1.000000,A=1.000000)" 2e+01)
  (Variables|Default|SetSecretRoomSpawned? true))

(fn SpawnProps
  (params (NewParam :type Base%20Ai%20Character%20Class%20Reference))
  (bind _returnvalue (Game|SpawnActorfromClass NewParam (Transformation|GetWorldTransform (Variables|Default|GetBox)) "AlwaysSpawn" 0 2e+01 0 5.0 false false 0))
  (Default|ZergPlayer _returnvalue))

(fn SpawnSortir
  (bind _sortirsocet (Variables|Default|GetSortirSocet))
  (bind _returnvalue (Game|SpawnActorfromClass "/Game/Blueprints/ProceduralGigahrush/Sortir.Sortir_C" (Transformation|GetWorldTransform _sortirsocet) "Undefined" 0 (Variables|Default|GetFloorNumber) false (Variables|Default|GetGameDificulty) "NewEnumerator0" false 0))
  (Transformation|AttachComponentToComponent _returnvalue _sortirsocet "None" "SnapToTarget" "SnapToTarget" "SnapToTarget" true)
  (Utilities|Array|Add (Variables|Default|GetSpawnedRoomArrey) _returnvalue))

(fn SpawnSecondRoom?
  (switch int (Math|Random|RandomIntegerinRange 0 2)
    (:Default
      (Variables|Default|SetAttachToSocet (Variables|Default|GetSmallRoomSocet1) :!label _label))
    (:0
      (goto _label))
    (:1
      (Variables|Default|SetAttachToSocet (Variables|Default|GetSmallRoomSocet2)))
    (:2
      (Variables|Default|SetAttachToSocet (Variables|Default|GetSmallRoomSocet3))))
  (bind _returnvalue (Game|SpawnActorfromClass "/Game/Blueprints/ProceduralGigahrush/SmallRoom.SmallRoom_C" (Transformation|GetWorldTransform (Variables|Default|GetAttachToSocet)) "Undefined" 0 (Variables|Default|GetFloorNumber) false (Variables|Default|GetGameDificulty) "NewEnumerator0" false 0))
  (Transformation|AttachComponentToComponent _returnvalue (Variables|Default|GetAttachToSocet) "None" "SnapToTarget" "SnapToTarget" "SnapToTarget" true)
  (Utilities|Array|Add (Variables|Default|GetSpawnedRoomArrey) _returnvalue))