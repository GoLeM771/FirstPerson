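; Living-room module for the procedural Gigahrush level, built on inherited room logic.
; On BeginPlay it registers with its modifier volume, then after a second hides paper sprites, spawns two civilians and drops loot, activating a room modification if Debug is set.
; Drop re-rolls at each branch per loot point to spawn a filter pickup, health pickup or nothing.
; Six plane overlaps feed a check for collisions with other rooms.
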(event OnComponentBeginOverlap(Plane1)
  (params (OverlappedComponent :type Primitive%20Component%20Object%20Reference) (OtherActor :type Actor%20Object%20Reference) (OtherComp :type Primitive%20Component%20Object%20Reference) (OtherBodyIndex :type Integer) (bFromSweep :type Boolean) (SweepResult :type Hit%20Result%20Structure%20%28by%20ref%29))
  (CallFunction|CheckCollisionWitchEnotherRoom OtherActor SweepResult))

(event OnComponentBeginOverlap(Plane3)
  (params (OverlappedComponent :type Primitive%20Component%20Object%20Reference) (OtherActor :type Actor%20Object%20Reference) (OtherComp :type Primitive%20Component%20Object%20Reference) (OtherBodyIndex :type Integer) (bFromSweep :type Boolean) (SweepResult :type Hit%20Result%20Structure%20%28by%20ref%29))
  (CallFunction|CheckCollisionWitchEnotherRoom OtherActor SweepResult))

(event OnComponentBeginOverlap(Plane4)
  (params (OverlappedComponent :type Primitive%20Component%20Object%20Reference) (OtherActor :type Actor%20Object%20Reference) (OtherComp :type Primitive%20Component%20Object%20Reference) (OtherBodyIndex :type Integer) (bFromSweep :type Boolean) (SweepResult :type Hit%20Result%20Structure%20%28by%20ref%29))
  (CallFunction|CheckCollisionWitchEnotherRoom OtherActor SweepResult))

(event OnComponentBeginOverlap(Plane7)
  (params (OverlappedComponent :type Primitive%20Component%20Object%20Reference) (OtherActor :type Actor%20Object%20Reference) (OtherComp :type Primitive%20Component%20Object%20Reference) (OtherBodyIndex :type Integer) (bFromSweep :type Boolean) (SweepResult :type Hit%20Result%20Structure%20%28by%20ref%29))
  (CallFunction|CheckCollisionWitchEnotherRoom OtherActor SweepResult))

(event OnComponentBeginOverlap(Plane6)
  (params (OverlappedComponent :type Primitive%20Component%20Object%20Reference) (OtherActor :type Actor%20Object%20Reference) (OtherComp :type Primitive%20Component%20Object%20Reference) (OtherBodyIndex :type Integer) (bFromSweep :type Boolean) (SweepResult :type Hit%20Result%20Structure%20%28by%20ref%29))
  (CallFunction|CheckCollisionWitchEnotherRoom OtherActor SweepResult))

(event OnComponentBeginOverlap(Plane2)
  (params (OverlappedComponent :type Primitive%20Component%20Object%20Reference) (OtherActor :type Actor%20Object%20Reference) (OtherComp :type Primitive%20Component%20Object%20Reference) (OtherBodyIndex :type Integer) (bFromSweep :type Boolean) (SweepResult :type Hit%20Result%20Structure%20%28by%20ref%29))
  (CallFunction|CheckCollisionWitchEnotherRoom OtherActor SweepResult))

(event Collision|EventActorBeginOverlap
  (params (OtherActor :type Actor%20Object%20Reference))
  (|CallParentFunction OtherActor) ; This node is disabled and will not be called.\nDrag off pins to build functionality.
)

(event EventTick
  (params (DeltaSeconds :type Float%20%28single-precision%29))
  (|CallParentFunction DeltaSeconds) ; This node is disabled and will not be called.\nDrag off pins to build functionality.
)

(event EventBeginPlay
  (Class|GigahruchInterface|RoomReferenceSetter(Message) (Variables|/Script/Engine.ChildActorComponent|GetChildActor (Variables|Default|GetRoomModyficatorVolume)) self)
  (Utilities|FlowControl|Delay 1.0)
  (CallFunction|TurnOffPaperSpriteVisibility)
  (CallFunction|SpawnCivil "/Game/Bot/Civil/Civil.Civil_C" (Transformation|GetWorldTransform (Variables|Default|GetCivilSpawner)))
  (CallFunction|SpawnCivil "/Game/Bot/Civil/Civil.Civil_C" (Transformation|GetWorldTransform (Variables|Default|GetCivilSpawner2)))
  (CallFunction|Drop)
  (if (Variables|Default|GetDebug?)
    (CallFunction|ActivateRoomModifications "NewEnumerator2")))

(fn ConstructionScript
  (|CallParentFunction))

(fn Drop
  (bind _returnvalue (Math|Random|RandomIntegerinRange 0 3))
  (for _array_element (Utilities|Array|MakeArray (Variables|Default|GetLootPoint) (Variables|Default|GetLootPoint1) (Variables|Default|GetLootPoint2) (Variables|Default|GetLootPoint3))
    (if (== _returnvalue 0)
      (Game|SpawnActorfromClass "/Game/Blueprints/Pickups/FiltersPickUP.FiltersPickUP_C" (Transformation|GetWorldTransform _array_element) "Undefined" 0 0.0 "NewEnumerator7" 0 0 1 false 0)
      (elif (not (== _returnvalue 1))
        (if (== _returnvalue 2)
          (Game|SpawnActorfromClass "/Game/Blueprints/Pickups/HealthPickup.HealthPickup_C" (Transformation|GetWorldTransform _array_element) "Undefined" 0 0.1 "NewEnumerator0" 20 1 0 false 0)
          (elif (== _returnvalue 3)
            _))))))