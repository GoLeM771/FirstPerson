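; Laser tripwire mine that explodes when an AI character, or the player if DamagePlayer is set, crosses its beam.
; On BeginPlay a forward line trace finds the beam end, spawns the laser particle and stretches the trigger box along it.
; Detonation fires effects and a radial impulse, applies sphere-overlap damage to AI and player characters regardless of DamagePlayer, then destroys the mine.
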(event OnComponentBeginOverlap(BoxExp)
  (params (OverlappedComponent :type Primitive%20Component%20Object%20Reference) (OtherActor :type Actor%20Object%20Reference) (OtherComp :type Primitive%20Component%20Object%20Reference) (OtherBodyIndex :type Integer) (bFromSweep :type Boolean) (SweepResult :type Hit%20Result%20Structure%20%28by%20ref%29))
  (bind _returnvalue (Transformation|GetActorLocation))
  (if (Variables|Default|GetDamagePlayer?)
    (Utilities|Casting|CastToTPCharacter OtherActor
      (:then
        _)
      (:CastFailed
        (Utilities|Casting|CastToAICharacter OtherActor :!label _label)))
    (else
      (goto _label)))
  (Effects|SpawnEmitteratLocation "/Game/StarterContent/Particles/P_Explosion.P_Explosion" _returnvalue)
  (Class|RadialForceComponent|FireImpulse (Variables|Default|GetRadialForce))
  (Audio|PlaySoundatLocation "/Game/StarterContent/Audio/Explosion_Cue.Explosion_Cue" _returnvalue "0, 0, 0" 1.0 1.0 0.0 0 0 0)
  (Components|DestroyComponent (Variables|Default|GetLaserBean))
  (bind _outactors (Collision|SphereOverlapActors (Transformation|GetActorLocation) (Variables|Default|GetDebugSphereRadius) (Utilities|Array|MakeArray "ObjectTypeQuery8" "ObjectTypeQuery3") 0))
  (for _array_element _outactors
    (bind _asaicharacter (Utilities|Casting|CastToAICharacter _array_element)
      (:then
        (Default|HealthMinus _asaicharacter 1e+02 false))
      (:CastFailed
        _))
    (bind _astpcharacter (Utilities|Casting|CastToTPCharacter _array_element))
    (Default|ModifyStat _astpcharacter -0.5 "NewEnumerator0"))
  (Actor|DestroyActor))

(event EventBeginPlay
  (bind _actorstoignore (Variables|Default|GetActorsToIgnore))
  (bind _laserstartpoint (Variables|Default|GetLaserStartPoint))
  ;[1 1 1] Создали лазерный луч + триггер
  (Collision|SetCollisionEnabled (Variables|Default|GetBoxExp) "NoCollision")
  (bind _output_get (Variables|Default|SetBeanEndPoint (+ (Transformation|GetWorldLocation _laserstartpoint) (* (Math|Vector|GetForwardVector _laserstartpoint) 5e+03))))
  (if (Variables|Default|GetDamagePlayer?)
    _
    (else
      (Utilities|Array|Add _actorstoignore (Game|Player|GetPlayerPawn 0))))
  (bind (_outhit _returnvalue) (Collision|LineTraceByChannel (Transformation|GetWorldLocation (Variables|Default|GetLaserStartPoint)) _output_get "TraceTypeQuery1" false _actorstoignore "None"))
  (if _returnvalue
    (Variables|Default|SetBeanEndPoint (.Location (Collision|BreakHitResult _outhit))))
  (CallFunction|CreateBean (Transformation|GetWorldLocation (Variables|Default|GetLaserStartPoint)) (Variables|Default|GetBeanEndPoint))
  (CallFunction|ScaleTriggerBox (Variables|Default|GetBeanEndPoint))
  (Collision|SetCollisionEnabled (Variables|Default|GetBoxExp) "QueryAndPhysics"))

(fn ConstructionScript)

(fn CreateBean
  (params (StartLocation :type Vector) (EndLocation :type Vector))
  (bind _returnvalue (Effects|SpawnEmitteratLocation "/Game/Blueprints/Bombs/LaserParticle.LaserParticle" StartLocation))
  (bind _output_get (Variables|Default|SetLaserBean _returnvalue))
  (Class|ParticleSystemComponent|SetBeamEndPoint _output_get 0 EndLocation))

(fn ScaleTriggerBox
  (params (EndLocation :type Vector))
  (bind _laserstartpoint (Variables|Default|GetLaserStartPoint))
  (bind _boxexp (Variables|Default|GetBoxExp))
  (bind _returnvalue (Transformation|GetWorldLocation _laserstartpoint))
  (bind _returnvalue_2 (- EndLocation _returnvalue))
  (bind _returnvalue_3 (Math|Vector|VectorLength _returnvalue_2))
  (bind _returnvalue_4 (/ _returnvalue_3 2.0))
  (Transformation|SetRelativeScale3D (Variables|Default|GetBoxExp) (Math|Vector|MakeVector _returnvalue_4 1.0 1.0))
  (Transformation|SetRelativeLocation _boxexp (+ (Variables|/Script/Engine.SceneComponent|GetRelativeLocation _boxexp) (Math|Vector|MakeVector _returnvalue_4 0.0 0.0)) false false))