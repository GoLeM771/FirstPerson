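; Gatling gun weapon Blueprint that spins up before firing and locks out when it overheats.
; A timeline scaled by charge time starts a looping fire timer at full charge; stopping clears the timer and reverses the timeline.
; Each shot adds heat scaled by fire rate, and Tick drains it per frame, holding an overheat lockout until heat reaches zero.
; BeginPlay refreshes the overheat widget in the StatusBar.
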(event EventBeginPlay
  (bind _foundwidgets (Widget|GetAllWidgetsOfClass "/Game/Blueprints/UI/StatusBar.StatusBar_C" true))
  (Default|UpdateWidget (Variables|/Game/Blueprints/UI/StatusBar.StatusBar_C|GetGutlingGunOverhit (Utilities|Array|Get(acopy) _foundwidgets))))

(event EventStartShooting
  (|CallParentFunction)
  (if (not (Variables|Default|GetIsOverhited?))
    (Components|Timeline|SetPlayRate (Variables|Default|GetChargeUpGun) (/ 1.0 (Variables|Default|GetChargeTime)))
    (bind _alpha (Timeline|ChargeUpGun Play)
      (:Update
        (bind _output_get (Variables|Default|SetCurrentCharge (Math|Float|Lerp 0.0 1.0 _alpha)))
        (if (>= _output_get 1.0)
          (bind _returnvalue (Utilities|Time|SetTimerbyFunctionName self "FireBullet" (Variables|Default|GetFireRate) true))
          (Variables|Default|SetGunTimer _returnvalue))))))

(event EventStopShooting
  (|CallParentFunction)
  (Utilities|Time|ClearandInvalidateTimerbyHandle (Variables|Default|GetGunTimer))
  (bind _alpha (Timeline|ChargeUpGun Reverse)
    (:Update
      (bind _output_get (Variables|Default|SetCurrentCharge (Math|Float|Lerp 0.0 1.0 _alpha)))
      (if (>= _output_get 1.0)
        (bind _returnvalue (Utilities|Time|SetTimerbyFunctionName self "FireBullet" (Variables|Default|GetFireRate) true))
        (Variables|Default|SetGunTimer _returnvalue)))))

(event EventFireBullet
  (if (not (Variables|Default|GetIsOverhited?))
    (|CallParentFunction)
    (bind _output_get (Variables|Default|SetCurrentHeat (+ (Variables|Default|GetCurrentHeat) (* (Variables|Default|GetFireRate) 1.5))))
    (Variables|Default|SetIsOverhited? (>= (Math|Float|Clamp(Float) _output_get) 1.0))))

(event EventTick
  (params (DeltaSeconds :type Float%20%28single-precision%29))
  (if (> (Variables|Default|GetCurrentHeat) 0.0)
    (if (Variables|Default|GetIsOverhited?)
      (bind _output_get (Variables|Default|SetCurrentHeat (Math|Float|Clamp(Float) (- (Variables|Default|GetCurrentHeat) 0.01))))
      (if (<= _output_get 0.0)
        (Variables|Default|SetIsOverhited? false))
      (else
        (Variables|Default|SetCurrentHeat (Math|Float|Clamp(Float) (- (Variables|Default|GetCurrentHeat) (* (Variables|Default|GetFireRate) 0.05))))))))

(fn ConstructionScript
  (|CallParentFunction))