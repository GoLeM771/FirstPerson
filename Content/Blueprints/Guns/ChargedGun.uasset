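; Gun Blueprint for a charged shot whose bullet speed depends on how long the trigger is held.
; A ChargeWeapon timeline plays at a rate set by ChargedTime to raise CurrentCharge, firing automatically at full charge.
; Releasing fires only above a minimum charge, then the timeline reverses at normal rate to drain.
; FireBullet temporarily scales BulletSpeed by the charge before calling the parent and restoring a hardcoded default.
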(event EventStartShooting
  (|CallParentFunction)
  (if (and (not (Variables|Default|GetIsCharging?)) (<= (Variables|Default|GetCurrentCharge) 0.0))
    (Variables|Default|SetIsCharging? true)
    (Components|Timeline|SetPlayRate (Variables|Default|GetChargeWeapon) (/ 1.0 (Variables|Default|GetChargedTime)))
    (bind _weaponcharge (Timeline|ChargeWeapon Play)
      (:Update
        (bind _output_get (Variables|Default|SetCurrentCharge (Math|Float|Clamp(Float) _weaponcharge)))
        (if (>= _output_get 1.0)
          (CallFunction|StopShooting))))))

(event EventStopShooting
  (|CallParentFunction)
  (if (and (Variables|Default|GetIsCharging?) (>= (Variables|Default|GetCurrentCharge) 0.2))
    (CallFunction|FireBullet))
  (Variables|Default|SetIsCharging? false)
  (Components|Timeline|SetPlayRate (Variables|Default|GetChargeWeapon) 1.0)
  (bind _weaponcharge (Timeline|ChargeWeapon Reverse)
    (:Update
      (bind _output_get (Variables|Default|SetCurrentCharge (Math|Float|Clamp(Float) _weaponcharge)))
      (if (>= _output_get 1.0)
        (CallFunction|StopShooting)))))

(event EventFireBullet
  (Variables|Default|SetBulletSpeed (* (Variables|Default|GetBulletSpeed) (Variables|Default|GetCurrentCharge)))
  (|CallParentFunction)
  (Variables|Default|SetBulletSpeed 3e+03))

(fn ConstructionScript
  (|CallParentFunction))