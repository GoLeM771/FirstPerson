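; Flamethrower weapon Blueprint that damages AI characters inside a capsule hit volume while draining ammo.
; Shooting slows the player and, after a short charge delay, starts the particles and a looping Flame timer at the fire rate.
; Each Flame tick plays audio and, while firing, toggles capsule collision on and off to retrigger overlap damage.
; Releasing or running out of ammo stops effects and timer and restores walk speed.
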(event OnComponentBeginOverlap(Capsule)
  (params (OverlappedComponent :type Primitive%20Component%20Object%20Reference) (OtherActor :type Actor%20Object%20Reference) (OtherComp :type Primitive%20Component%20Object%20Reference) (OtherBodyIndex :type Integer) (bFromSweep :type Boolean) (SweepResult :type Hit%20Result%20Structure%20%28by%20ref%29))
  (if (> (Variables|Default|GetAmmoCurrent) 0)
    (bind _asbase_ai_character (Utilities|Casting|CastToBaseAiCharacter OtherActor))
    (Default|HealthMinus _asbase_ai_character 1e+01 false)))

(event Custom|PlayMainSound
  (Audio|Components|Audio|Play (Variables|Default|GetAudioCurveSource) 0.0))

(event EventBeginPlay
  (|CallParentFunction)
  (Collision|SetCollisionEnabled (Variables|Default|GetCapsule) "NoCollision"))

(event Collision|EventActorBeginOverlap
  (params (OtherActor :type Actor%20Object%20Reference))
  (|CallParentFunction OtherActor) ; This node is disabled and will not be called.\nDrag off pins to build functionality.
)

(event EventTick
  (params (DeltaSeconds :type Float%20%28single-precision%29))
  (|CallParentFunction DeltaSeconds) ; This node is disabled and will not be called.\nDrag off pins to build functionality.
)

(event EventStartShooting
  (|CallParentFunction)
  (Variables|/Script/Engine.CharacterMovementComponent|SetMaxWalkSpeed (Variables|/Script/Engine.Character|GetCharacterMovement (Variables|Default|GetPlayerRef)) 2e+02)
  (Variables|Default|SetIsCharging? true)
  (Audio|PlaySound2D (Variables|Default|GetStartSound) 1.0 1.0 0.0 0 0)
  (Utilities|FlowControl|Delay 0.72)
  (if (Variables|Default|GetIsCharging?)
    (Collision|SetCollisionEnabled (Variables|Default|GetCapsule) "QueryAndPhysics")
    (CallFunction|Flame)
    (bind _returnvalue (Utilities|Time|SetTimerbyFunctionName self "Flame" (Variables|Default|GetFireRate) true))
    (Variables|Default|SetGunTimer _returnvalue)
    (Components|Activation|Activate (Variables|Default|GetParticleSystem) true)
    (else
      (Utilities|IsValid (Variables|Default|GetParticleSystem)
        (:Is%20Valid
          (Components|DestroyComponent (Variables|Default|GetParticleSystem)))))))

(event EventStopShooting
  (Audio|Components|Audio|Stop (Variables|Default|GetAudioCurveSource))
  (Audio|PlaySound2D "/Game/Sound/flamethowerend.flamethowerend" 1.0 1.0 0.0 0 0)
  (Components|Activation|Deactivate (Variables|Default|GetParticleSystem))
  (Variables|Default|SetIsCharging? false)
  (|CallParentFunction)
  (Utilities|Time|ClearandInvalidateTimerbyHandle (Variables|Default|GetGunTimer))
  (Variables|/Script/Engine.CharacterMovementComponent|SetMaxWalkSpeed (Variables|/Script/Engine.Character|GetCharacterMovement (Variables|Default|GetPlayerRef)) 6e+02))

(fn ConstructionScript
  (|CallParentFunction))

(fn Flame
  (if (> (Variables|Default|GetAmmoCurrent) 0)
    (CallFunction|PlayMainSound)
    (if (Variables|Default|GetIsFiering?)
      (Collision|SetCollisionEnabled (Variables|Default|GetCapsule) "QueryAndPhysics")
      (Collision|SetCollisionEnabled (Variables|Default|GetCapsule) "NoCollision")
      (Variables|Default|SetAmmoCurrent (- (Variables|Default|GetAmmoCurrent) 1)))
    (else
      (CallFunction|StopShooting))))