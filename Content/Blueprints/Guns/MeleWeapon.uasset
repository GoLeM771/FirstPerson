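; Melee weapon that reuses gun shoot and zoom events for stamina-costed light attacks, charged heavy attacks and blocking.
; Releasing before or after the charge delay picks the attack, whose flag holds for its animation length.
; AttackTrace line-traces from five blade points, damaging each zombie not already listed by attack type and chipping SpawnBeton actors.
; Blocking alters stamina drain, with a temporary out-of-breath state on release if PlayerWasHet is set.
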(event Custom|HitEvent
  (params (Damage :type Float%20%28single-precision%29) (Hit :type Hit%20Result%20Structure))
  (Variables|Default|SetDamage Damage)
  (bind _outactors (Actor|GetAllActorsOfClass "/Game/Bot/BaseEnemyCharacter/BaseZombieCharacter.BaseZombieCharacter_C"))
  (for _array_element _outactors
    (Variables|Default|SetDamagedEnamy _array_element)
    (if (and (== _array_element (.HitActor (Collision|BreakHitResult Hit))) (not (Utilities|Array|ContainsItem (Variables|Default|GetAlredyDamageEnemy) (Variables|Default|GetDamagedEnamy))))
      (Utilities|Array|Add (Variables|Default|GetAlredyDamageEnemy) (Variables|Default|GetDamagedEnamy))
      (if (Variables|Default|GetIsLAttack?)
        (Default|HealthDecrease (Variables|/Game/Bot/BaseEnemyCharacter/BaseZombieCharacter.BaseZombieCharacter_C|GetWoundSystemExtras (Variables|Default|GetDamagedEnamy)) 2e+01 "None")
        (else
          (Default|HealthDecrease (Variables|/Game/Bot/BaseEnemyCharacter/BaseZombieCharacter.BaseZombieCharacter_C|GetWoundSystemExtras (Variables|Default|GetDamagedEnamy)) 1.5e+02 "None"))))))

(event Custom|LAttack
  (bind _stamina (Class|PlayerInterface|CurrentandMaxStaminaGetter(Message) (Game|GetPlayerCharacter 0)))
  (if (>= _stamina 3e+01)
    (Class|PlayerInterface|CurrentStaminaSetter(Message) (Game|GetPlayerCharacter 0) (- _stamina 3e+01))
    (Variables|Default|SetLAttack? true)
    (bind _returnvalue (Animation|GetPlayLength (Variables|Default|GetLightAttack)))
    (Utilities|FlowControl|Delay _returnvalue)
    (Variables|Default|SetLAttack? false)))

(event Custom|HAttack
  (bind _returnvalue (Game|GetPlayerCharacter 0))
  (bind _issprinting_ (Class|PlayerInterface|IsSprintingGetter(Message) _returnvalue))
  (bind _stamina (Class|PlayerInterface|CurrentandMaxStaminaGetter(Message) _returnvalue))
  (if (and (not _issprinting_) (>= _stamina 6e+01))
    (Class|PlayerInterface|CurrentStaminaSetter(Message) (Game|GetPlayerCharacter 0) (- _stamina 6e+01))
    (Variables|Default|SetHAttack? true)
    (bind _returnvalue_2 (Animation|GetPlayLength (Variables|Default|GetHeavyAttack)))
    (Utilities|FlowControl|Delay _returnvalue_2)
    (Variables|Default|SetHAttack? false)))

(event Custom|AttackTrace
  (for _array_element (Utilities|Array|MakeArray (Variables|Default|GetCollision1) (Variables|Default|GetCollision2) (Variables|Default|GetCollision3) (Variables|Default|GetCollision4) (Variables|Default|GetCollision5))
    (bind (_outhit _returnvalue) (Collision|LineTraceForObjects (Transformation|GetWorldLocation _array_element) (Math|Vector|MakeVector (.x (- (Transformation|GetWorldLocation _array_element) (* (Math|Vector|GetForwardVector (Transformation|GetWorldRotation _array_element)) 4e+01))) (.y (- (Transformation|GetWorldLocation _array_element) (* (Math|Vector|GetForwardVector (Transformation|GetWorldRotation _array_element)) 4e+01))) (.z (- (Transformation|GetWorldLocation _array_element) (* (Math|Vector|GetForwardVector (Transformation|GetWorldRotation _array_element)) 4e+01)))) (Utilities|Array|MakeArray "ObjectTypeQuery3" "ObjectTypeQuery11") true (Utilities|Array|MakeArray (Game|GetPlayerCharacter 0)) "ForDuration" true "(R=1.000000,G=0.000000,B=0.000000,A=1.000000)" "(R=0.000000,G=1.000000,B=0.000000,A=1.000000)" 2e+01))
    ;[1 1 1] Ошибка
    (if _returnvalue
      (switch Utilities|FlowControl|Switch|SwitchonECollisionChannel (Collision|GetCollisionObjectType (.HitComponent (Collision|BreakHitResult _outhit)))
        (:ECC_Pawn
          (CallFunction|HitEvent 5e+01 _outhit))
        (:ECC_GameTraceChannel1
          (bind _asspawn_beton (Utilities|Casting|CastToSpawnBeton (.HitActor (Collision|BreakHitResult _outhit))))
          (Default|BetonHealthMinusEvent _asspawn_beton))))))

(event EventBeginPlay
  (|CallParentFunction) ; This node is disabled and will not be called.\nDrag off pins to build functionality.
)

(event EventStartShooting
  (if (not (Variables|Default|GetInBlock?))
    (Variables|Default|SetIsCharged? true)
    (Development|PrintString "ChargeStart")
    (Utilities|FlowControl|RetriggerableDelay (Variables|Default|GetChargeAttackTime))
    (if (Variables|Default|GetIsCharged?)
      (Variables|Default|SetChargeComplete? true)
      (Development|PrintString "Charge complete"))))

(event EventStopShooting
  (if (not (Variables|Default|GetInBlock?))
    (if (Variables|Default|GetChargeComplete?)
      (Development|PrintString "Heavy Attack")
      (Variables|Default|SetChargeComplete? false)
      (Variables|Default|SetIsCharged? false)
      (bind _stamina (Class|PlayerInterface|CurrentandMaxStaminaGetter(Message) (Game|GetPlayerCharacter 0)))
      (if (and (>= _stamina 6e+01) (not (Variables|Default|GetHAttack?)))
        (CallFunction|HAttack)
        (Variables|Default|SetIsLAttack? false))
      (else
        (Variables|Default|SetChargeComplete? false)
        (if (Variables|Default|GetIsCharged?)
          (Variables|Default|SetIsCharged? false)
          (bind _stamina_2 (Class|PlayerInterface|CurrentandMaxStaminaGetter(Message) (Game|GetPlayerCharacter 0)))
          (if (and (>= _stamina_2 3e+01) (not (Variables|Default|GetLAttack?)))
            (CallFunction|LAttack)
            (Variables|Default|SetIsLAttack? true)))))))

(event EventStartZoom
  (Variables|Default|SetInBlock? true)
  (Class|PlayerInterface|StaminaDecreaceAmountSetter(Message) (Game|GetPlayerCharacter 0) 0.1))

(event EventStopZoom
  (bind _returnvalue (Game|GetPlayerCharacter 0))
  (bind _returnvalue_2 (Game|GetPlayerCharacter 0))
  (Variables|Default|SetInBlock? false)
  (if (Variables|Default|GetPlayerWasHet?)
    (Class|PlayerInterface|OutOfBreathSetter(Message) _returnvalue_2 true)
    (Class|PlayerInterface|StaminaDecreaceAmountSetter(Message) _returnvalue_2 1e+01)
    (Utilities|FlowControl|Delay 3.0)
    (Class|PlayerInterface|StaminaDecreaceAmountSetter(Message) _returnvalue 2e+01)
    (Class|PlayerInterface|OutOfBreathSetter(Message) _returnvalue false)
    (Variables|Default|SetPlayerWasHet? false)))

(fn ConstructionScript
  (|CallParentFunction))