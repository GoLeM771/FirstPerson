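; Bullet projectile actor for guns that damages AI characters it overlaps.
; On spawn it rotates its Velocity by the actor's rotation to drive ProjectileMovement, while the LifeSpan timeline animates its scale.
; When the timeline finishes, it toggles the mesh's active state and destroys itself after a short delay.
; Any hit or overlap destroys it immediately, with AICharacter overlaps first applying fixed damage through HealthMinus.
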(event EventBeginPlay
  (Variables|/Script/Engine.MovementComponent|SetVelocity (Variables|Default|GetProjectileMovement) (Math|Vector|RotateVector (Variables|Default|GetVelocity) (Transformation|GetActorRotation)))
  (bind _scale (Timeline|LifeSpan Play)
    (:Update
      (Transformation|SetActorRelativeScale3D (* (Math|Vector|MakeVector 1.0 1.0 1.0) _scale)))
    (:Finished
      (Components|Activation|ToggleActive (Variables|Default|GetStaticMesh))
      (Utilities|FlowControl|Delay 0.1)
      (Actor|DestroyActor))))

(event Collision|EventActorBeginOverlap
  (params (OtherActor :type Actor%20Object%20Reference))
  (bind _asaicharacter (Utilities|Casting|CastToAICharacter OtherActor)
    (:then
      (Default|HealthMinus _asaicharacter 5e+01 false))
    (:CastFailed
      _))
  (Actor|DestroyActor))

(event Collision|EventHit
  (params (MyComp :type Primitive%20Component%20Object%20Reference) (Other :type Actor%20Object%20Reference) (OtherComp :type Primitive%20Component%20Object%20Reference) (bSelfMoved :type Boolean) (HitLocation :type Vector :default "0, 0, 0") (HitNormal :type Vector :default "0, 0, 0") (NormalImpulse :type Vector :default "0, 0, 0") (Hit :type Hit%20Result%20Structure%20%28by%20ref%29))
  (Actor|DestroyActor))

(fn ConstructionScript)