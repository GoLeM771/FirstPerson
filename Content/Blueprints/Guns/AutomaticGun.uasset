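; Automatic gun Blueprint, a child of a base gun class, that fires continuously while shooting is active.
; StartShooting fires one bullet at once, then a looping timer repeats FireBullet every FireRate seconds until StopShooting clears it.
; Zooming blends the player's view to the gun and back to its parent actor.
; While InZoom is set, Tick keeps the gun's Camera aligned to the player's control rotation.
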(event EventBeginPlay
  (|CallParentFunction) ; This node is disabled and will not be called.\nDrag off pins to build functionality.
)

(event Collision|EventActorBeginOverlap
  (params (OtherActor :type Actor%20Object%20Reference))
  (|CallParentFunction OtherActor) ; This node is disabled and will not be called.\nDrag off pins to build functionality.
)

(event EventStartShooting
  (|CallParentFunction)
  (CallFunction|FireBullet)
  (bind _returnvalue (Utilities|Time|SetTimerbyFunctionName self "FireBullet" (Variables|Default|GetFireRate) true))
  (Variables|Default|SetGunTimer _returnvalue))

(event EventStopShooting
  (|CallParentFunction)
  (Utilities|Time|ClearandInvalidateTimerbyHandle (Variables|Default|GetGunTimer)))

(event EventStartZoom
  (|CallParentFunction)
  (Game|Player|SetViewTargetwithBlend (Game|GetPlayerController 0) self 0.2 "VTBlend_Linear" 0.0 false))

(event EventStopZoom
  (|CallParentFunction)
  (Game|Player|SetViewTargetwithBlend (Game|GetPlayerController 0) (Actor|GetParentActor) 0.2 "VTBlend_Linear" 0.0 false))

(event EventTick
  (params (DeltaSeconds :type Float%20%28single-precision%29))
  (|CallParentFunction DeltaSeconds)
  (CallFunction|CheckZoom))

(fn ConstructionScript
  (|CallParentFunction))

(fn CheckZoom
  (if (Variables|Default|GetInZoom?)
    (Transformation|SetWorldRotation (Variables|Default|GetCamera) (Pawn|GetControlRotation (Game|GetPlayerController 0) :!class /Script/Engine.Controller) false false)
    (return)))