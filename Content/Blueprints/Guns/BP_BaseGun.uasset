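; Base gun for the player's TPCharacter, handling hitscan and projectile fire, ammo, reloading and stopping when empty.
; FireBullet traces from the gun's sight when zoomed or the player camera otherwise, with random spread only while moving, then pushes physics objects.
; It also spawns muzzle bullets with randomly hidden tracers, muzzle flash, recoil and crosshair animation.
; ChargedGunFire instead launches a projectile at BulletSpeed from the Arrow.
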(event Custom|StartShooting
  (Variables|Default|SetIsFiering? true))

(event Custom|StopShooting
  (Variables|Default|SetIsFiering? false)
  (CallFunction|StopMuzzleFlash))

(event Custom|StartZoom
  (Variables|Default|SetInZoom? true))

(event Custom|StopZoom
  (Variables|Default|SetInZoom? false))

(event EventBeginPlay
  (bind _astpcharacter (Utilities|Casting|CastToTPCharacter (Game|GetPlayerCharacter 0)))
  (Variables|Default|SetPlayerRef _astpcharacter))

(event EventTick
  (params (DeltaSeconds :type Float%20%28single-precision%29))
  (bind _playerref (Variables|Default|GetPlayerRef))
  (Development|PrintString (Utilities|String|Append "BaseGun weapon int: " (Utilities|String|ToString(Integer) (Variables|Default|GetWeaponInt))) true true "(R=0.000000,G=0.660000,B=1.000000,A=1.000000)" 0.0)
  (if (not (> (Variables|Default|GetAmmoCurrent) 0))
    (Default|StopShootGun _playerref)
    (Variables|/Game/Blueprints/TPCharacter.TPCharacter_C|SetWeaponFire? _playerref false)))

(fn ConstructionScript)

(fn FireBullet
  (bind _returnvalue (Game|Player|GetPlayerPawn 0))
  (if (> (Variables|Default|GetAmmoCurrent) 0)
    ;[1 1 1] На виджете перекрестья прицела проигрываем анимацию
    (Default|ShootEvent (Variables|/Game/Blueprints/UI/StatusBar.StatusBar_C|GetCrosshair (Variables|/Game/Blueprints/TPCharacter.TPCharacter_C|GetHUDRef (Variables|Default|GetPlayerRef))))
    (CallFunction|MuzzleFlash)
    ;[1 1 1] Выясняем - от какой камеры начинать лучь от камеры автомата или игрока
    (if (Variables|Default|GetInZoom?)
      (LocalVariables|SetStartPoint (Transformation|GetWorldLocation (Variables|Default|GetArrow)))
      (LocalVariables|SetGunDirection (Math|Vector|GetForwardVector (Transformation|GetWorldRotation (Variables|Default|GetCamera))))
      (LocalVariables|SetEndPoint (+ (Transformation|GetWorldLocation (Variables|Default|GetCamera)) (* (LocalVariables|GetGunDirection) 2e+03) (CallFunction|SpreadFunc (Variables|Default|GetSpreadMinIronSights) (Variables|Default|GetSpreadMaxIronSights))))
      (else
        (LocalVariables|SetStartPoint (Transformation|GetWorldLocation (Variables|/Game/Blueprints/TPCharacter.TPCharacter_C|GetCameraTP (Variables|Default|GetPlayerRef))))
        (LocalVariables|SetGunDirection (Math|Vector|GetForwardVector (Transformation|GetWorldRotation (Variables|/Game/Blueprints/TPCharacter.TPCharacter_C|GetCameraTP (Variables|Default|GetPlayerRef)))))
        (LocalVariables|SetEndPoint (+ (LocalVariables|GetStartPoint) (* (LocalVariables|GetGunDirection) 2e+03) (CallFunction|SpreadFunc (Variables|Default|GetSpreadMinOpenSights) (Variables|Default|GetSpreadMaxOpenSights))))))
    (bind (_outhit _returnvalue_2) (Collision|LineTraceByChannel (LocalVariables|GetStartPoint) (LocalVariables|GetEndPoint) "TraceTypeQuery1" false (Utilities|Array|MakeArray (Variables|Default|GetPlayerRef)) "None"))
    (CallFunction|BulletSpawn _outhit _returnvalue_2 (LocalVariables|GetEndPoint))
    (CallFunction|AddImpulce? _outhit (LocalVariables|GetGunDirection))
    (Variables|Default|SetAmmoCurrent (- (Variables|Default|GetAmmoCurrent) 1))
    ;[1 1 1] Отдача
    (Pawn|Input|AddControllerPitchInput _returnvalue (Math|Random|RandomFloatinRange -0.1 0.1))
    (Pawn|Input|AddControllerYawInput _returnvalue (Math|Random|RandomFloatinRange -0.1 0.1))))

(fn ReloadGun
  (bind _output_get (LocalVariables|SetBulletDifference (- (Variables|Default|GetClipSize) (Variables|Default|GetAmmoCurrent))))
  (if (>= (Variables|Default|GetCharacterAmmoMax) _output_get)
    (Variables|Default|SetAmmoCurrent (Variables|Default|GetClipSize))
    (Variables|Default|SetCharacterAmmoMax (- (Variables|Default|GetCharacterAmmoMax) (LocalVariables|GetBulletDifference)))
    (else
      (Variables|Default|SetAmmoCurrent (+ (Variables|Default|GetAmmoCurrent) (Variables|Default|GetCharacterAmmoMax)))
      (Variables|Default|SetCharacterAmmoMax 0))))

(fn AddImpulce?
  (params (Hit :type Hit%20Result%20Structure%20%28by%20ref%29) (GunDir :type Vector))
  (bind (_bblockinghit _binitialoverlap _time _distance _location _impactpoint _normal _impactnormal _physmat _hitactor _hitcomponent) (Collision|BreakHitResult Hit))
  (LocalVariables|SetGunDirection GunDir)
  (if _bblockinghit
    (if (Physics|IsSimulatingPhysics _hitcomponent "None")
      (Physics|AddImpulseatLocation _hitcomponent (* (LocalVariables|GetGunDirection) 8e+05) _impactpoint "None")))
  (return))

(fn BulletSpawn
  (params (HitResult :type Hit%20Result%20Structure) (HitSomething :type Boolean) (EndForwardVector :type Vector))
  (bind (_bblockinghit _binitialoverlap _time _distance _location _impactpoint _normal) (Collision|BreakHitResult HitResult))
  (bind _guns (Variables|Default|GetGuns))
  (bind _returnvalue (Transformation|GetSocketLocation _guns "Muzzle"))
  (if HitSomething
    (LocalVariables|SetEndPoint (+ _location (* _normal -1.0)))
    (else
      (LocalVariables|SetEndPoint EndForwardVector)))
  (bind _outhit (Collision|LineTraceByChannel _returnvalue EndForwardVector "TraceTypeQuery1" false (Utilities|Array|MakeArray (Variables|Default|GetPlayerRef)) "None"))
  (bind _returnvalue_2 (Game|SpawnActorfromClass "/Game/Blueprints/Guns/BulletProjectile.BulletProjectile_C" (Math|Transform|MakeTransform _returnvalue (Math|Rotator|FindLookatRotation _returnvalue (.TraceEnd (Collision|BreakHitResult _outhit)))) "AlwaysSpawn" 0 0))
  ;[1 1 1] Отключение видимости Nного трейса пули
  (if (> (Math|Random|RandomIntegerinRange 1 10) 7)
    (Rendering|SetVisibility (Variables|/Game/Blueprints/Guns/BulletProjectile.BulletProjectile_C|GetTraceModel _returnvalue_2) false false)))

(fn SpreadFunc
  (params (MinSpread :type Float%20%28single-precision%29) (MaxSpread :type Float%20%28single-precision%29))
  (bind _playerref (Variables|Default|GetPlayerRef))
  (bind _returnvalue (Transformation|GetVelocity _playerref))
  (bind _returnvalue_2 (Math|Vector|ClampVectorSize _returnvalue 0.0 1.0))
  (bind _returnvalue_3 (Math|Vector|VectorLength _returnvalue_2))
  (return (Math|Vector|MakeVector (* _returnvalue_3 (Math|Random|RandomFloatinRange MinSpread MaxSpread)) (* _returnvalue_3 (Math|Random|RandomFloatinRange MinSpread MaxSpread)) (* _returnvalue_3 (Math|Random|RandomFloatinRange MinSpread MaxSpread)))))

(fn MuzzleFlash
  (bind _returnvalue (Math|Random|RandomFloatinRange 0.1 0.3))
  (bind _muzzlemesh (Variables|Default|GetMuzzleMesh))
  (if (> (Variables|Default|GetAmmoCurrent) 0)
    (Rendering|Components|Light|SetIntensity (Variables|Default|GetPointLight_0) 2e+04)
    (Rendering|SetVisibility (Variables|Default|GetMuzzleMesh) true true)
    (Transformation|SetRelativeRotation _muzzlemesh (Math|Rotator|MakeRotator -9e+01 (Math|Random|RandomFloatinRange -9e+01 9e+01) 0.0) false false)
    (Transformation|SetWorldScale3D _muzzlemesh (Math|Vector|MakeVector _returnvalue _returnvalue _returnvalue))
    (else
      (CallFunction|StopMuzzleFlash))))

(fn StopMuzzleFlash
  (Rendering|Components|Light|SetIntensity (Variables|Default|GetPointLight_0) 0.0)
  (Rendering|SetVisibility (Variables|Default|GetMuzzleMesh) false true)
  (Variables|Default|SetIsFiering? false))

(fn ChargedGunFire
  (bind _returnvalue (Game|Player|GetPlayerPawn 0))
  (bind _bulletspeed (Variables|Default|GetBulletSpeed))
  (Utilities|Casting|CastToTPCharacter (Actor|GetParentActor))
  (if (> (Variables|Default|GetAmmoCurrent) 0)
    (if (Variables|Default|GetInZoom?)
      (LocalVariables|SetDirection (Transformation|GetWorldRotation (Variables|Default|GetArrow)))
      (else
        (LocalVariables|SetDirection (Transformation|GetWorldRotation (Variables|/Game/Blueprints/TPCharacter.TPCharacter_C|GetCameraTP (Variables|Default|GetPlayerRef))))))
    (bind _returnvalue_2 (Game|SpawnActorfromClass (Variables|Default|GetProjectile) (Math|Transform|MakeTransform (Transformation|GetWorldLocation (Variables|Default|GetArrow)) (LocalVariables|GetDirection) "1,1,1") "Undefined" 0 0))
    (Variables|/Script/Engine.ProjectileMovementComponent|SetInitialSpeed (Variables|/Game/Blueprints/FirstPersonProjectile.FirstPersonProjectile_C|GetProjectile _returnvalue_2) _bulletspeed)
    (Variables|/Script/Engine.ProjectileMovementComponent|SetMaxSpeed (Variables|/Game/Blueprints/FirstPersonProjectile.FirstPersonProjectile_C|GetProjectile _returnvalue_2) _bulletspeed)
    (bind _result (Math|Integer|DecrementInt (Variables|Default|GetAmmoCurrent))
      (:%20%20
        (Variables|Default|SetAmmoCurrent _result)
        ;[1 1 1] Отдача
        (Pawn|Input|AddControllerPitchInput _returnvalue (Math|Random|RandomFloatinRange -0.1 0.1))
        (Pawn|Input|AddControllerYawInput _returnvalue (Math|Random|RandomFloatinRange -0.1 0.1))
        ;[1 1 1] На виджете перекрестья прицела проигрываем анимацию
        (Default|ShootEvent (Variables|/Game/Blueprints/UI/StatusBar.StatusBar_C|GetCrosshair (Variables|/Game/Blueprints/TPCharacter.TPCharacter_C|GetHUDRef (Variables|Default|GetPlayerRef))))))))