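; Bullet projectile actor that damages AI characters on impact.
; On spawn it rotates its Velocity variable by the actor's rotation to drive ProjectileMovement, while a timeline rescales the whole actor as a tracer effect.
; When the timeline finishes, it toggles the mesh's active state and destroys itself after a short delay.
; Sphere or mesh hits destroy it immediately, with only sphere hits on an AICharacter applying fixed damage through HealthMinus.
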(event OnComponentHit(StaticMesh)
  (params (HitComponent :type Primitive%20Component%20Object%20Reference) (OtherActor :type Actor%20Object%20Reference) (OtherComp :type Primitive%20Component%20Object%20Reference) (NormalImpulse :type Vector :default "0, 0, 0") (Hit :type Hit%20Result%20Structure%20%28by%20ref%29))
  ;[1 1 1] При пересечении сферы с чемнить проверит - является ли объект ботом и в любом случае самоуничтожится
  ;;[1 1 1] При попадании во что то просто уничтожаем меш трейса
  (Actor|DestroyActor))

(event OnComponentHit(Sphere)
  (params (HitComponent :type Primitive%20Component%20Object%20Reference) (OtherActor :type Actor%20Object%20Reference) (OtherComp :type Primitive%20Component%20Object%20Reference) (NormalImpulse :type Vector :default "0, 0, 0") (Hit :type Hit%20Result%20Structure%20%28by%20ref%29))
  ;[1 1 1] При пересечении сферы с чемнить проверит - является ли объект ботом и в любом случае самоуничтожится
  (bind _asaicharacter (Utilities|Casting|CastToAICharacter OtherActor)
    (:then
      (Default|HealthMinus _asaicharacter 5e+01 false))
    (:CastFailed
      _))
  (Actor|DestroyActor))

(event EventBeginPlay
  ;[1 1 1] При спавне пули задаём направление и начальную скорость
  (Variables|/Script/Engine.MovementComponent|SetVelocity (Variables|Default|GetProjectileMovement) (Math|Vector|RotateVector (Variables|Default|GetVelocity) (Transformation|GetActorRotation)))
  ;[1 1 1] Со времинем уменьшаем трейс пули
  (bind _scale (Timeline|Timeline_0 Play)
    (:Update
      (Transformation|SetActorRelativeScale3D (* (Math|Vector|MakeVector 1.0 1.0 1.0) _scale)))
    (:Finished
      ;[1 1 1] После проигрывания таймлайна трес пули самоуничтожится
      (Components|Activation|ToggleActive (Variables|Default|GetStaticMesh))
      (Utilities|FlowControl|Delay 0.1)
      (Actor|DestroyActor))))

(fn ConstructionScript)