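; TestLootBox is a test loot container that generates random contents and opens its inventory for a player.
; On BeginPlay it rolls a count up to the slot limit, picks items via DropRandomLoot, sizes stacks from class defaults and copies them into InventoryComponent slots.
; A short delay later it sets its widget label.
; Interaction toggles both inventories and hands the box's inventory reference to the player through PlayerInterface.
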(event Custom|FillLootArrey
  (Variables|Default|SetDropQuantity 0)
  (bind _lootclass (CallFunction|DropRandomLoot (Variables|Default|GetStartLoot)))
  (if (.IsStacable? (Utilities|Struct|BreakST_PickupItem (Utilities|GetClassDefaults _lootclass)))
    (Variables|Default|SetDropQuantity (Math|Random|RandomIntegerinRange 1 (.MaxStackSize (Utilities|Struct|BreakST_PickupItem (Utilities|GetClassDefaults _lootclass)))))
    (else
      (Variables|Default|SetDropQuantity 1)))
  (Utilities|Array|Add (Variables|Default|GetLootToDrop) (Utilities|Struct|MakeST_InventorySlot (Utilities|Struct|MakeST_PickupItem _lootclass) (Variables|Default|GetDropQuantity))))

(event EventBeginPlay
  (Variables|Default|SetRollLootIterations (Math|Random|RandomIntegerinRange 1 (Variables|/Game/Blueprints/InventorySystem/InventoryComponent.InventoryComponent_C|GetNumberOfSlots (Variables|Default|GetInventoryComponent))))
  (while (> (Variables|Default|GetRollLootIterations) 0)
    (CallFunction|FillLootArrey)
    (Variables|Default|SetRollLootIterations (- (Variables|Default|GetRollLootIterations) 1)))
  (for (_array_element _array_index) (Variables|Default|GetLootToDrop)
    (Utilities|Array|SetArrayElem (Variables|/Game/Blueprints/InventorySystem/InventoryComponent.InventoryComponent_C|GetInventory (Variables|Default|GetInventoryComponent)) _array_index _array_element))
  (Utilities|FlowControl|Delay 0.2)
  (Class|ElevatorInterface|SetWidgetText(Message) (UserInterface|GetUserWidgetObject (Variables|Default|GetWidget)) "Loot box blat'"))

(event EventInteraction
  (params (Interacter :type Actor%20Object%20Reference))
  (if (Utilities|DoesObjectImplementInterface Interacter "/Game/Blueprints/Interfaces/PlayerInterface.PlayerInterface_C")
    (Default|ToggleInventory (Variables|Default|GetInventoryComponent))
    (bind _inventoryreference (Class|PlayerInterface|GetInventoryReference(Message) Interacter))
    (Default|ToggleInventory _inventoryreference)
    (Class|PlayerInterface|InventoryOpenSetter(Message) Interacter true)
    (Class|PlayerInterface|OtherInventoryReferenceSetter(Message) Interacter (Variables|Default|GetInventoryComponent))))

(fn ConstructionScript)