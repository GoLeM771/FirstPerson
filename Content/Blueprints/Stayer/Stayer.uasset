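; Stayer is an actor that clamps the player character (TPCharacter) while it overlaps the actor's Box.
; On overlap it registers itself on the player, sets IsClamping, switches movement to Flying and opens a Tick-driven Gate that keeps the player facing the Stayer's forward vector.
; Leaving the Box, or a hit between the Stayer and a TPCharacter through a handler bound on overlap, clears clamping, restores Walking and closes the Gate.
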(event OnComponentBeginOverlap(Box)
  (params (OverlappedComponent :type Primitive%20Component%20Object%20Reference) (OtherActor :type Actor%20Object%20Reference) (OtherComp :type Primitive%20Component%20Object%20Reference) (OtherBodyIndex :type Integer) (bFromSweep :type Boolean) (SweepResult :type Hit%20Result%20Structure%20%28by%20ref%29))
  (bind _playerref (Variables|Default|GetPlayerRef))
  (if (== OtherActor _playerref)
    (Variables|/Game/Blueprints/TPCharacter.TPCharacter_C|SetStayerVar _playerref self)
    (Collision|AssignOnActorHit (delegate Custom|OnActorHit_Event_0))
    (Variables|/Game/Blueprints/TPCharacter.TPCharacter_C|SetIsClamping? _playerref true)
    (Pawn|Components|CharacterMovement|SetMovementMode (Variables|/Script/Engine.Character|GetCharacterMovement _playerref) "MOVE_Flying" 0)
    (Utilities|FlowControl|Gate true) ; enters at Open
  ))

(event OnComponentEndOverlap(Box)
  (params (OverlappedComponent :type Primitive%20Component%20Object%20Reference) (OtherActor :type Actor%20Object%20Reference) (OtherComp :type Primitive%20Component%20Object%20Reference) (OtherBodyIndex :type Integer))
  (bind _playerref (Variables|Default|GetPlayerRef))
  (if (== OtherActor _playerref)
    (Variables|/Game/Blueprints/TPCharacter.TPCharacter_C|SetIsClamping? _playerref false)
    (Pawn|Components|CharacterMovement|SetMovementMode (Variables|/Script/Engine.Character|GetCharacterMovement _playerref) "MOVE_Walking" 0)
    (Utilities|FlowControl|Gate true) ; enters at Close
  ))

(event Custom|OnActorHit_Event_0
  (params (SelfActor :type Actor%20Object%20Reference) (OtherActor :type Actor%20Object%20Reference) (NormalImpulse :type Vector) (Hit :type Hit%20Result%20Structure%20%28by%20ref%29))
  (if (!= OtherActor self)
    (bind _astpcharacter (Utilities|Casting|CastToTPCharacter OtherActor))
    (Variables|/Game/Blueprints/TPCharacter.TPCharacter_C|SetIsClamping? _astpcharacter false)
    (Pawn|Components|CharacterMovement|SetMovementMode (Variables|/Script/Engine.Character|GetCharacterMovement _astpcharacter) "MOVE_Walking" 0)
    (Utilities|FlowControl|Gate true) ; enters at Close
  ))

(event EventBeginPlay
  (bind _outactors (Actor|GetAllActorsOfClass "/Game/Blueprints/TPCharacter.TPCharacter_C"))
  (Variables|Default|SetPlayerRef (Utilities|Array|Get(acopy) _outactors)))

(event Collision|EventActorBeginOverlap
  (params (OtherActor :type Actor%20Object%20Reference)))

(event EventTick
  (params (DeltaSeconds :type Float%20%28single-precision%29))
  (Utilities|FlowControl|Gate true
    (:Exit
      (Transformation|SetActorRotation (Variables|Default|GetPlayerRef) (Math|Conversions|RotationFromXVector (Transformation|GetActorForwardVector))))))

(fn ConstructionScript)