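; InDoor is a one-way door that swings open automatically when the player or a zombie walks into its trigger.
; An overlap on the Re component casts to TPCharacter or BaseZombieCharacter, playing a pitch-randomized sound only for the player.
; Both paths call a once-only OpenDoor1 event, whose timeline lerps the INdoor component's relative rotation open, then destroys the trigger.
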(event OnComponentBeginOverlap(re)
  (params (OverlappedComponent :type Primitive%20Component%20Object%20Reference) (OtherActor :type Actor%20Object%20Reference) (OtherComp :type Primitive%20Component%20Object%20Reference) (OtherBodyIndex :type Integer) (bFromSweep :type Boolean) (SweepResult :type Hit%20Result%20Structure%20%28by%20ref%29))
  (Utilities|Casting|CastToTPCharacter OtherActor
    (:then
      (Utilities|FlowControl|DoOnce false
        (:Completed
          (Audio|PlaySoundatLocation "/Game/Sound/DoorOpen.DoorOpen" (Transformation|GetActorLocation self) "0, 0, 0" 1.0 (Math|Random|RandomFloatinRange 0.95 1.0) 0.0 0 0 0)
          (CallFunction|OpenDoor1))))
    (:CastFailed
      (Utilities|Casting|CastToBaseZombieCharacter OtherActor)
      (CallFunction|OpenDoor1))))

(event Custom|OpenDoor1
  (Utilities|FlowControl|DoOnce false
    (:Completed
      (bind _openroomdor (Timeline|OpenDoor Play)
        (:Update
          (Transformation|SetRelativeRotation (Variables|Default|GetINdoor) (Math|Rotator|Lerp(Rotator) "0, 0, 0" "0,150.000000, 0" _openroomdor) false false))
        (:Finished
          (Components|DestroyComponent (Variables|Default|Getre)))))))

(event EventBeginPlay)

(event EventTick
  (params (DeltaSeconds :type Float%20%28single-precision%29)))

(fn ConstructionScript)