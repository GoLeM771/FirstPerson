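; Door actor that tracks whether its INdoor component is open or closed from its world yaw, with physics simulation turned off at BeginPlay.
; Tick flips DoorOpen when yaw reaches a threshold that alternates between starting yaw plus 80 degrees and starting yaw.
; Each flip sends the player character an unfocus-door interface message and toggles BlockingVolume collision, disabled while open.
; An unused DebugInfo function prints component locations.
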(event EventTick
  (params (DeltaSeconds :type Float%20%28single-precision%29))
  (if (Variables|Default|GetDoorOpen?)
    (if (>= (Variables|Default|GetCheckerVar) (CallFunction|GetDoorYawRotation))
      (Class|PlayerInterface|UnfocusDoorInterface(Message) (Game|GetPlayerCharacter 0))
      (Variables|Default|SetDoorOpen? false)
      (Variables|Default|SetCheckerVar (+ (Variables|Default|GetCheckerVar) 8e+01))
      (Collision|SetCollisionEnabled (Variables|Default|GetBlockingVolume) "QueryAndPhysics"))
    (elif (>= (CallFunction|GetDoorYawRotation) (Variables|Default|GetCheckerVar))
      (Class|PlayerInterface|UnfocusDoorInterface(Message) (Game|GetPlayerCharacter 0))
      (Variables|Default|SetDoorOpen? true)
      (Variables|Default|SetCheckerVar (- (Variables|Default|GetCheckerVar) 8e+01))
      (Collision|SetCollisionEnabled (Variables|Default|GetBlockingVolume) "NoCollision"))))

(event EventBeginPlay
  (Variables|Default|SetOrientalDoorRotatipn (Transformation|GetWorldRotation (Variables|Default|GetINdoor)))
  (Physics|SetSimulatePhysics (Variables|Default|GetINdoor) false)
  (Variables|Default|SetCheckerVar (+ (.Yaw (Math|Rotator|BreakRotator (Variables|Default|GetOrientalDoorRotatipn))) 8e+01)))

(fn ConstructionScript)

(fn DebugInfo
  (Development|PrintString (Utilities|String|Append "Rama world location is: " (Utilities|String|ToString(Vector) (Transformation|GetWorldLocation (Variables|Default|GetINdoorRama))) "Door world location is: " (Utilities|String|ToString(Vector) (Transformation|GetWorldLocation (Variables|Default|GetINdoor)))) true true "(R=0.956622,G=0.086891,B=1.000000,A=1.000000)" 0.0)
  (return))

(fn GetDoorYawRotation
  (return (.Yaw (Math|Rotator|BreakRotator (Transformation|GetWorldRotation (Variables|Default|GetINdoor))))))