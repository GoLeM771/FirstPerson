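; GermodoorActor is an interactable door that the player opens once by pressing F while inside its trigger.
; Overlapping OpenTrigger while closed enables player input and shows an interaction widget prompt; leaving disables input and hides it.
; Pressing F plays the door's opening animation and sets DoorOpened, blocking further prompts and replays.
; The overlap events do not check which actor entered or left.
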(event OnComponentBeginOverlap(OpenTrigger)
  (params (OverlappedComponent :type Primitive%20Component%20Object%20Reference) (OtherActor :type Actor%20Object%20Reference) (OtherComp :type Primitive%20Component%20Object%20Reference) (OtherBodyIndex :type Integer) (bFromSweep :type Boolean) (SweepResult :type Hit%20Result%20Structure%20%28by%20ref%29))
  (if (not (Variables|Default|GetDoorOpened?))
    (Input|EnableInput (Game|GetPlayerController 0))
    (Variables|Default|SetInDoorR true)
    (Rendering|SetVisibility (Variables|Default|GetWidget) true false)
    (bind _asinteraction_widget (Utilities|Casting|CastToInteractionWidget (UserInterface|GetUserWidgetObject (Variables|Default|GetWidget))))
    (Rendering|Components|TextRender|SetText (Variables|/Game/Blueprints/UI/InteractionWidget.InteractionWidget_C|GetName _asinteraction_widget) "Open Germodoor")))

(event OnComponentEndOverlap(OpenTrigger)
  (params (OverlappedComponent :type Primitive%20Component%20Object%20Reference) (OtherActor :type Actor%20Object%20Reference) (OtherComp :type Primitive%20Component%20Object%20Reference) (OtherBodyIndex :type Integer))
  (Input|DisableInput (Game|GetPlayerController 0))
  (Variables|Default|SetInDoorR false)
  (Rendering|SetVisibility (Variables|Default|GetWidget) false false))

(event EventBeginPlay)

(event Collision|EventActorBeginOverlap
  (params (OtherActor :type Actor%20Object%20Reference)))

(event EventTick
  (params (DeltaSeconds :type Float%20%28single-precision%29)))

(event Input|KeyboardEvents|F
  (params (Key :type Key%20Structure))
  (:Pressed
    (if (Variables|Default|GetInDoorR)
      (if (not (Variables|Default|GetDoorOpened?))
        (Components|Animation|PlayAnimation (Variables|Default|GetGermodoor) "/Game/Geometry/Props/MatTextAnim/Germodoor/Germodoor_Anim.Germodoor_Anim" false)
        (Variables|Default|SetDoorOpened? true)))))

(fn ConstructionScript)