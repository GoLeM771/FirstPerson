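; Quest giver actor that offers the player two quest sets, each a main and secondary quest, through a trigger-shown widget.
; On BeginPlay it spawns random, non-repeating quests, or reuses the rejected set plus a new one if a save exists, doubling main rewards.
; A completed main quest shows a reward widget instead; claiming it reopens selection and saves.
; An active quest triggers a workaround respawning saved quests and disabling the first-set button.
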(event OnComponentBeginOverlap(WidgetTrigger)
  (params (OverlappedComponent :type Primitive%20Component%20Object%20Reference) (OtherActor :type Actor%20Object%20Reference) (OtherComp :type Primitive%20Component%20Object%20Reference) (OtherBodyIndex :type Integer) (bFromSweep :type Boolean) (SweepResult :type Hit%20Result%20Structure%20%28by%20ref%29))
  (bind _returnvalue (Game|GetPlayerController 0))
  (if (Utilities|DoesObjectImplementInterface OtherActor "/Game/Blueprints/Interfaces/PlayerInterface.PlayerInterface_C")
    (bind _mainquestcompleted_ (Class|PlayerInterface|MainQuestComplitedBoolGetter(Message) (Game|GetPlayerCharacter 0)))
    (if _mainquestcompleted_
      ;[1 1 1] При коллизии с игроком просто переключаем visiable у виджета
      (Widget|SetVisibility (Variables|Default|GetRewardWidgetReference) "Visible")
      (else
        (Widget|SetVisibility (Variables|Default|GetQuestWidgetRef) "Visible")))
    (Input|SetInputModeGameandUI _returnvalue (Variables|Default|GetQuestWidgetRef) "DoNotLock" true)
    (Variables|/Script/Engine.PlayerController|SetbShowMouseCursor _returnvalue true)))

(event OnComponentEndOverlap(WidgetTrigger)
  (params (OverlappedComponent :type Primitive%20Component%20Object%20Reference) (OtherActor :type Actor%20Object%20Reference) (OtherComp :type Primitive%20Component%20Object%20Reference) (OtherBodyIndex :type Integer))
  (bind _returnvalue (Game|GetPlayerController 0))
  (if (Utilities|DoesObjectImplementInterface OtherActor "/Game/Blueprints/Interfaces/PlayerInterface.PlayerInterface_C")
    (bind _mainquestcompleted_ (Class|PlayerInterface|MainQuestComplitedBoolGetter(Message) (Game|GetPlayerCharacter 0)))
    (if _mainquestcompleted_
      ;[1 1 1] При коллизии с игроком просто переключаем visiable у виджета
      (Widget|SetVisibility (Variables|Default|GetRewardWidgetReference) "Hidden")
      (else
        (Widget|SetVisibility (Variables|Default|GetQuestWidgetRef) "Hidden")))
    (Input|SetInputModeGameOnly _returnvalue)
    (Variables|/Script/Engine.PlayerController|SetbShowMouseCursor _returnvalue false)))

(event Custom|CreateQuestSelectWidget
  ;[1 1 1] Создаём виджет и сразу делаем его невидимым
  (bind _returnvalue (UserInterface|CreateWidget "/Game/Blueprints/QuestSystem/QuestWidget.QuestWidget_C" 0 (Variables|Default|GetFirstSetMainQuestRef) (Variables|Default|GetFirstSetSecondQuestRef) (Variables|Default|GetSecondSetMainQuestRef) (Variables|Default|GetSecondSetSecondQuestRef)))
  (UserInterface|Viewport|AddtoViewport _returnvalue 0)
  (bind _output_get (Variables|Default|SetQuestWidgetRef _returnvalue))
  (Widget|SetVisibility _output_get "Hidden"))

(event Custom|GetRewardFromWidget
  (bind _returnvalue (Game|GetPlayerController 0))
  (Widget|RemovefromParent (Variables|Default|GetRewardWidgetReference))
  (CallFunction|CreateQuestSelectWidget)
  (Class|QuestInterface|DiscardQuestBool(Message) (Variables|Default|GetQuestSystemReference))
  (Class|PlayerInterface|SaveGameInterface(Message) (Game|GetPlayerCharacter 0))
  (Widget|SetVisibility (Variables|Default|GetQuestWidgetRef) "Visible")
  (Input|SetInputModeGameandUI _returnvalue 0 "DoNotLock" true)
  (Variables|/Script/Engine.PlayerController|SetbShowMouseCursor _returnvalue true))

(event Custom|LoadQuestKostil
  (bind _questsystemreference (Variables|Default|GetQuestSystemReference))
  (bind _outactors (Actor|GetAllActorsOfClass "/Game/Blueprints/QuestSystem/Quests/bp_baseQuest.bp_baseQuest_C"))
  (for _array_element _outactors
    (Actor|DestroyActor _array_element))
  (bind (_mainquesttoloadongamelocation _secondquesttoloadongamelocation _rejectedmainquest _rejectedsecondquest) (Class|PlayerInterface|GetQuestStructure(Message) (Game|GetPlayerCharacter 0)))
  (bind _output_get (Default|SpawnQuest _questsystemreference (.QuestClass (Utilities|Struct|BreakST_Quest _mainquesttoloadongamelocation)) true (.GoalCount (Utilities|Struct|BreakST_Quest _mainquesttoloadongamelocation)) 0 (.QuestReward (Utilities|Struct|BreakST_Quest _mainquesttoloadongamelocation))))
  (Variables|Default|SetFirstSetMainQuestRef _output_get)
  (bind _output_get_2 (Default|SpawnQuest _questsystemreference (.QuestClass (Utilities|Struct|BreakST_Quest _secondquesttoloadongamelocation)) false (.GoalCount (Utilities|Struct|BreakST_Quest _secondquesttoloadongamelocation)) 0 (.QuestReward (Utilities|Struct|BreakST_Quest _secondquesttoloadongamelocation))))
  (Variables|Default|SetFirstSetSecondQuestRef _output_get_2)
  (bind _output_get_3 (Default|SpawnQuest _questsystemreference (.QuestClass (Utilities|Struct|BreakST_Quest _rejectedmainquest)) true (.GoalCount (Utilities|Struct|BreakST_Quest _rejectedmainquest)) 0 (.QuestReward (Utilities|Struct|BreakST_Quest _rejectedmainquest))))
  (Variables|Default|SetSecondSetMainQuestRef _output_get_3)
  (bind _output_get_4 (Default|SpawnQuest _questsystemreference (.QuestClass (Utilities|Struct|BreakST_Quest _rejectedsecondquest)) false (.GoalCount (Utilities|Struct|BreakST_Quest _rejectedsecondquest)) 0 (.QuestReward (Utilities|Struct|BreakST_Quest _rejectedsecondquest))))
  (Variables|Default|SetSecondSetSecondQuestRef _output_get_4)
  (CallFunction|CreateQuestSelectWidget)
  (Default|DisableFirstSetButton (Variables|Default|GetQuestWidgetRef)))

(event EventBeginPlay
  (Utilities|FlowControl|Delay 1.0)
  (bind _returnvalue (SaveGame|DoesSaveGameExist "SaveTest"))
  (Variables|Default|SetGameLoad? _returnvalue)
  (bind _questsystem (Class|PlayerInterface|QuestSystemReferenceGetter(Message) (Game|GetPlayerCharacter 0)))
  (Variables|Default|SetQuestSystemReference _questsystem)
  ;[1 1 1] Проверка системы сохранений, если сохранения нет, генерим 2 рандомных сета, если есть, см. комменты в GenerateQuestSet
  (CallFunction|GenerateQuestSet)
  (bind _mainquestcompleted_ (Class|PlayerInterface|MainQuestComplitedBoolGetter(Message) (Game|GetPlayerCharacter 0)))
  (if _mainquestcompleted_
    (bind _returnvalue_2 (UserInterface|CreateWidget "/Game/Blueprints/QuestSystem/QuestReward.QuestReward_C" 0 self))
    (UserInterface|Viewport|AddtoViewport _returnvalue_2 0)
    (Widget|SetVisibility _returnvalue_2 "Hidden")
    (Variables|Default|SetRewardWidgetReference _returnvalue_2)
    (else
      (bind _result (Class|PlayerInterface|QuestGivedBoolGetter(Message) (Game|GetPlayerCharacter 0)))
      (if _result
        (CallFunction|LoadQuestKostil)
        (else
          (CallFunction|CreateQuestSelectWidget))))))

(fn ConstructionScript)

(fn GenerateQuestSet
  (bind _setarrey (Variables|Default|GetSetArrey))
  (bind _reward (Variables|Default|GetReward))
  (bind _setarrey_2 (Variables|Default|GetSetArrey))
  (bind _reward_2 (Variables|Default|GetReward))
  (bind _allquestclassarrey (Variables|Default|GetAllQuestClassArrey))
  (bind _questsystemreference (Variables|Default|GetQuestSystemReference))
  (bind _questsystemreference_2 (Variables|Default|GetQuestSystemReference))
  (bind _rejmainquest (Variables|/Game/Blueprints/QuestSystem/QuestSystem.QuestSystem_C|GetRejMainQuest _questsystemreference))
  (bind _rejsecondquest (Variables|/Game/Blueprints/QuestSystem/QuestSystem.QuestSystem_C|GetRejSecondQuest _questsystemreference))
  (bind (_mainquest_ _goalcount _currentcount _questreward _questclass) (Utilities|Struct|BreakST_Quest _rejsecondquest))
  (bind (_mainquest__2 _goalcount_2 _currentcount_2 _questreward_2 _questclass_2) (Utilities|Struct|BreakST_Quest _rejmainquest))
  (if (Variables|Default|GetGameLoad?)
    ;[1 1 1] Из сейва достаём 1 квестовый сет, который мы не взяли прошлый раз и генерируем 1 новый квестовый сет
    (bind _questref (CallFunction|GenerateQuest _mainquest__2 _questclass_2 _goalcount_2 0 _questreward_2))
    (Variables|Default|SetFirstSetMainQuestRef _questref)
    (bind _questref_2 (CallFunction|GenerateQuest _mainquest_ _questclass _goalcount 0 _questreward))
    (Variables|Default|SetFirstSetSecondQuestRef _questref_2)
    ;[1 1 1] Генерируем 1 новый квестовый сет
    (Utilities|Array|RemoveItem _allquestclassarrey _questclass_2)
    (Utilities|Array|RemoveItem _allquestclassarrey _questclass)
    (Variables|Default|SetMaxQuestCount (- (Variables|Default|GetMaxQuestCount) 2))
    (CallFunction|GetOneRandomQuest)
    (CallFunction|GetOneRandomQuest)
    (bind _questref_3 (CallFunction|GenerateQuest true (Utilities|Array|Get(acopy) _setarrey_2) 100000 0 _reward))
    (Variables|Default|SetSecondSetMainQuestRef _questref_3)
    (bind _questref_4 (CallFunction|GenerateQuest false (Utilities|Array|Get(acopy) _setarrey_2 1) 55555 0 _reward))
    (Variables|Default|SetSecondSetSecondQuestRef _questref_4)
    (else
      ;[1 1 1] Для игрока рандомайзятся 2 квестовых сета
      (CallFunction|QuestRandomizer)
      (bind _questref_5 (CallFunction|GenerateQuest true (Utilities|Array|Get(acopy) _setarrey) 1 0 _reward_2))
      (Variables|Default|SetFirstSetMainQuestRef _questref_5)
      (bind _questref_6 (CallFunction|GenerateQuest false (Utilities|Array|Get(acopy) _setarrey 1) 2 0 _reward_2))
      (Variables|Default|SetFirstSetSecondQuestRef _questref_6)
      (bind _questref_7 (CallFunction|GenerateQuest true (Utilities|Array|Get(acopy) _setarrey 2) 3 0 _reward_2))
      (Variables|Default|SetSecondSetMainQuestRef _questref_7)
      (bind _questref_8 (CallFunction|GenerateQuest false (Utilities|Array|Get(acopy) _setarrey 3) 4 0 _reward_2))
      (Variables|Default|SetSecondSetSecondQuestRef _questref_8)))
  ;[1 1 1] Сбрасываем переменные выполнения квестов, функция, которая запишет всё в сейвгейм игрока будит вызвана в QuestWidget
  (Variables|/Game/Blueprints/QuestSystem/QuestSystem.QuestSystem_C|SetMainQuestCompleted? _questsystemreference_2 false)
  (Variables|/Game/Blueprints/QuestSystem/QuestSystem.QuestSystem_C|SetSecondQuestCompleted? _questsystemreference_2 false)
  (return))

(fn GenerateQuest
  (params (MainQuest? :type Boolean) (QuestClass :type Bp%20Base%20Quest%20Class%20Reference) (GoalCount :type Integer) (CurrentCount :type Integer) (QuestReward :type Integer))
  (if MainQuest?
    (bind _output_get (LocalVariables|SetMultiplyer 2))
    (bind _returnvalue (Game|SpawnActorfromClass QuestClass (Math|Transform|MakeTransform "0, 0, 0") "Undefined" 0 (Utilities|Struct|MakeST_Quest MainQuest? GoalCount CurrentCount (* QuestReward _output_get) QuestClass) 0 0))
    (return _returnvalue)
    (else
      (bind _returnvalue_2 (Game|SpawnActorfromClass QuestClass (Math|Transform|MakeTransform "0, 0, 0") "Undefined" 0 (Utilities|Struct|MakeST_Quest MainQuest? GoalCount CurrentCount QuestReward QuestClass) 0 0))
      (return _returnvalue_2))))

(fn QuestRandomizer
  (CallFunction|GetOneRandomQuest)
  (CallFunction|GetOneRandomQuest)
  (CallFunction|GetOneRandomQuest)
  (CallFunction|GetOneRandomQuest)
  (return))

(fn GetOneRandomQuest
  (bind _output_get (LocalVariables|SetLocalRandomInteger (Math|Random|RandomIntegerinRange 0 (Variables|Default|GetMaxQuestCount))))
  (bind _output_get_2 (LocalVariables|SetLocalQuestClass (Utilities|Array|Get(acopy) (Variables|Default|GetAllQuestClassArrey) _output_get)))
  (Utilities|Array|Add (Variables|Default|GetSetArrey) _output_get_2)
  (Variables|Default|SetMaxQuestCount (- (Variables|Default|GetMaxQuestCount) 1))
  (Utilities|Array|RemoveItem (Variables|Default|GetAllQuestClassArrey) _output_get_2))