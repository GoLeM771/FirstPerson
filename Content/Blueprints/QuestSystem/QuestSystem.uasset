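; Quest manager that tracks the player's main and secondary quest across the hub and game levels.
; GiveQuest caches each quest's class, goal and reward; LoadQuestFromSave destroys existing quest actors and respawns both from those values with tick enabled.
; BeginPlay disables quest actor tick so hub quests don't count progress.
; One-shot completion events from quest actors save the game, and main quest completion also enables the lift transition.
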(event Custom|LoadQuestFromSave
  ;[1 1 1] Только на игровом уровне. Загрузка квестов из сейва
  (bind _outactors (Actor|GetAllActorsOfClass "/Game/Blueprints/QuestSystem/Quests/bp_baseQuest.bp_baseQuest_C"))
  (for _array_element _outactors
    (Actor|DestroyActor _array_element))
  (CallFunction|SpawnQuest (Variables|Default|GetMainQuestClass) true (Variables|Default|GetMainGoalCount) 0 (Variables|Default|GetMainQuestReward))
  (CallFunction|SpawnQuest (Variables|Default|GetSecondQuestClass) false (Variables|Default|GetSecndGoalCount) 0 (Variables|Default|GetSecondQuestReward)))

(event Custom|GiveQuest
  (params (MainQuest :type Bp%20Base%20Quest%20Object%20Reference) (SecondQuest :type Bp%20Base%20Quest%20Object%20Reference))
  ;[1 1 1] Получаем от quest giver квесты. Просто переписываем переменные 2х квестов
  (Utilities|FlowControl|Sequence
    (:then_0
      (bind _output_get (Variables|Default|SetMainQuestReference MainQuest))
      (Variables|Default|SetMainQuestClass (Utilities|GetClass _output_get))
      (Variables|Default|SetMainGoalCount (Variables|/Game/Blueprints/QuestSystem/Quests/bp_baseQuest.bp_baseQuest_C|GetGoalCount _output_get))
      (Variables|Default|SetMainQuestReward (Variables|/Game/Blueprints/QuestSystem/Quests/bp_baseQuest.bp_baseQuest_C|GetQuestReward _output_get)))
    (:then_1
      (bind _output_get_2 (Variables|Default|SetSecondQuestReference SecondQuest))
      (Variables|Default|SetSecondQuestClass (Utilities|GetClass _output_get_2))
      (Variables|Default|SetSecndGoalCount (Variables|/Game/Blueprints/QuestSystem/Quests/bp_baseQuest.bp_baseQuest_C|GetGoalCount _output_get_2))
      (Variables|Default|SetSecondQuestReward (Variables|/Game/Blueprints/QuestSystem/Quests/bp_baseQuest.bp_baseQuest_C|GetQuestReward _output_get_2)))))

(event Custom|DebugCompleteMainQuest
  (bind _mainquestreference (Variables|Default|GetMainQuestReference))
  ;[1 1 1] Дебаг, завершить квесты
  (if (not (Variables|/Game/Blueprints/TPCharacter.TPCharacter_C|GetInHubLocation? (Variables|Default|GetCharacterRef)))
    (Variables|/Game/Blueprints/QuestSystem/Quests/bp_baseQuest.bp_baseQuest_C|SetCurrentCount _mainquestreference (Variables|/Game/Blueprints/QuestSystem/Quests/bp_baseQuest.bp_baseQuest_C|GetGoalCount _mainquestreference))))

(event Custom|DebugCompleteSecondQuest
  (bind _secondquestreference (Variables|Default|GetSecondQuestReference))
  ;[1 1 1] Дебаг, завершить квесты
  (if (not (Variables|/Game/Blueprints/TPCharacter.TPCharacter_C|GetInHubLocation? (Variables|Default|GetCharacterRef)))
    (Variables|/Game/Blueprints/QuestSystem/Quests/bp_baseQuest.bp_baseQuest_C|SetCurrentCount _secondquestreference (Variables|/Game/Blueprints/QuestSystem/Quests/bp_baseQuest.bp_baseQuest_C|GetGoalCount _secondquestreference))))

(event EventBeginPlay
  (bind _astpcharacter (Utilities|Casting|CastToTPCharacter (Game|GetPlayerCharacter 0)))
  (Variables|Default|SetCharacterRef _astpcharacter)
  ;[1 1 1] Для хаба, когда event tick отключен квесты не считают каунтеры. Event tick включает QuestWidget
  (bind _outactors (Actor|GetAllActorsOfClass "/Game/Blueprints/QuestSystem/Quests/bp_baseQuest.bp_baseQuest_C"))
  (for _array_element _outactors
    (Actor|Tick|SetActorTickEnabled _array_element))
  (Development|PrintString "Tick Disabled"))

(event EventTick
  (params (DeltaSeconds :type Float%20%28single-precision%29))
  (Development|PrintString (Utilities|String|Append "Quest Gived? " (Utilities|String|ToString(Boolean) (Variables|Default|GetQuestGived?))) true true "(R=0.000000,G=0.660000,B=1.000000,A=1.000000)" 0.0))

(event EventSecondQuestCompleted
  ;[1 1 1] Интерфейс, слушает сообщения, которые отправляются с bp_baseQuest, вызывают сейв гейм на игроке, ревард за квест начисляет сам актор квеста
  (Utilities|FlowControl|DoOnce false
    (:Completed
      (Variables|Default|SetSecondQuestCompleted? true)
      (Development|PrintString "Done second quest" true true "(R=0.000000,G=0.660000,B=1.000000,A=1.000000)" 2e+01)
      (Default|SaveGame (Variables|Default|GetCharacterRef)))))

(event EventMainQuestCompleted
  (bind _characterref (Variables|Default|GetCharacterRef))
  (bind _liftreference (Variables|/Game/Blueprints/TPCharacter.TPCharacter_C|GetLiftReference _characterref))
  ;[1 1 1] Интерфейс, слушает сообщения, которые отправляются с bp_baseQuest, вызывают сейв гейм на игроке, ревард за квест начисляет сам актор квеста
  (Utilities|FlowControl|DoOnce false
    (:Completed
      (Variables|Default|SetMainQuestCompleted? true)
      (Development|PrintString "Done main quest" true true "(R=0.000000,G=0.660000,B=1.000000,A=1.000000)" 2e+01)
      (Default|SaveGame (Variables|Default|GetCharacterRef))
      (Utilities|IsValid _liftreference
        (:Is%20Valid
          (Variables|/Game/Blueprints/Elevator/BP_Elevator.BP_Elevator_C|SetEnableTransition? _liftreference true))
        (:Is%20Not%20Valid
          (Development|PrintString "Lift object is not valid" true true "(R=1.000000,G=0.060593,B=0.030746,A=1.000000)" 2e+01))))))

(event EventMainQuestFailed
  (params (MainQuest :type Boolean))
  ;[1 1 1] Интерфейс, слушает сообщения, которые отправляются с bp_baseQuest, вызывают сейв гейм на игроке, ревард за квест начисляет сам актор квеста
)

(event EventSecondQuestFailed
  ;[1 1 1] Интерфейс, слушает сообщения, которые отправляются с bp_baseQuest, вызывают сейв гейм на игроке, ревард за квест начисляет сам актор квеста
)

(fn SpawnQuest
  (params (QuestClass :type Bp%20Base%20Quest%20Class%20Reference) (MainQuest? :type Boolean) (GoalCount :type Integer) (CurrentCount :type Integer) (QuestReward :type Integer))
  (bind _returnvalue (Game|SpawnActorfromClass QuestClass (Math|Transform|MakeTransform "0, 0, 0") "Undefined" 0 (Utilities|Struct|MakeST_Quest MainQuest? GoalCount CurrentCount QuestReward QuestClass) self 0))
  (Actor|Tick|SetActorTickEnabled _returnvalue true)
  (if MainQuest?
    (bind _output_get (Variables|Default|SetMainQuestReference _returnvalue))
    (return _output_get)
    (else
      (bind _output_get_2 (Variables|Default|SetSecondQuestReference _returnvalue))
      (return _output_get_2))))