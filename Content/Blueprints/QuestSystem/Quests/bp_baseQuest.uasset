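; Base quest Blueprint for the quest system, holding a quest's type, goal and current counts, reward, completion state and text color.
; On BeginPlay it copies its data from the STQuest struct and tints the text yellow for secondary quests.
; On completion it sets the completed flag, turns the text green and triggers the main or secondary completion message through QuestSystemRef.
; The failure and count increment/decrement events are empty.
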(event Custom|OnQuestCompleted
  (bind _questsystemref (Variables|Default|GetQuestSystemRef))
  (Variables|Default|SetQuestCompleted? true)
  (Variables|Default|SetTextColor "(R=0.000000,G=1.000000,B=0.086107,A=1.000000)")
  (if (Variables|Default|GetMainQuest?)
    (Class|QuestInterface|MainQuestCompleted(Message) _questsystemref)
    (else
      (Class|QuestInterface|SecondQuestCompleted(Message) _questsystemref))))

(event Custom|OnQuestFailed)

(event EventBeginPlay
  (bind _stquest (Variables|Default|GetSTQuest))
  (bind (_mainquest_ _goalcount _currentcount _questreward) (Utilities|Struct|BreakST_Quest _stquest))
  (Variables|Default|SetMainQuest? _mainquest_)
  (Variables|Default|SetGoalCount _goalcount)
  (Variables|Default|SetCurrentCount _currentcount)
  (Variables|Default|SetQuestReward _questreward)
  (if (not (Variables|Default|GetMainQuest?))
    (Variables|Default|SetTextColor "(R=0.932733,G=1.000000,B=0.291360,A=1.000000)")))

(event EventCountMinus)

(event EventCountPlus)

(event EventTick
  (params (DeltaSeconds :type Float%20%28single-precision%29)))

(fn ConstructionScript)