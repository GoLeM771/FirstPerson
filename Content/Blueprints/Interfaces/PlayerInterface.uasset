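; PlayerInterface is a Blueprint Interface that lets other objects talk to the player without casting to its class.
; It declares setters, getters and event calls for health, armor, stamina, weapons, ammo, bombs, currency and movement.
; Further functions cover hub and elevator state, floor number, quests, saving, the respirator system, UI state, camera data and brightness.
; All functions are empty signatures with default returns, so implementers supply the logic.
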(fn StopShootinHubInterfaceEvent)

(fn InHubLocationSetter
  (params (InHubLocation? :type Boolean)))

(fn SwitchWeapontoInterface
  (params (ArreyElement :type Integer)))

(fn UnfocusDoorInterface)

(fn ModifyStatInterface
  (params (NewParam :type Float%20%28single-precision%29) (Stat :type E_Stat%20Enum :default "NewEnumerator0")))

(fn SetLiftReferenceInterface
  (params (ElevatorRef :type BP%20Elevator%20Object%20Reference)))

(fn SwitchinLiftBool
  (params (InLift? :type Boolean)))

(fn InLiftBoolGetter
  (return false))

(fn QuestGivedBoolGetter
  (return false))

(fn MainQuestComplitedBoolGetter
  (return false))

(fn InHubLocationGetter
  (return false))

(fn SaveGameInterface)

(fn EnableLiftTransition)

(fn GetQuestVariable
  (return "" "" "" "" "" "" false))

(fn AddAlternativeCurrency
  (params (AlternativeCurrency :type Integer)))

(fn GetQuestStructure
  (return "" "" "" ""))

(fn QuestSystemReferenceGetter
  (return 0))

(fn SaveRejectedQuestInterface
  (params (RejectedMainQuest :type Bp%20Base%20Quest%20Object%20Reference) (RejectedSecondQuest :type Bp%20Base%20Quest%20Object%20Reference)))

(fn GetLiftReferenceInterface
  (return 0))

(fn PlayBreatheAudio?
  (params (Play? :type Boolean) (HaveAir? :type Boolean)))

(fn EscMenuOpenSetter
  (params (Open? :type Boolean)))

(fn CreateHudHitWidgetInterface
  (params (HitLocation :type Vector)))

(fn GetPlayerForvardVectorandLocation
  (return "0, 0, 0" "0, 0, 0"))

(fn GetVelocityInterface
  (return "0, 0, 0"))

(fn GetPlayerCameraWorldRotationandLocation
  (return "0, 0, 0" "0, 0, 0"))

(fn CrosshairEventInterface)

(fn StopShootInterface)

(fn WoundSystemShootInterface)

(fn SetCharacterMaxWolkSpeed
  (params (WalkSpeed :type Float%20%28single-precision%29)))

(fn FlamethroverUnequip
  (params (Unequip? :type Boolean)))

(fn StaminaDecreaceAmountSetter
  (params (Param :type Float%20%28single-precision%29)))

(fn OutOfBreathSetter
  (params (Param :type Boolean)))

(fn CurrentandMaxStaminaGetter
  (return 0.0 0.0))

(fn CurrentStaminaSetter
  (params (Stamina :type Float%20%28single-precision%29)))

(fn IsSprintingGetter
  (return false))

(fn WeaponActorGetter
  (return 0))

(fn CurrentHealthGetter
  (return 0.0 0.0))

(fn CurrentArmorGetter
  (return 0.0 0.0))

(fn CurrentBombGetter
  (return 0 0))

(fn CurrentBombSetter
  (params (Bomb :type Integer)))

(fn InputEnablerInterface)

(fn AlternativeCurrencyGetter
  (return 0))

(fn StartRegenInterface)

(fn BrightnesSetterInterface
  (params (Brightness :type Float%20%28single-precision%29)))

(fn BrightnessGetterInterface
  (return 0.0))

(fn InventoryOpenSetter
  (params (InvOpen? :type Boolean)))

(fn FullMapReferenceGetter
  (return 0))

(fn FootstepsReferenceGetter
  (return 0 false false 0.0 0.0 false))

(fn CanSpawnBombSetter
  (params (CanSpawn? :type Boolean)))

(fn SkeletalMeshGetter
  (return 0))

(fn ResperatorSystemActivateSetter
  (params (Activate? :type Boolean)))

(fn ResperatorSystemGetter
  (return 0))

(fn FilllWeaponData
  (params (St_WeaponData :type S%20Weapon%20Component%20Property%20Structure)))

(fn WeaponStatsGetter
  (return 0 0 0 0 ""))

(fn AddAmmoInterface
  (params (AmmoToAdd :type Integer) (WeaponClass :type Actor%20Class%20Reference))
  (return 0))

(fn PresetArreySetterInterface
  (params (PresetStruct :type S%20Preset%20Data%20Structure)))

(fn PossessBack
  (params (ControllerReference :type Controller%20Object%20Reference)))

(fn InitializeWidjetsInterface)

(fn WeaponBaseComponentRefSetter
  (params (BaseComponentActorr :type Actor%20Object%20Reference)))

(fn BreakLineTraceFire)

(fn PlayeronFloorSetter
  (params (FloorNum :type Integer)))

(fn PlayeronFloorGetter
  (return 0))

(fn CloseMapCostil)