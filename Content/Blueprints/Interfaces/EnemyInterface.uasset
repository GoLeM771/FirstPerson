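; EnemyInterface is a Blueprint interface that declares the shared calls for enemies, apparently monsters generated from body parts.
; It covers damage, dead and damageable states, death animation selection, and a spawn-permission flag.
; Body-part functions expose mass, torso, head and arm coordinates, the skeletal mesh and the part array, plus spawn and shooting hooks.
; Further calls start mass-limited monster generation, set wall material and pass a room reference.
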(fn SimpleDamageEnemy
  (params (Damage :type Float%20%28single-precision%29)))

(fn BetonCounterPlus)

(fn IsDeadBoolSetter
  (params (Dead? :type Boolean)))

(fn RandomDeathSelect
  (params (DeathAnim :type Integer)))

(fn StartGenerateMonster
  (params (MaxPossiableMass :type Float%20%28single-precision%29)))

(fn IsDeadGetter
  (return false))

(fn BodyPartMassGetter
  (return 0.0))

(fn TorsoCoordinateGetter
  (return 0))

(fn HeadCoordinateGetter
  (return 0))

(fn ArmsCoordinateGetter
  (return 0))

(fn EnemySkeletalMeshGetter
  (return 0))

(fn CanSpawnEnemySetter
  (params (CanSpawn? :type Boolean)))

(fn BodyPartSpawnEnemy
  (params (SpawnWithoutCount? :type Boolean)))

(fn BodyPartsArreyGetter
  (return 0))

(fn CanSpawnEnemyGetter
  (return false))

(fn BodyPartsCanShoot?)

(fn SetWallMaterial
  (params (MaterialToSet :type Material%20Interface%20Object%20Reference)))

(fn CanbeDamagedBoolSetter
  (params (CanBeDamaged? :type Boolean)))

(fn RoomReferenceSetter
  (params (ActorReference :type Actor%20Object%20Reference)))