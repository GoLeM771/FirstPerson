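; BP_Lift is a two-panel lift that gates and sets up the player's travel between the hub and a game level.
; Overlapping the Checcer trigger opens the doors if the quest state allows it for LiftDirection: main quest completed for the hub, quest given for the level.
; The Box trigger sets the character's destination and InLift flag, and leaving it closes the doors after a delay by reversing the timeline.
; On BeginPlay it registers with the character and reopens for arriving riders.
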(event OnComponentBeginOverlap(Checcer)
  (params (OverlappedComponent :type Primitive%20Component%20Object%20Reference) (OtherActor :type Actor%20Object%20Reference) (OtherComp :type Primitive%20Component%20Object%20Reference) (OtherBodyIndex :type Integer) (bFromSweep :type Boolean) (SweepResult :type Hit%20Result%20Structure%20%28by%20ref%29))
  (bind _astpcharacter (Utilities|Casting|CastToTPCharacter OtherActor))
  (switch Utilities|FlowControl|Switch|SwitchonLiftEnum (Variables|Default|GetLiftDirection)
    (:NewEnumerator0
      (if (Variables|/Game/Blueprints/QuestSystem/QuestSystem.QuestSystem_C|GetMainQuestCompleted? (Variables|/Game/Blueprints/TPCharacter.TPCharacter_C|GetQuestSystem _astpcharacter))
        (CallFunction|OpenDoor :!label _label)
        (else
          (Development|PrintString "Main quest not completed"))))
    (:NewEnumerator1
      (if (Variables|/Game/Blueprints/QuestSystem/QuestSystem.QuestSystem_C|GetQuestGived? (Variables|/Game/Blueprints/TPCharacter.TPCharacter_C|GetQuestSystem _astpcharacter))
        (goto _label)
        (else
          (Development|PrintString "Quest not acepted"))))))

(event OnComponentBeginOverlap(Box)
  (params (OverlappedComponent :type Primitive%20Component%20Object%20Reference) (OtherActor :type Actor%20Object%20Reference) (OtherComp :type Primitive%20Component%20Object%20Reference) (OtherBodyIndex :type Integer) (bFromSweep :type Boolean) (SweepResult :type Hit%20Result%20Structure%20%28by%20ref%29))
  ;[1 1 1] Тут управление отправкой на определённый уровень
  (bind _astpcharacter (Utilities|Casting|CastToTPCharacter OtherActor))
  (switch Utilities|FlowControl|Switch|SwitchonLiftEnum (Variables|Default|GetLiftDirection)
    (:NewEnumerator0
      (Variables|/Game/Blueprints/TPCharacter.TPCharacter_C|SetGoToLevel _astpcharacter "LikvidatorHUB")
      (Variables|/Game/Blueprints/TPCharacter.TPCharacter_C|SetInLift? _astpcharacter true))
    (:NewEnumerator1
      (Variables|/Game/Blueprints/TPCharacter.TPCharacter_C|SetGoToLevel _astpcharacter "MechanicCheck")
      (Variables|/Game/Blueprints/TPCharacter.TPCharacter_C|SetInLift? _astpcharacter true))))

(event OnComponentEndOverlap(Box)
  (params (OverlappedComponent :type Primitive%20Component%20Object%20Reference) (OtherActor :type Actor%20Object%20Reference) (OtherComp :type Primitive%20Component%20Object%20Reference) (OtherBodyIndex :type Integer))
  (Utilities|Casting|CastToTPCharacter OtherActor)
  (Utilities|FlowControl|Delay 1.0)
  (CallFunction|CloseDoor))

(event Custom|OpenDoor
  (bind _panel1 (Variables|Default|GetPanel1))
  (bind _panel2 (Variables|Default|GetPanel2))
  (bind _relativelocation (Variables|/Script/Engine.SceneComponent|GetRelativeLocation _panel2))
  (bind _relativelocation_2 (Variables|/Script/Engine.SceneComponent|GetRelativeLocation _panel1))
  (Variables|Default|SetStartPositionPanel1 _relativelocation_2)
  (Variables|Default|SetStartPositionPanel2 _relativelocation)
  (Variables|Default|SetEndPositionPanel1 (+ _relativelocation_2 "0.000000,-100.000000, 0"))
  (Variables|Default|SetEndPositionPanel2 (+ _relativelocation "0,100.000000, 0"))
  (bind _openliftdor (Timeline|OpenLift Play)
    (:Update
      (Transformation|SetRelativeLocation _panel1 (Math|Vector|Lerp(Vector) (Variables|Default|GetStartPositionPanel1) (Variables|Default|GetEndPositionPanel1) _openliftdor) false false)
      (Transformation|SetRelativeLocation _panel2 (Math|Vector|Lerp(Vector) (Variables|Default|GetStartPositionPanel2) (Variables|Default|GetEndPositionPanel2) _openliftdor) false false))))

(event Custom|CloseDoor
  (bind _openliftdor (Timeline|OpenLift Reverse)
    (:Update
      (Transformation|SetRelativeLocation (Variables|Default|GetPanel1) (Math|Vector|Lerp(Vector) (Variables|Default|GetStartPositionPanel1) (Variables|Default|GetEndPositionPanel1) _openliftdor) false false)
      (Transformation|SetRelativeLocation (Variables|Default|GetPanel2) (Math|Vector|Lerp(Vector) (Variables|Default|GetStartPositionPanel2) (Variables|Default|GetEndPositionPanel2) _openliftdor) false false))))

(event EventBeginPlay
  (bind _astpcharacter (Utilities|Casting|CastToTPCharacter (Game|GetPlayerCharacter 0)))
  (Variables|/Game/Blueprints/TPCharacter.TPCharacter_C|SetLiftReference _astpcharacter self)
  (if (Variables|/Game/Blueprints/TPCharacter.TPCharacter_C|GetInLift? _astpcharacter)
    (Utilities|FlowControl|Delay 2.0)
    (CallFunction|OpenDoor)))

(fn ConstructionScript)