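; An actor component that records unlocked items in the player's save game.
; Shortly after BeginPlay, it caches the save game reference obtained from the player character through an interface message.
; UnlockItem adds an item only if it is not already in the saved array, then tells the character to save.
; GetCharactersUnlock returns that array, while GetPlayerUnlocksArrey is an empty stub.
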(event EventBeginPlay
  (Utilities|FlowControl|Delay 0.1)
  (bind _savegameref (Class|PlayerInterface|GetSaveGameReference(Message) (Game|GetPlayerCharacter 0)))
  (Variables|Default|SetSaveGameRef _savegameref))

(event EventTick
  (params (DeltaSeconds :type Float%20%28single-precision%29)))

(event EventUnlockItem
  (params (UnlockItem :type ST%20Unlock%20Item%20Structure))
  (if (== (Utilities|Array|FindItem (Variables|/Game/Blueprints/SaveGameBlueprint/New_FPS_SaveGame.New_FPS_SaveGame_C|GetUnlockedItem (Variables|Default|GetSaveGameRef)) UnlockItem) -1)
    (Utilities|Array|Add (Variables|/Game/Blueprints/SaveGameBlueprint/New_FPS_SaveGame.New_FPS_SaveGame_C|GetUnlockedItem (Variables|Default|GetSaveGameRef)) UnlockItem)
    (Class|PlayerInterface|SaveGameInterface(Message) (Game|GetPlayerCharacter 0))))

(fn GetCharactersUnlock
  (return (Variables|/Game/Blueprints/SaveGameBlueprint/New_FPS_SaveGame.New_FPS_SaveGame_C|GetUnlockedItem (Variables|Default|GetSaveGameRef))))

(fn GetPlayerUnlocksArrey
  (return 0))