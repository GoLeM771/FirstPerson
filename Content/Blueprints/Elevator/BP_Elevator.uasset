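; Elevator actor with two sliding doors that tracks whether the player character is inside and registers itself on that character.
; The OpenLift timeline lerps both panels apart and reverses to close, while BlockingBox collision is off during opening.
; Doors open after a delay on BeginPlay if the player is inside; leaving restores collision and closes them after a delay.
; Tick prints optional debug state; SaveData is an unwired stub.
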(event OnComponentBeginOverlap(Box)
  (params (OverlappedComponent :type Primitive%20Component%20Object%20Reference) (OtherActor :type Actor%20Object%20Reference) (OtherComp :type Primitive%20Component%20Object%20Reference) (OtherBodyIndex :type Integer) (bFromSweep :type Boolean) (SweepResult :type Hit%20Result%20Structure%20%28by%20ref%29))
  (bind _astpcharacter (Utilities|Casting|CastToTPCharacter OtherActor))
  (Variables|/Game/Blueprints/TPCharacter.TPCharacter_C|SetInLift? _astpcharacter true))

(event OnComponentEndOverlap(Box)
  (params (OverlappedComponent :type Primitive%20Component%20Object%20Reference) (OtherActor :type Actor%20Object%20Reference) (OtherComp :type Primitive%20Component%20Object%20Reference) (OtherBodyIndex :type Integer))
  ;[1 1 1] Закрывает двери когда игрок вышел
  (bind _astpcharacter (Utilities|Casting|CastToTPCharacter OtherActor))
  (Variables|/Game/Blueprints/TPCharacter.TPCharacter_C|SetInLift? _astpcharacter false)
  (CallFunction|SwitchCollision "QueryAndPhysics")
  (Utilities|FlowControl|Delay 2.0)
  (if (not (Variables|/Game/Blueprints/TPCharacter.TPCharacter_C|GetInLift? _astpcharacter))
    (CallFunction|CloseDoor)))

(event Custom|OpenDoor
  ;[1 1 1] Анимация открытия
  (CallFunction|SwitchCollision "NoCollision")
  (bind _openliftdor (Timeline|OpenLift Play)
    (:Update
      (Transformation|SetRelativeLocation (Variables|Default|GetPanel1) (Math|Vector|Lerp(Vector) (Variables|Default|GetStartPositionPanel1) (Variables|Default|GetEndPositionPanel1) _openliftdor) false false)
      (Transformation|SetRelativeLocation (Variables|Default|GetPanel2) (Math|Vector|Lerp(Vector) (Variables|Default|GetStartPositionPanel2) (Variables|Default|GetEndPositionPanel2) _openliftdor) false false))))

(event Custom|CloseDoor
  ;[1 1 1] Анимация открытия
  (bind _openliftdor (Timeline|OpenLift Reverse)
    (:Update
      (Transformation|SetRelativeLocation (Variables|Default|GetPanel1) (Math|Vector|Lerp(Vector) (Variables|Default|GetStartPositionPanel1) (Variables|Default|GetEndPositionPanel1) _openliftdor) false false)
      (Transformation|SetRelativeLocation (Variables|Default|GetPanel2) (Math|Vector|Lerp(Vector) (Variables|Default|GetStartPositionPanel2) (Variables|Default|GetEndPositionPanel2) _openliftdor) false false))))

(event EventBeginPlay
  ;[1 1 1] Открывает дверь если игрок в лифте
  (CallFunction|InitializeDoorVariable)
  (Variables|Default|SetEnableTransition? false)
  (bind _astpcharacter (Utilities|Casting|CastToTPCharacter (Game|GetPlayerCharacter 0)))
  (Variables|Default|SetCharacterRef _astpcharacter)
  (Variables|/Game/Blueprints/TPCharacter.TPCharacter_C|SetLiftReference _astpcharacter self)
  (if (Variables|/Game/Blueprints/TPCharacter.TPCharacter_C|GetInLift? (Variables|Default|GetCharacterRef))
    (Utilities|FlowControl|Delay 2.0)
    (CallFunction|OpenDoor)))

(event EventTick
  (params (DeltaSeconds :type Float%20%28single-precision%29))
  (bind _characterref (Variables|Default|GetCharacterRef))
  (if (Variables|Default|GetEnableDebugLog?)
    (Development|PrintString (Utilities|String|Append "Enable transition? " (Utilities|String|ToString(Boolean) (Variables|Default|GetEnableTransition?))) true true "(R=0.000000,G=0.660000,B=1.000000,A=1.000000)" 0.0)
    (Development|PrintString (Utilities|String|Append "Characre in lift? " (Utilities|String|ToString(Boolean) (Variables|/Game/Blueprints/TPCharacter.TPCharacter_C|GetInLift? _characterref))) true true "(R=0.000000,G=0.660000,B=1.000000,A=1.000000)" 0.0)
    (Development|PrintString (Utilities|String|Append "QuestGived? " (Utilities|String|ToString(Boolean) (Variables|/Game/Blueprints/QuestSystem/QuestSystem.QuestSystem_C|GetQuestGived? (Variables|/Game/Blueprints/TPCharacter.TPCharacter_C|GetQuestSystem _characterref)))) true true "(R=0.000000,G=0.660000,B=1.000000,A=1.000000)" 0.0)))

(fn ConstructionScript)

(fn SaveData
  (params (MainQuestCompleted? :type Boolean)))

(fn SwitchCollision
  (params (NewType :type ECollisionEnabled%20Enum :default "NoCollision"))
  (Collision|SetCollisionEnabled (Variables|Default|GetBlockingBox) NewType))

(fn InitializeDoorVariable
  (bind _panel1 (Variables|Default|GetPanel1))
  (bind _panel2 (Variables|Default|GetPanel2))
  (bind _relativelocation (Variables|/Script/Engine.SceneComponent|GetRelativeLocation _panel2))
  (bind _relativelocation_2 (Variables|/Script/Engine.SceneComponent|GetRelativeLocation _panel1))
  (Variables|Default|SetStartPositionPanel1 _relativelocation_2)
  (Variables|Default|SetStartPositionPanel2 _relativelocation)
  (Variables|Default|SetEndPositionPanel1 (+ _relativelocation_2 "0.000000,-100.000000, 0"))
  (Variables|Default|SetEndPositionPanel2 (+ _relativelocation "0,100.000000, 0"))
  (return))