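; Interactive elevator button inside a BP_Elevator parent that either calls the elevator or starts the trip to another level.
; Radius events toggle its prompt and F-key input.
; Calling opens the door if the player's quest flag suits the lift direction; travel mode closes it after a delay, then shows StatisticUI and disables movement.
; An interface event rechecks the quest and loads the hub or target level, otherwise reopens the door.
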(event EventBeginPlay
  (bind _widget (Variables|Default|GetWidget))
  ;[1 1 1] Подпись кнопки
  (bind _asbp_elevator (Utilities|Casting|CastToBP_Elevator (Actor|GetParentActor)))
  (Variables|Default|SetElevatorRef _asbp_elevator)
  (if (Variables|Default|GetGoToLevelButton?)
    (Class|ElevatorInterface|SetWidgetText(Message) _widget "To Floor")
    (else
      (Class|ElevatorInterface|SetWidgetText(Message) _widget "Call Elevator"))))

(event EventPlayerinRadius
  ;[1 1 1] Выведение подсказки
  (Rendering|SetVisibility (Variables|Default|GetWidget) true false)
  (Input|EnableInput (Game|GetPlayerController 0))
  (Variables|Default|SetInIntRadius? true))

(event EventPlayerOutRadius
  ;[1 1 1] Выведение подсказки
  (Rendering|SetVisibility (Variables|Default|GetWidget) false false)
  (Input|DisableInput (Game|GetPlayerController 0))
  (Variables|Default|SetInIntRadius? false))

(event EventGotoLevelInterface
  (CallFunction|GotoLevel))

(event Input|KeyboardEvents|F
  (params (Key :type Key%20Structure :default "None"))
  ;[1 1 1] Нажали кнопку
  (:Pressed
    (if (Variables|Default|GetInIntRadius?)
      (if (Variables|Default|GetGoToLevelButton?)
        (Utilities|FlowControl|Delay 2.0)
        (Default|CloseDoor (Variables|Default|GetElevatorRef))
        (Utilities|FlowControl|Delay 4.0)
        (bind _foundwidgets (Widget|GetAllWidgetsOfClass "/Game/Blueprints/UI/StatisticUI.StatisticUI_C" true))
        (Widget|SetVisibility (Utilities|Array|Get(acopy) _foundwidgets) "Visible")
        (Class|PlayerInterface|DisableCharacterMovement(Message) (Game|GetPlayerCharacter 0))
        (else
          (CallFunction|OpenDoor))))))

(fn ConstructionScript)

(fn SetHighlite
  (params (Highlight? :type Boolean))
  (Rendering|SetRenderCustomDepth (Variables|Default|GetCube) Highlight?))

(fn GotoLevel
  (bind _returnvalue (Game|GetPlayerCharacter 0))
  (bind _elevatorref (Variables|Default|GetElevatorRef))
  (switch Utilities|FlowControl|Switch|SwitchonElevatorTargetsEnum (Variables|/Game/Blueprints/Elevator/BP_Elevator.BP_Elevator_C|GetLiftDirection _elevatorref)
    (:NewEnumerator0
      (bind _mainquestcompleted_ (Class|PlayerInterface|MainQuestComplitedBoolGetter(Message) _returnvalue))
      (if _mainquestcompleted_
        (Game|OpenLevel(byName) "LikvidatorHUB")
        (else
          (Development|PrintString "Main quest not completed")
          (Default|OpenDoor _elevatorref)
          (Default|SwitchCollision (Variables|Default|GetElevatorRef) "NoCollision"))))
    (:NewEnumerator1
      (bind _result (Class|PlayerInterface|QuestGivedBoolGetter(Message) _returnvalue))
      (if _result
        (Game|OpenLevel(byName) (Utilities|String|StringToName (Variables|/Game/Blueprints/Elevator/BP_Elevator.BP_Elevator_C|GetTargetLevel _elevatorref)))
        (else
          (Development|PrintString "Quest not acepted")
          (Default|OpenDoor _elevatorref)
          (Default|SwitchCollision (Variables|Default|GetElevatorRef) "NoCollision"))))))

(fn OpenDoor
  (bind _returnvalue (Game|GetPlayerCharacter 0))
  (bind _elevatorref (Variables|Default|GetElevatorRef))
  (switch Utilities|FlowControl|Switch|SwitchonElevatorTargetsEnum (Variables|/Game/Blueprints/Elevator/BP_Elevator.BP_Elevator_C|GetLiftDirection _elevatorref)
    (:NewEnumerator0
      (bind _mainquestcompleted_ (Class|PlayerInterface|MainQuestComplitedBoolGetter(Message) _returnvalue))
      (if _mainquestcompleted_
        _
        (else
          (Development|PrintString "Main quest not completed")
          (return false))))
    (:NewEnumerator1
      (bind _result (Class|PlayerInterface|QuestGivedBoolGetter(Message) _returnvalue))
      (if _result
        _
        (else
          (Development|PrintString "Quest not acepted")
          (return false)))))
  (Default|OpenDoor _elevatorref)
  (return true))