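; Inventory component that stores items in a resizable slot array and toggles its on-screen widget.
; Adding fills a partial stack, recursing on overflow, or takes an empty slot, then applies the item's buff to the player and refreshes the widget.
; Toggling switches input mode and cursor; closing also clears dealer state and closes any linked inventory.
; Slot items refresh from class defaults, "Quality" holds stack count, and InventoryQuery checks item totals.
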(event Custom|InitializeInventory
  (CallFunction|PrepareInventory))

(event Custom|UpdateInventorySlots
  (params (Amount :type Integer))
  (Variables|Default|SetNumberOfSlots (+ (Variables|Default|GetNumberOfSlots) Amount))
  (CallFunction|PrepareInventory))

(event EventBeginPlay
  (CallFunction|PrepareInventory))

(event EventTick
  (params (DeltaSeconds :type Float%20%28single-precision%29)))

(fn ToggleInventory
  (bind _returnvalue (Game|GetPlayerController 0))
  (bind _returnvalue_2 (Game|GetPlayerCharacter 0))
  (bind _returnvalue_3 (Game|GetPlayerCharacter 0))
  (bind _returnvalue_4 (Game|GetPlayerController 0))
  (bind _inventorywidgetreference (Variables|Default|GetInventoryWidgetReference)
    (:then
      (Widget|RemovefromParent _inventorywidgetreference)
      (Variables|Default|SetInventoryWidgetReference 0)
      (Class|PlayerInterface|DealerInventorySetter(Message) _returnvalue_3 false)
      (Class|PlayerInterface|DealerReferenceSetter(Message) _returnvalue_3)
      (bind _invopen_ (Class|PlayerInterface|InventoryOpenGetter(Message) _returnvalue_2))
      (if _invopen_
        (Class|PlayerInterface|InventoryOpenSetter(Message) _returnvalue_2 false)
        (bind _inventoryreference (Class|PlayerInterface|OtherInventoryReferenseGetter(Message) _returnvalue_2))
        (CallFunction|ToggleInventory _inventoryreference))
      (Input|SetInputModeGameOnly _returnvalue)
      (Variables|/Script/Engine.PlayerController|SetbShowMouseCursor _returnvalue false))
    (:else
      (CallFunction|PrepareInventory)
      (bind _returnvalue_5 (UserInterface|CreateWidget "/Game/Blueprints/InventorySystem/InventoryMainWidget.InventoryMainWidget_C" 0 self (Variables|Default|GetInventoryMaster)))
      (Variables|Default|SetInventoryWidgetReference _returnvalue_5)
      (bind _hudref (Class|PlayerInterface|GetHudReferenceInterface(Message) (Game|GetPlayerCharacter 0)))
      (bind _returnvalue_6 (Class|CanvasPanel|AddChildtoCanvas (Variables|/Game/Blueprints/UI/StatusBar.StatusBar_C|GetHUD_Canvas _hudref) (Variables|Default|GetInventoryWidgetReference)))
      (Class|CanvasPanelSlot|SetAutoSize _returnvalue_6 true)
      (Class|CanvasPanelSlot|SetAlignment _returnvalue_6 "(X=0.500000,Y=0.500000)")
      (Class|CanvasPanelSlot|SetAnchors _returnvalue_6 (Utilities|Struct|MakeAnchors "(X=0.500000,Y=0.500000)" "(X=0.500000,Y=0.500000)"))
      (Class|CanvasPanelSlot|SetPosition _returnvalue_6 (Variables|Default|GetPosition))
      (Input|SetInputModeUIOnly _returnvalue_4 (Variables|Default|GetInventoryWidgetReference) "LockAlways")
      (Variables|/Script/Engine.PlayerController|SetbShowMouseCursor _returnvalue_4 true))))

(fn AddtoInventory
  (params (ContentToAdd :type ST%20Inventory%20Slot%20Structure))
  (bind (_bufftype _buffamount) (Utilities|GetClassDefaults (.class (.item ContentToAdd))))
  (bind _inventorywidgetreference (Variables|Default|GetInventoryWidgetReference))
  (if (.isstacable? (.item ContentToAdd))
    (bind _stackindex (Utilities|HasPartialStack ContentToAdd)
      (:True
        (bind (_success_ _itemquantityafteroperation) (CallFunction|AddtoStack ContentToAdd _stackindex))
        (LocalVariables|SetL_ItemQuantityAfterOperation _itemquantityafteroperation)
        (LocalVariables|SetIsSuccessful? _success_))
      (:False
        (bind _hasspaceininventory_ (CallFunction|HasSpaceinInventory?))
        (if _hasspaceininventory_
          (bind _succes_ (CallFunction|CreateStuck ContentToAdd :!label _label))
          (LocalVariables|SetIsSuccessful? _succes_)
          (else
            (return (LocalVariables|GetIsSuccessful?) (LocalVariables|GetL_ItemQuantityAfterOperation))))))
    (else
      (goto _label)))
  (if (LocalVariables|GetIsSuccessful?)
    (Class|PlayerInterface|BuffPlayerInterface(Message) (Game|GetPlayerCharacter 0) _bufftype _buffamount)
    (Utilities|IsValid _inventorywidgetreference
      (:Is%20Valid
        (Default|UpdateInventorySlots _inventorywidgetreference))
      (:Is%20Not%20Valid
        _)))
  (return (LocalVariables|GetIsSuccessful?) (LocalVariables|GetL_ItemQuantityAfterOperation)))

(fn PrepareInventory
  (Utilities|Array|Resize (Variables|Default|GetInventory) (Variables|Default|GetNumberOfSlots))
  (for (_array_element _array_index) (Variables|Default|GetInventory)
    (if (!= (.Class (Utilities|Struct|BreakST_PickupItem (.item _array_element))) 0)
      (Utilities|Array|SetArrayElem (Variables|Default|GetInventory) _array_index (Utilities|Struct|MakeST_InventorySlot (Utilities|GetClassDefaults (.Class (Utilities|Struct|BreakST_PickupItem (.item _array_element)))) (.quality _array_element) 0)))))

(fn CreateStuck
  (params (ContentToAdd :type ST%20Inventory%20Slot%20Structure))
  (bind (_array_element _array_index) (Utilities|Array|ForEachLoopwithBreak (Variables|Default|GetInventory) :!label _label)
    (:LoopBody
      (if (<= (.quality _array_element) 0)
        (LocalVariables|SetHasSpace? true)
        (LocalVariables|SetIdentifyIndex _array_index)
        (goto _label Break)))
    (:Completed
      (if (LocalVariables|GetHasSpace?)
        (Utilities|Array|SetArrayElem (Variables|Default|GetInventory) (LocalVariables|GetIdentifyIndex) ContentToAdd)
        (return (LocalVariables|GetHasSpace?))
        (else
          (return false))))))

(fn AddtoStack
  (params (Content :type ST%20Inventory%20Slot%20Structure) (SlotIndex :type Integer))
  (bind _inventory (Variables|Default|GetInventory))
  (bind _inventorywidgetreference (Variables|Default|GetInventoryWidgetReference))
  (bind _inventory_2 (Variables|Default|GetInventory))
  (bind _maxstacksize (Utilities|Struct|BreakST_PickupItem (.item Content)))
  (bind _output (Utilities|Array|Get(acopy) _inventory SlotIndex))
  (bind _output_2 (Utilities|Array|Get(acopy) _inventory_2 SlotIndex))
  (bind _output_get (LocalVariables|SetCurrentStackQuantity (.quality _output)))
  (if (> (+ _output_get (.Quality (Utilities|Struct|BreakST_InventorySlot Content))) (.maxstacksize (.item _output)))
    (Utilities|Array|SetArrayElem (Variables|Default|GetInventory) SlotIndex (Utilities|Struct|MakeST_InventorySlot (.item Content) _maxstacksize 0))
    (bind _hasspaceininventory_ (CallFunction|HasSpaceinInventory?))
    (if _hasspaceininventory_
      (bind _success_ (CallFunction|AddtoInventory (Utilities|Struct|MakeST_InventorySlot (.item Content) (- (.quality Content) (- _maxstacksize (LocalVariables|GetCurrentStackQuantity))) 0)))
      (Utilities|IsValid _inventorywidgetreference
        (:Is%20Valid
          (Default|UpdateInventorySlots _inventorywidgetreference))
        (:Is%20Not%20Valid
          _))
      (return _success_ (- (.quality Content) (- _maxstacksize (LocalVariables|GetCurrentStackQuantity))))
      (else
        (return true (- (.quality Content) (- _maxstacksize (LocalVariables|GetCurrentStackQuantity))))))
    (else
      (Utilities|Array|SetArrayElem _inventory_2 SlotIndex (Utilities|Struct|MakeST_InventorySlot (.item _output_2) (+ (.quality _output_2) (.quality Content)) 0))
      (return true 0))))

(fn InventoryQuery
  (params (Item :type Pickup%20Base%20Class%20Reference) (QueryAmount :type Integer))
  (bind _array_element (Utilities|Array|ForEachLoopwithBreak (Variables|Default|GetInventory))
    (:LoopBody
      (if (== (.Class (Utilities|Struct|BreakST_PickupItem (.item _array_element))) Item)
        (LocalVariables|SetRunningTotal (+ (.quality _array_element) (LocalVariables|GetRunningTotal)))))
    (:Completed
      (return (>= (LocalVariables|GetRunningTotal) QueryAmount)))))

(fn HasSpaceinInventory?
  (bind (_array_element _array_index) (Utilities|Array|ForEachLoopwithBreak (Variables|Default|GetInventory) :!label _label)
    (:LoopBody
      (if (<= (.quality _array_element) 0)
        (LocalVariables|SetL_HasSpace? true)
        (LocalVariables|SetL_IdentifyIndex _array_index)
        (goto _label Break)))
    (:Completed
      (return (LocalVariables|GetL_HasSpace?)))))