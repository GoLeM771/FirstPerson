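; Test AI enemy character that walks to the first TargetPoint in the level, then pauses and moves to the player.
; Tick repeatedly triggers this ZergPlayer sequence through a Delay.
; Attack stops movement, line-traces forward, applies a hit and stat change to TPCharacter, and randomizes AttackVar.
; Helpers, not called here, pick the nearest target within range and advance Bp_baseQuest actors with a matching quest type.
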(event Custom|ZergPlayer
  (Utilities|FlowControl|Delay 2.0)
  (bind _outactors (Actor|GetAllActorsOfClass "/Script/Engine.TargetPoint"))
  (AI|AIMoveTo self "0, 0, 0" (Utilities|Array|Get(acopy) _outactors) 5.0 false
    (:then
      (Utilities|FlowControl|Delay 4.0)
      (bind _astpcharacter (Utilities|Casting|CastToTPCharacter (Game|GetPlayerCharacter 0)))
      (bind _output_get (Variables|Default|SetCharRef _astpcharacter))
      (AI|AIMoveTo self "0, 0, 0" _output_get 5.0 false))))

(event EventBeginPlay)

(event EventTick
  (params (DeltaSeconds :type Float%20%28single-precision%29))
  (Utilities|FlowControl|Delay 2.0)
  (CallFunction|ZergPlayer))

(fn ConstructionScript)

(fn Attack
  (params (Damage :type Float%20%28single-precision%29) (AttackRange :type Integer))
  (bind _capsulecomponent (Variables|Collision|GetCapsuleComponent))
  (bind _returnvalue (Transformation|GetWorldLocation _capsulecomponent))
  (if (not (Variables|Death|GetisDead))
    (Components|Movement|StopMovementImmediately (Variables|Character|GetCharacterMovement))
    (bind _outhit (Collision|LineTraceByChannel _returnvalue (+ _returnvalue (* (Math|Vector|GetForwardVector (Transformation|GetWorldRotation _capsulecomponent)) AttackRange)) "TraceTypeQuery2" false 0 "ForDuration"))
    (bind _astpcharacter (Utilities|Casting|CastToTPCharacter (.HitActor (Collision|BreakHitResult _outhit)))
      (:then
        (Default|HudHit _astpcharacter (.Location (Collision|BreakHitResult _outhit)))
        (Default|ModifyStat _astpcharacter Damage "NewEnumerator1")
        (Variables|Attack|SetAttackVar (Math|Random|RandomIntegerinRange 0 2)))
      (:CastFailed
        (Development|PrintString "PlayerNotFound")))))

(fn FindTarget
  (Variables|Default|SetAttackDistance 1e+03)
  (for _array_element (Variables|Default|GetTargets)
    (if (< (Transformation|GetDistanceTo self _array_element) (Variables|Default|GetAttackDistance))
      (Variables|Default|SetAttackTarget _array_element)
      (Variables|Default|SetAttackDistance (Transformation|GetDistanceTo self _array_element))))
  (return (Variables|Default|GetAttackTarget)))

(fn CountPlus?
  (bind _outactors (Actor|GetAllActorsOfClass "/Game/Blueprints/QuestSystem/Quests/bp_baseQuest.bp_baseQuest_C"))
  (for _array_element _outactors
    (bind _asbp_base_quest (Utilities|Casting|CastTobp_baseQuest _array_element)
      (:then
        (if (Utilities|Enum|Equal(Enum) (Variables|/Game/Blueprints/QuestSystem/Quests/bp_baseQuest.bp_baseQuest_C|GetQuestType _asbp_base_quest) (Variables|Default|GetQuestType))
          (Default|CountPlus _asbp_base_quest)
          (else
            (Development|PrintString (Utilities|String|Append "Текущий квест " (Utilities|String|EnumtoString (Variables|/Game/Blueprints/QuestSystem/Quests/bp_baseQuest.bp_baseQuest_C|GetQuestType _asbp_base_quest)))))))
      (:CastFailed
        (Development|PrintString "CastFailed" true true "(R=0.000000,G=0.660000,B=1.000000,A=1.000000)" 1e+01))))
  (return))