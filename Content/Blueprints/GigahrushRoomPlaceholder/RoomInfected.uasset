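; RoomInfected is a Gigahrush room actor that populates its attachment sockets with sub-rooms at runtime.
; On BeginPlay it runs the parent logic, attaches a Sortir, then randomly either attaches a SmallRoom to one of three sockets or registers one with GigahruchManager as a secret-room candidate.
; SpawnSecretRoom attaches a SecretRoom to a freshly randomized socket, independent of the registered one, prints its location and sets SecretRoomSpawned.
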(event EventBeginPlay
  (bind _sortirsocet (Variables|Default|GetSortirSocet))
  (bind _gigahruchmanager (Variables|Default|GetGigahruchManager))
  (bind _sokettospawnsecretroom (Variables|/Game/Blueprints/ProceduralGigahrush/GigahruchManager.GigahruchManager_C|GetSoketToSpawnSecretRoom _gigahruchmanager))
  (|CallParentFunction)
  (bind _returnvalue (Game|SpawnActorfromClass "/Game/Blueprints/ProceduralGigahrush/Sortir.Sortir_C" (Transformation|GetWorldTransform _sortirsocet) "Undefined" 0 0))
  (Transformation|AttachComponentToComponent _returnvalue _sortirsocet "None" "SnapToTarget" "SnapToTarget" "SnapToTarget" true)
  (if (Math|Random|RandomBool)
    ;[1 1 1] Спавним 2ю комнату?
    (switch int (Math|Random|RandomIntegerinRange 0 2)
      (:Default
        (Variables|Default|SetAttachToSocet (Variables|Default|GetSmallRoomSocet1) :!label _label))
      (:0
        (goto _label))
      (:1
        (Variables|Default|SetAttachToSocet (Variables|Default|GetSmallRoomSocet2)))
      (:2
        (Variables|Default|SetAttachToSocet (Variables|Default|GetSmallRoomSocet3))))
    (bind _returnvalue_2 (Game|SpawnActorfromClass "/Game/Blueprints/ProceduralGigahrush/SmallRoom.SmallRoom_C" (Transformation|GetWorldTransform (Variables|Default|GetAttachToSocet)) "Undefined" 0 0))
    (Transformation|AttachComponentToComponent _returnvalue_2 (Variables|Default|GetAttachToSocet) "None" "SnapToTarget" "SnapToTarget" "SnapToTarget" true)
    (else
      ;[1 1 1] Отправляем рандомный сокет на гигахрущ менеджер. На какой то из отправленых заспавнится секретная комната
      (switch int (Math|Random|RandomIntegerinRange 0 2)
        (:Default
          (Utilities|Array|Add _sokettospawnsecretroom (Variables|Default|GetSmallRoomSocet1) :!label _label_2))
        (:0
          (goto _label_2))
        (:1
          (Utilities|Array|Add _sokettospawnsecretroom (Variables|Default|GetSmallRoomSocet2)))
        (:2
          (Utilities|Array|Add _sokettospawnsecretroom (Variables|Default|GetSmallRoomSocet3)))))))

(event Collision|EventActorBeginOverlap
  (params (OtherActor :type Actor%20Object%20Reference)))

(event EventTick
  (params (DeltaSeconds :type Float%20%28single-precision%29)))

(fn ConstructionScript)

(fn SpawnSecretRoom
  (switch int (Math|Random|RandomIntegerinRange 0 2)
    (:Default
      (Variables|Default|SetAttachToSocet (Variables|Default|GetSmallRoomSocet1) :!label _label))
    (:0
      (goto _label))
    (:1
      (Variables|Default|SetAttachToSocet (Variables|Default|GetSmallRoomSocet2)))
    (:2
      (Variables|Default|SetAttachToSocet (Variables|Default|GetSmallRoomSocet3))))
  (bind _returnvalue (Game|SpawnActorfromClass "/Game/Blueprints/ProceduralGigahrush/SecretRoom.SecretRoom_C" (Transformation|GetWorldTransform (Variables|Default|GetAttachToSocet)) "Undefined" 0 0))
  (Transformation|AttachComponentToComponent _returnvalue (Variables|Default|GetAttachToSocet) "None" "SnapToTarget" "SnapToTarget" "SnapToTarget" true)
  (Development|PrintString (Utilities|String|Append "Room spawned in " (Utilities|String|ToString(Vector) (Transformation|GetWorldLocation (Variables|Default|GetAttachToSocet)))) true true "(R=0.000000,G=0.660000,B=1.000000,A=1.000000)" 2e+01)
  (Variables|Default|SetSecretRoomSpawned? true))