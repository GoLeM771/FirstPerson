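; FPS save game Blueprint that stores an array of named presets, apparently for weapon configurations.
; CreateNewPresetData overwrites the entry with a matching PresetName, or inserts the new preset at the front if none matches.
; Companion functions remove a preset by index and return the whole array.
; AddWeaponComponentSpawnData and SetBaseWeaponComponentClass are empty stubs.
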(fn AddWeaponComponentSpawnData
  (params (SpawnData :type S%20Weapon%20Component%20Spawn%20Data%20Structure%20%28by%20ref%29)))

(fn SetBaseWeaponComponentClass
  (params (BaseWeaponComponentClass :type Actor%20Class%20Reference)))

(fn CreateNewPresetData
  (params (CurrentPresetData :type S%20Preset%20Data%20Structure%20%28by%20ref%29))
  (Utilities|FlowControl|Sequence
    (:then_0
      (for (_array_element _array_index) (Variables|Default|GetPresetDataArrey)
        (if (Utilities|Enum|Equal(Enum) (.PresetName (Utilities|Struct|BreakS_PresetData _array_element)) (.PresetName (Utilities|Struct|BreakS_PresetData CurrentPresetData)))
          (Utilities|Array|SetArrayElem (Variables|Default|GetPresetDataArrey) _array_index CurrentPresetData)
          (return))))
    (:then_1
      (Utilities|Array|Insert (Variables|Default|GetPresetDataArrey) CurrentPresetData)
      (return))))

(fn RemovePresetData
  (params (Index :type Integer))
  (Utilities|Array|RemoveIndex (Variables|Default|GetPresetDataArrey) Index)
  (return))

(fn GetPresetData
  (return (Variables|Default|GetPresetDataArrey)))