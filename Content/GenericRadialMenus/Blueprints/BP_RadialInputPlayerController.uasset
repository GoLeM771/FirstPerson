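; Player controller that shows a radial menu widget while Left Alt is held.
; Pressing the key creates the menu and adds it to the viewport if none exists; releasing it removes the widget and clears the reference.
; GetJoystickDirection returns the chosen stick's axis values as a 2D vector, negating Y for the left stick only.
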(event Input|KeyboardEvents|LeftAlt
  (params (Key :type Key%20Structure :default "None"))
  (:Pressed
    (Variables|Default|GetSelectionWeel
      (:then)
      (:else
        (bind _returnvalue (UserInterface|CreateWidget "/Game/Blueprints/UI/RadialMenu.RadialMenu_C" self))
        (bind _output_get (Variables|Default|SetSelectionWeel _returnvalue))
        (UserInterface|Viewport|AddtoViewport _output_get 0))))
  (:Released
    (bind _selectionweel (Variables|Default|GetSelectionWeel)
      (:then
        (Widget|RemovefromParent _selectionweel)
        (Variables|Default|SetSelectionWeel 0))
      (:else))))

(fn ConstructionScript)

(fn GetJoystickDirection
  (params (Stick :type EJoystickTypes%20Enum :default "NewEnumerator0"))
  (switch Utilities|FlowControl|Switch|SwitchonEJoystickTypes Stick
    (:NewEnumerator0
      (return (Math|Vector2D|MakeVector2D (Class|Actor|GetInputAxisKeyValue) (* (Class|Actor|GetInputAxisKeyValue) -1.0))))
    (:NewEnumerator1
      (return (Math|Vector2D|MakeVector2D (Class|Actor|GetInputAxisKeyValue) (Class|Actor|GetInputAxisKeyValue))))))